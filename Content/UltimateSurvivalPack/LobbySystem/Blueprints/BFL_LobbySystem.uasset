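; Blueprint function library of helper lookups for the lobby system: components, player identity and body mesh.
; Lobby and online component getters search the passed controller as an Actor, printing a red error if that cast fails.
; Player name and unique ID both come from the controller's object name, while the icon ignores the ID and returns a fixed asset.
; Gender body currently returns the male mesh for both genders.
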(fn `Get Gender Body`
  (params (Gender :type "/Game/UltimateSurvivalPack/Blueprints/Enum/E_Gender Enum" :default "NewEnumerator0"))
  (returns (Mesh :type "SkeletalMesh Object Reference"))
  (return (select `/Game/UltimateSurvivalPack/Blueprints/Enum/E_Gender` Gender :`NewEnumerator0` "/Game/UltimateSurvivalPack/Demo/Character/SK_MaleMesh.SK_MaleMesh" :`NewEnumerator1` "/Game/UltimateSurvivalPack/Demo/Character/SK_MaleMesh.SK_MaleMesh" :!type "SkeletalMesh Object Reference")))

(fn `Get Lobby Component`
  (params (`Player Controller` :type "Object Object Reference"))
  (returns (BP_LobbyComponent :type "/Game/UltimateSurvivalPack/LobbySystem/Blueprints/BP_LobbyComponent Object Reference"))
  ;[1 0.1771 0.1771] Get Component From Your Controller
  (bind _asactor (cast `Actor` `Player Controller`)
    (:`then`
      (bind _returnvalue (`Actor.GetComponentByClass` _asactor "/Game/UltimateSurvivalPack/LobbySystem/Blueprints/BP_LobbyComponent.BP_LobbyComponent_C"))
      (`/Engine/EditorBlueprintResources/StandardMacros.IsValid` _returnvalue
        (:`Is Valid`
          (return _returnvalue))))
    (:`CastFailed`
      (`KismetSystemLibrary.PrintString` null (`KismetStringLibrary.Concat_StrStr` "The called controlled does not have \"BP_LobbyComponent\" integrated. It has to be a \"Player Controller\"." " \nCaller:" (`KismetSystemLibrary.GetDisplayName` `Player Controller`)) true true (struct :`R` 1.0 :`A` 1.0) 4.0)
      (return null))))

(fn `Get Online Component`
  (params (`Player Controller` :type "Object Object Reference"))
  (returns (BP_OnlineComponent :type "/Game/UltimateSurvivalPack/Blueprints/Components/BP_OnlineComponent Object Reference"))
  ;[1 0.1771 0.1771] Get Component From Your Controller
  (bind _asactor (cast `Actor` `Player Controller`)
    (:`then`
      (bind _returnvalue (`Actor.GetComponentByClass` _asactor "/Game/UltimateSurvivalPack/Blueprints/Components/BP_OnlineComponent.BP_OnlineComponent_C"))
      (`/Engine/EditorBlueprintResources/StandardMacros.IsValid` _returnvalue
        (:`Is Valid`
          (return _returnvalue))))
    (:`CastFailed`
      (`KismetSystemLibrary.PrintString` null (`KismetStringLibrary.Concat_StrStr` "The called controlled does not have \"BP_OnlineComponent\" integrated. It has to be a \"Player Controller\"." " \nCaller:" (`KismetSystemLibrary.GetDisplayName` `Player Controller`)) true true (struct :`R` 1.0 :`A` 1.0) 4.0)
      (return null))))

(fn `Get Player Icon`
  (params (`Unique ID` :type String))
  (returns (Icon :type "Texture2D Object Reference"))
  (return "/Engine/EngineResources/AICON-Green.AICON-Green"))

(fn `Get Player Name`
  (params (Controller :type "PlayerController Object Reference"))
  (returns (Name :type String))
  (return (`KismetSystemLibrary.GetObjectName` Controller)))

(fn `Get Player Unique ID`
  (params (Controller :type "PlayerController Object Reference"))
  (returns (`Unique ID` :type String))
  (return (`KismetSystemLibrary.GetObjectName` Controller)))