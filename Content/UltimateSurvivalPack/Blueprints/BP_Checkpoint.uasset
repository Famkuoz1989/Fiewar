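; BP_Checkpoint is a checkpoint actor that shows custom mission markers pointing at itself.
; On BeginPlay it continues only if its owner is a local Controller, then passes its marker data to player 0's mission component, provided that component's HUD is valid.
; It stores the returned markers and removes each through the same component when the checkpoint is destroyed.
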(event `self.ReceiveBeginPlay`
  (bind _returnvalue (`GameplayStatics.GetPlayerController` 0))
  (bind _missioncomponent (`/Game/UltimateSurvivalPack/Blueprints/BFL_UMSPack.Get Mission Component` _returnvalue))
  ;[1 1 1] Create Markers
  ;;[1 1 1] Filter Local
  (bind _ascontroller (cast `Controller` (`self.GetOwner`)))
  (if (`Controller.IsLocalController` _ascontroller)
    (`/Engine/EditorBlueprintResources/StandardMacros.IsValid` _returnvalue
      (:`Is Valid`
        (`/Engine/EditorBlueprintResources/StandardMacros.IsValid` (`/Game/UltimateSurvivalPack/Blueprints/Components/BP_MissionComponent.HUD` _missioncomponent)
          (:`Is Valid`
            (bind _marker_reference (`/Game/UltimateSurvivalPack/Blueprints/Components/BP_MissionComponent.Add Custom Marker` _missioncomponent (`self.Marker Data`) self))
            (set `self.Markers` _marker_reference)))))))

(event `self.ReceiveDestroyed`
  ;[1 1 1] Remove all markers
  (for _array_element (`self.Markers`)
    (`/Game/UltimateSurvivalPack/Blueprints/Components/BP_MissionComponent.Remove Marker` (`/Game/UltimateSurvivalPack/Blueprints/BFL_UMSPack.Get Mission Component` (`GameplayStatics.GetPlayerController` 0)) _array_element)))

(fn `UserConstructionScript`)