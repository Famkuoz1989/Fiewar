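; BP_GasSource is a fuel reservoir in the survival pack that can be filled, drained and queried for current fuel and capacity.
; AddFuel caps at capacity and returns a fraction of 100: the amount added, or on overflow the excess over a hardcoded 100.
; RemoveFuel drains up to 10 units per call, returning that fraction.
; Vehicle health, tire hover and passenger dismount functions are stubs returning defaults.
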(fn `Add Fuel`
  (params (`Fuel Amount` :type "Float (double-precision)"))
  (returns (`Take Durability` :type "Float (double-precision)"))
  (locals (`L Durab` :type "Float (double-precision)"))
  (bind _fuel_amount (`local.Fuel Amount`))
  (bind _returnvalue (+ (`self.Fuel`) `Fuel Amount`))
  (if (< (`self.Fuel`) (`self.Fuel Capacity`))
    (if (> _returnvalue (`self.Fuel Capacity`))
      (set `local.L Durab` (- _returnvalue 100.0))
      (set `self.Fuel` (`self.Fuel Capacity`))
      (return (/ (`local.L Durab`) 100.0))
      (else
        (set `self.Fuel` (+ (`self.Fuel`) _fuel_amount))
        (return (/ _fuel_amount 100.0))))
    (else
      (return 0.0))))

(fn `Add Health to Vehicle`
  (params (Amount :type "Float (double-precision)"))
  (returns (Success :type Boolean))
  (return false))

(fn `BPI_TireSystem_HoveredOnTire`
  (params (HitComponent :type "SceneComponent Object Reference"))
  (returns (`Punctured Tire Index` :type Byte))
  (return 0))

(fn `Get Fuel`
  (returns (`Fuel Amount` :type "Float (double-precision)") (`Max Fuel` :type "Float (double-precision)"))
  (return (`self.Fuel`) (`self.Fuel Capacity`)))

(fn `Passenger DIsmount Request`
  (params (`From Attach Point` :type "SceneComponent Object Reference") (`Info Call Only` :type Boolean))
  (returns (`Dismount Location` :type "Vector Structure"))
  (return (0.0 0.0 0.0)))

(fn `Remove Fuel`
  (returns (`Add Durability` :type "Float (double-precision)"))
  (locals (`L Cached Fuel` :type "Float (double-precision)"))
  (bind _fuel (`self.Fuel`))
  (if (> _fuel 0.0)
    (bind _output_get (set `local.L Cached Fuel` _fuel))
    (if (< _output_get 10.0)
      (set `self.Fuel` 0.0)
      (return (/ (`local.L Cached Fuel`) 100.0))
      (else
        (set `self.Fuel` (- (`self.Fuel`) 10.0))
        (return 0.1)))
    (else
      (return 0.0))))

(fn `UserConstructionScript`)