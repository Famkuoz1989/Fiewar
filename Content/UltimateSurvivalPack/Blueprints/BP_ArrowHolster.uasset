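; Arrow holster that swaps its static mesh to show up to five arrows from the local player's inventory.
; UpdateHolster subtracts the arrow visible on a held bow unless it is being dequipped.
; OnArrowGrabbed waits a tick, then shows one fewer than the inventory count.
; Local updates apply the mesh directly, while SERVERUpdateMesh sets ArrowAmount, whose OnRep refreshes the mesh.
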(event `/Game/UltimateSurvivalPack/Blueprints/Interface/BPI_Holster.Update Holster`
  (bind _returnvalue (`/Game/UltimateSurvivalPack/Blueprints/BFL_UMSPack.Get Inventory Component` (`GameplayStatics.GetPlayerController` 0)))
  (bind _holdable_actor (`/Game/UltimateSurvivalPack/Blueprints/Components/BP_PlayerComponent.Holdable Actor` (`/Game/UltimateSurvivalPack/Blueprints/BFL_UMSPack.Get Player Component` (`/Game/UltimateSurvivalPack/Blueprints/Components/BP_PlayerInventoryComponent.Human Player Character` _returnvalue))))
  (bind _asbp_holdable_range_weapon_bow (cast `/Game/UltimateSurvivalPack/Blueprints/Holdable/HoldableActors/BP_Holdable_RangeWeapon_Bow` _holdable_actor)
    (:`then`
      (`/Engine/EditorBlueprintResources/StandardMacros.IsValid` _holdable_actor
        (:`Is Valid`
          (if (`/Game/UltimateSurvivalPack/Blueprints/Holdable/HoldableActors/Parent/BP_Holdable.Dequiping` _holdable_actor)
            (set `self.Arrow Amount` (`KismetMathLibrary.Clamp` (`/Game/UltimateSurvivalPack/Blueprints/Components/BP_PlayerInventoryComponent.Find Item Amount` _returnvalue "Arrow") 0 5) :!label _label)
            (`self.Update Holster Mesh` (`self.Arrow Amount`))
            (else
              (set `self.Arrow Amount` (`KismetMathLibrary.Clamp` (- (`/Game/UltimateSurvivalPack/Blueprints/Components/BP_PlayerInventoryComponent.Find Item Amount` _returnvalue "Arrow") (`KismetMathLibrary.Conv_BoolToInt` (`SceneComponent.IsVisible` (`/Game/UltimateSurvivalPack/Blueprints/Holdable/HoldableActors/BP_Holdable_RangeWeapon_Bow.Arrow` _asbp_holdable_range_weapon_bow)))) 0 5))
              (`self.Update Holster Mesh` (`self.Arrow Amount`)))))
        (:`Is Not Valid`
          (goto _label))))
    (:`CastFailed`
      (goto _label))))

(event `SERVER Update Mesh`
  (params (Amount :type Integer))
  (set `self.Arrow Amount` Amount))

(event `/Game/UltimateSurvivalPack/Blueprints/Interface/BPI_Holster.On Arrow Grabbed`
  (`KismetSystemLibrary.Delay` 0.0)
  (set `self.Arrow Amount` (`KismetMathLibrary.Clamp` (- (`/Game/UltimateSurvivalPack/Blueprints/Components/BP_PlayerInventoryComponent.Find Item Amount` (`/Game/UltimateSurvivalPack/Blueprints/BFL_UMSPack.Get Inventory Component` (`GameplayStatics.GetPlayerController` 0)) "Arrow") 1) 0 5))
  (`self.Update Holster Mesh` (`self.Arrow Amount`)))

(fn `OnRep_Arrow Amount`
  (`self.Update Holster Mesh` (`self.Arrow Amount`)))

(fn `Update Holster Mesh`
  (params (Item :type Integer))
  (`StaticMeshComponent.SetStaticMesh` (`self.StaticMesh`) (select `int` Item :`0` "/Game/UltimateSurvivalPack/Demo/Mesh/SM_ArrowHolster_06.SM_ArrowHolster_06" :`1` "/Game/UltimateSurvivalPack/Demo/Mesh/SM_ArrowHolster_05.SM_ArrowHolster_05" :`2` "/Game/UltimateSurvivalPack/Demo/Mesh/SM_ArrowHolster_04.SM_ArrowHolster_04" :`3` "/Game/UltimateSurvivalPack/Demo/Mesh/SM_ArrowHolster_03.SM_ArrowHolster_03" :`4` "/Game/UltimateSurvivalPack/Demo/Mesh/SM_ArrowHolster_02.SM_ArrowHolster_02" :`5` "/Game/UltimateSurvivalPack/Demo/Mesh/SM_ArrowHolster_01.SM_ArrowHolster_01" :!type "StaticMesh Object Reference")))

(fn `UserConstructionScript`)