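; BP_Ghost_ChickenCoop is the ghost Blueprint for placing a chicken coop in the building system.
; It extends a parent ghost class, overriding the custom placement condition to require both the parent check and a near-flat, upward-facing surface, tested through the hit normal's Z.
; It passes the parent check an unlocked location, returns a zero vector from Vector Modification and leaves construction to the parent.
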(fn `Custom Condition Pass`
  (params (Hit :type "HitResult Structure") (`Locked Location` :type Boolean))
  (returns (Return :type Boolean))
  (bind _return (`parent.Custom Condition Pass` Hit false)) ; Is Build Type = Building?
  (if _return
    (return (> (.z (`.ImpactNormal` (`GameplayStatics.BreakHitResult` Hit))) 0.9))
    (else
      (return false))))

(fn `UserConstructionScript`
  (`parent.UserConstructionScript`))

(fn `Vector Modification`
  (params (Vector :type "Vector Structure"))
  (returns (Return :type "Vector Structure"))
  (return (0.0 0.0 0.0)))