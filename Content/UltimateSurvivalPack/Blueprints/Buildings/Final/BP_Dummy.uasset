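; BP_Dummy is a hittable target dummy that tilts and plays a sound when damaged.
; Point damage converts the shot direction relative to the actor's yaw into a pitch and roll tilt using sine and cosine.
; A multicast event plays the Effect timeline, lerping the static mesh from the actor's rotation toward that tilt.
; Any damage triggers a separate multicast that spawns a hit sound at the actor's location.
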(event `self.ReceivePointDamage`
  (params (Damage :type "Float (single-precision)") (DamageType :type "DamageType Object Reference") (HitLocation :type "Vector Structure") (HitNormal :type "Vector Structure") (HitComponent :type "PrimitiveComponent Object Reference") (BoneName :type Name) (ShotFromDirection :type "Vector Structure") (InstigatedBy :type "Controller Object Reference") (DamageCauser :type "Actor Object Reference") (HitInfo :type "HitResult Structure (by ref)"))
  (bind (_returnvalue_roll _returnvalue_pitch _returnvalue_yaw) (`KismetMathLibrary.BreakRotator` (`self.K2_GetActorRotation`)))
  (bind (_returnvalue_roll_2 _returnvalue_pitch_2 _returnvalue_yaw_2) (`KismetMathLibrary.BreakRotator` (`KismetMathLibrary.MakeRotFromX` ShotFromDirection)))
  (bind (_returnvalue_roll_3 _returnvalue_pitch_3 _returnvalue_yaw_3) (`KismetMathLibrary.BreakRotator` (`self.K2_GetActorRotation`)))
  (bind (_returnvalue_roll_4 _returnvalue_pitch_4 _returnvalue_yaw_4) (`KismetMathLibrary.BreakRotator` (`KismetMathLibrary.NormalizedDeltaRotator` (`KismetMathLibrary.MakeRotator` 0.0 0.0 _returnvalue_yaw_2) (`KismetMathLibrary.MakeRotator` 0.0 0.0 _returnvalue_yaw))))
  (bind _output_get (set `self.Target Rotation` (`KismetMathLibrary.MakeRotator` (* (`KismetMathLibrary.DegSin` _returnvalue_yaw_4) 30.0) (* (`KismetMathLibrary.DegCos` _returnvalue_yaw_4) -30.0) _returnvalue_yaw_3)))
  (`self.Multicast Hit Effect` _output_get))

(event `Multicast Hit Effect`
  (params (`Target Rotation` :type "Rotator Structure"))
  (set `self.Target Rotation` `Target Rotation`)
  (bind (_direction _alpha) (`Timeline|Effect` :!via `PlayFromStart`)
    (:`Update`
      (`SceneComponent.K2_SetWorldRotation` (`self.StaticMesh`) (`KismetMathLibrary.RLerp` (`self.K2_GetActorRotation`) (`self.Target Rotation`) _alpha true) false false))))

(event `self.ReceiveAnyDamage`
  (params (Damage :type "Float (single-precision)") (DamageType :type "DamageType Object Reference") (InstigatedBy :type "Controller Object Reference") (DamageCauser :type "Actor Object Reference"))
  (`self.MUTLICAST Plas Hit Sound`))

(event `MUTLICAST Plas Hit Sound`
  (`GameplayStatics.SpawnSoundAtLocation` null (`self.K2_GetActorLocation`) (struct) 1.0 1.0 0.0 null null))

(fn `UserConstructionScript`)