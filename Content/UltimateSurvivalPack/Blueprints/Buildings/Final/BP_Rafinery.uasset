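; Refinery building for the survival pack: an interactable chest that burns fuel items to convert resources placed in it into output items.
; On the server, storage updates restart per-slot timers and consume fuel, enabling Tick only while fueled.
; Each tick decrements fuel and slot timers, batching finished outputs into the inventory or dropping them.
; Replicated Active calls an empty toggle hook; cupboard access locking and progress saving exist but are unwired.
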(event `Toggle Rafinery Action`
  (params (Toggle :type Boolean)))

(event `/Game/UltimateSurvivalPack/Blueprints/Interface/BPI_InventorySystem.On Interacted`
  (params (Executor :type "Controller Object Reference"))
  (bind _returnvalue (`/Game/UltimateSurvivalPack/Blueprints/BFL_UMSPack.Get Inventory Component` Executor))
  (bind _bp_chestinventorycomponent (`self.BP_ChestInventoryComponent`))
  ;[0.3083 0.573 1] On Interacted
  (`KismetArrayLibrary.Array_AddUnique` (`/Game/UltimateSurvivalPack/Blueprints/Components/BP_ChestInventoryComponent.Controlling Components` (`self.BP_ChestInventoryComponent`)) _returnvalue)
  (`/Game/UltimateSurvivalPack/Blueprints/Components/BP_PlayerInventoryComponent.Open Chest Inventory` _returnvalue _bp_chestinventorycomponent true (`/Game/UltimateSurvivalPack/Blueprints/Components/BP_MasterInventoryComponent.Inventory` _bp_chestinventorycomponent)))

(event `/Game/UltimateSurvivalPack/Blueprints/Interface/BPI_InventorySystem.Toggle Selected`
  (params (Toggle :type Boolean))
  (bind _chest (`self.Chest`))
  (bind _chest_2 (`self.Chest`))
  ;[1 1 1] On Selected
  (if Toggle
    (`PrimitiveComponent.SetRenderCustomDepth` _chest_2 true)
    (`PrimitiveComponent.SetCustomDepthStencilValue` _chest_2 1)
    (else
      (`PrimitiveComponent.SetRenderCustomDepth` _chest false)
      (`PrimitiveComponent.SetCustomDepthStencilValue` _chest 0))))

(event `self.ReceiveBeginPlay`
  (`/Engine/EditorBlueprintResources/ActorMacros.Switch Has Authority`
    (:`Authority`
      (add `/Game/UltimateSurvivalPack/Blueprints/Components/BP_ChestInventoryComponent.Storage Updated` (`self.BP_ChestInventoryComponent`) (delegate `On Storage Updated`)))))

(event `On Storage Updated`
  (`self.Check Slot Time`)
  (if (<= (`self.Current Fuel Time`) 0)
    (bind (_item_id _return) (`self.Has Fuel`))
    (if _return
      (bind (_amount _time) (break `/Game/UltimateSurvivalPack/Blueprints/Structs/S_ItemFuel` (`BlueprintMapLibrary.Map_Find` (`self.Fuel Types`) _item_id)))
      (set `self.Current Fuel Time` _time)
      (`/Game/UltimateSurvivalPack/Blueprints/Components/BP_ChestInventoryComponent.Remove Items` (`self.BP_ChestInventoryComponent`) _item_id _amount true)
      (`self.SetActorTickEnabled` true)
      (set `self.Active` true)
      (else
        (`self.SetActorTickEnabled` false)
        (set `self.Active` false)))))

(event `self.ReceiveTick`
  (params (DeltaSeconds :type "Float (single-precision)"))
  ;[1 1 1] Update Furnace Progress
  (`self.Update Slot Time`)
  (bind _result (`/Engine/EditorBlueprintResources/StandardMacros.DecrementInt` (`self.Current Fuel Time`))
    (:`  `
      (if (<= _result 0)
        (`self.On Storage Updated`)))))

(fn `Check Slot Time`
  (locals (`L Item ID` :type Name))
  (bind _slot_time (`self.Slot Time`))
  (bind (_value _returnvalue) (`BlueprintMapLibrary.Map_Find` (`self.Final Resource Types`) (`local.L Item ID`)))
  (for (_array_element _array_index) (`/Game/UltimateSurvivalPack/Blueprints/Components/BP_MasterInventoryComponent.Inventory` (`self.BP_ChestInventoryComponent`))
    (set `local.L Item ID` (`.ID_2_1F4451EE4759095BA0D31BB237483A5E` (break `/Game/UltimateSurvivalPack/Blueprints/Structs/S_InventoryItem` _array_element)))
    (if _returnvalue
      (if (`KismetArrayLibrary.Array_IsValidIndex` _slot_time _array_index)
        (if (or (<= (`|GetArrayItem` _slot_time _array_index) 0) (!= (`|GetArrayItem` (`self.Slot Items`) _array_index) (`local.L Item ID`)))
          (`KismetArrayLibrary.Array_Set` (`self.Slot Time`) _array_index (`.Time_13_0E4389D04B6ECEF5E382B59CEBFA9E62` (break `/Game/UltimateSurvivalPack/Blueprints/Structs/S_FinalResources` _value)) true :!label _label)
          (`KismetArrayLibrary.Array_Set` (`self.Slot Items`) _array_index (`local.L Item ID`) true))
        (else
          (goto _label)))
      (else
        (`KismetArrayLibrary.Array_Set` (`self.Slot Time`) _array_index 0 true)
        (`KismetArrayLibrary.Array_Set` (`self.Slot Items`) _array_index (`local.L Item ID`) true)))))

(fn `Get Interaction Data`
  (returns (`Interaction Text` :type Text))
  (return "Open Chest"))

(fn `Get Team ID`
  (returns (`Team ID` :type Byte))
  (return 0))

(fn `Has Fuel`
  (returns (`Item ID` :type Name) (Return :type Boolean))
  (locals (`L Found Item` :type "/Game/UltimateSurvivalPack/Blueprints/Structs/S_ItemFuel Structure"))
  (for _array_element (`/Game/UltimateSurvivalPack/Blueprints/Components/BP_MasterInventoryComponent.Inventory` (`self.BP_ChestInventoryComponent`))
    (bind ((`ID_2_1F4451EE4759095BA0D31BB237483A5E` _id)) (break `/Game/UltimateSurvivalPack/Blueprints/Structs/S_InventoryItem` _array_element))
    (bind (_value _returnvalue) (`BlueprintMapLibrary.Map_Find` (`self.Fuel Types`) _id))
    (set `local.L Found Item` _value)
    (if _returnvalue
      (if (>= (`/Game/UltimateSurvivalPack/Blueprints/Components/BP_MasterInventoryComponent.Find Items Amount` (`self.BP_ChestInventoryComponent`) _id) (`.Amount_11_25079F65431D59B667D8B3B5108CD890` (break `/Game/UltimateSurvivalPack/Blueprints/Structs/S_ItemFuel` (`local.L Found Item`))))
        (return _id true))))
  (return "None" false))

(fn `Local Can Overlap`
  (returns (Success :type Boolean))
  (return false))

(fn `OnRep_Active`
  (`self.Toggle Rafinery Action` (`self.Active`)))

(fn `Save Rafinery Progress`
  (locals (`L Float` :type "Array of Float (double-precision)") (`L String` :type "Array of String"))
  (bind _returnvalue (`self.GetComponentByClass` "/Game/UltimateSurvivalPack/Blueprints/Buildings/Parent/BP_BuildingComponent.BP_BuildingComponent_C"))
  (bind _build_id (`/Game/UltimateSurvivalPack/Blueprints/Buildings/Parent/BP_BuildingComponent.Build ID` _returnvalue))
  (`KismetArrayLibrary.Array_Add` (`local.L Float`) (`KismetMathLibrary.Conv_IntToDouble` (`self.Current Fuel Time`)))
  (for _array_element (`self.Slot Time`)
    (`KismetArrayLibrary.Array_Add` (`local.L Float`) (`KismetMathLibrary.Conv_IntToDouble` _array_element)))
  (for _array_element_2 (`self.Slot Items`)
    (`KismetArrayLibrary.Array_Add` (`local.L String`) (`KismetStringLibrary.Conv_NameToString` _array_element_2)))
  (`/Engine/EditorBlueprintResources/StandardMacros.IsValid` _returnvalue
    (:`Is Valid`
      (bind _assurvival_gamemode (cast `/Game/UltimateSurvivalPack/Blueprints/SurvivalGamemode` (`GameplayStatics.GetGameMode`)))
      (bind (_saved_data _returnvalue_2) (`/Game/UltimateSurvivalPack/Blueprints/SurvivalGamemode.Get Saved Build Data` _assurvival_gamemode _build_id))
      (if _returnvalue_2
        (bind ((`BuildData_2_700EB4E148DBEF7281188785324662CA` _builddata) (`Transform_6_227D833D45720C2C90F11EB731C1BBAA` _transform) (`OnAttachedActor_9_07069BCA4FEF9223D5BEC6BA5C09F0C5` _onattachedactor) (`WorldName_11_6840022640BD07C9638712B3FDD0588F` _worldname) (`CustomFloat_21_2B1EE62141F1CF01B611A4BB124FA5E8` _customfloat) (`CustomString_25_358AA98E4F4B4693E56F5CB4422E5AF2` _customstring) (`Cupboard_28_E77CCD52410AEBABC31F47A904A01FB2` _cupboard)) (break `/Game/UltimateSurvivalPack/Blueprints/Structs/S_BuildSave` _saved_data))
        (`/Game/UltimateSurvivalPack/Blueprints/SurvivalGamemode.Save Existing Building` _assurvival_gamemode _build_id (make `/Game/UltimateSurvivalPack/Blueprints/Structs/S_BuildSave` _builddata _transform _onattachedactor _worldname (`/Game/UltimateSurvivalPack/Blueprints/Components/BP_MasterInventoryComponent.Inventory` (`self.BP_ChestInventoryComponent`)) (`local.L Float`) (`local.L String`) _cupboard (`/Game/UltimateSurvivalPack/Blueprints/Buildings/Parent/BP_BuildingComponent.Health` _returnvalue)))))))

(fn `Update Slot Time`
  (locals (`L Item Index` :type Integer) (`L Item To Give` :type "Map of Name to Object Object Reference") (`L Updated` :type Boolean) (`L Item To Remove` :type "Map of Name to Object Object Reference"))
  (bind ((`Items_12_67D92B8E47B4EC356DBFF5ABED5F9F30` _items)) (break `/Game/UltimateSurvivalPack/Blueprints/Structs/S_FinalResources` (`BlueprintMapLibrary.Map_Find` (`self.Final Resource Types`) (`|GetArrayItem` (`self.Slot Items`) (`local.L Item Index`)))))
  (for (_array_element _array_index) (`self.Slot Time`)
    (if (> _array_element 0)
      (set `local.L Item Index` _array_index)
      (if (== _array_element 1)
        (`KismetArrayLibrary.Array_Set` (`self.Slot Time`) (`local.L Item Index`))
        ;[1 1 1] Item Finished
        (bind _keys (`BlueprintMapLibrary.Map_Keys` _items))
        (for _array_element_2 _keys
          (`BlueprintMapLibrary.Map_Add` (`local.L Item To Give`) _array_element_2 (+ (`BlueprintMapLibrary.Map_Find` _items _array_element_2) (`BlueprintMapLibrary.Map_Find` (`local.L Item To Give`) _array_element_2)))
          (set `local.L Updated` true))
        (`/Game/UltimateSurvivalPack/Blueprints/Components/BP_MasterInventoryComponent.Remove Item` (`self.BP_ChestInventoryComponent`) (`local.L Item Index`) 1 (`self.BP_ChestInventoryComponent`))
        (else
          (`KismetArrayLibrary.Array_Set` (`self.Slot Time`) (`local.L Item Index`) (- (`|GetArrayItem` (`self.Slot Time`) (`local.L Item Index`)) 1))))))
  (if (`local.L Updated`)
    (bind _keys_2 (`BlueprintMapLibrary.Map_Keys` (`local.L Item To Give`)))
    (for _array_element_3 _keys_2
      (`/Game/UltimateSurvivalPack/Blueprints/Components/BP_MasterInventoryComponent.Add Item or Drop` (`self.BP_ChestInventoryComponent`) _array_element_3 (`BlueprintMapLibrary.Map_Find` (`local.L Item To Give`) _array_element_3) (`SceneComponent.K2_GetComponentLocation` (`self.Drop Location`)) false))
    (`/Game/UltimateSurvivalPack/Blueprints/Components/BP_ChestInventoryComponent.Update All Clients Inventory` (`self.BP_ChestInventoryComponent`))))

(fn `UserConstructionScript`)