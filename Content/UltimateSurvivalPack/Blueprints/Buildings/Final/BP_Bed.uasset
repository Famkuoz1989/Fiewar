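; Placeable bed building that lets a player set a new respawn point by interacting with it.
; Interaction writes a point above the bed and the building's BuildID into that player's GameInstance save entry, then persists it through the inventory component.
; A client notification follows via the leveling component, even if no building component is found.
; Selection toggles a custom depth stencil on the mesh for highlighting.
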(event `/Game/UltimateSurvivalPack/Blueprints/Interface/BPI_InventorySystem.On Interacted`
  (params (Executor :type "Controller Object Reference"))
  (`self.Set New Respawn Point` Executor)
  (`/Game/UltimateSurvivalPack/Blueprints/Components/BP_Player_ExperienceComponent.CLIENT Add Notification` (`/Game/UltimateSurvivalPack/Blueprints/BFL_UMSPack.Get Leveling Component` Executor) (make `/Game/UltimateSurvivalPack/Blueprints/Structs/S_Notification` "Respawn Point" "You have set new respawn point")))

(event `/Game/UltimateSurvivalPack/Blueprints/Interface/BPI_InventorySystem.Toggle Selected`
  (params (Toggle :type Boolean))
  (bind _staticmesh (`self.StaticMesh`))
  (bind _staticmesh_2 (`self.StaticMesh`))
  (if Toggle
    (`PrimitiveComponent.SetRenderCustomDepth` _staticmesh_2 true)
    (`PrimitiveComponent.SetCustomDepthStencilValue` _staticmesh_2 1)
    (else
      (`PrimitiveComponent.SetRenderCustomDepth` _staticmesh false)
      (`PrimitiveComponent.SetCustomDepthStencilValue` _staticmesh 0))))

(fn `Get Interaction Data`
  (returns (`Interaction Text` :type Text))
  (return "Set Respawn Point"))

(fn `Get Team ID`
  (returns (`Team ID` :type Byte))
  (return 0))

(fn `Local Can Overlap`
  (returns (Success :type Boolean))
  (return false))

(fn `Set New Respawn Point`
  (params (Controller :type "Actor Object Reference"))
  (bind _returnvalue (`self.GetComponentByClass` "/Game/UltimateSurvivalPack/Blueprints/Buildings/Parent/BP_BuildingComponent.BP_BuildingComponent_C"))
  (bind _asplayer_controller (cast `PlayerController` Controller))
  (`/Engine/EditorBlueprintResources/StandardMacros.IsValid` _returnvalue
    (:`Is Valid`
      ;[1 1 1] Save Player Location
      (bind _asbp_game_instance_umsp (cast `/Game/UltimateSurvivalPack/Blueprints/BP_GameInstance_UMSP` (`GameplayStatics.GetGameInstance`)))
      (bind _players_save (`/Game/UltimateSurvivalPack/Blueprints/Save/SAV_ServerData.Players Save` (`/Game/UltimateSurvivalPack/Blueprints/BP_GameInstance_UMSP.Player Save` _asbp_game_instance_umsp)))
      (bind _unique_id (`/Game/UltimateSurvivalPack/LobbySystem/Blueprints/BFL_LobbySystem.Get Player Unique ID` _asplayer_controller))
      (bind _structout (setmembers `/Game/UltimateSurvivalPack/Blueprints/Structs/S_PlayerSave` :`StructRef` (`BlueprintMapLibrary.Map_Find` _players_save _unique_id) :`Respawn Point` (+ (`self.K2_GetActorLocation`) (0.0 0.0 100.0)) :`Respawn Building` (`/Game/UltimateSurvivalPack/Blueprints/Buildings/Parent/BP_BuildingComponent.Build ID` _returnvalue)))
      (`BlueprintMapLibrary.Map_Add` _players_save _unique_id _structout)
      (`/Game/UltimateSurvivalPack/Blueprints/Components/BP_MasterInventoryComponent.Save Player Data` (`/Game/UltimateSurvivalPack/Blueprints/BFL_UMSPack.Get Inventory Component` _asplayer_controller)))))

(fn `UserConstructionScript`)