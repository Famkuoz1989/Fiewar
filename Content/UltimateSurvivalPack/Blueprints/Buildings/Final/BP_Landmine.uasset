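; Landmine building that explodes when a player overlaps it or a bullet hits it.
; The PlayerOverlap trigger is destroyed on clients to save collision cost, so only the server detonates on overlap.
; Point damage runs the parent handler first and detonates only for the bullet damage type.
; Both triggers share one path that spawns a scaled-up BP_Explosion just above the mine and destroys the actor.
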(event `self.ReceiveBeginPlay`
  ;[1 1 1] Save collision performance on client
  (`/Engine/EditorBlueprintResources/ActorMacros.Switch Has Authority`
    (:`Remote`
      (`ActorComponent.K2_DestroyComponent` (`self.Player Overlap`)))))

(event `self.ReceivePointDamage`
  (params (Damage :type "Float (single-precision)") (DamageType :type "DamageType Object Reference") (HitLocation :type "Vector Structure") (HitNormal :type "Vector Structure") (HitComponent :type "PrimitiveComponent Object Reference") (BoneName :type Name) (ShotFromDirection :type "Vector Structure") (InstigatedBy :type "Controller Object Reference") (DamageCauser :type "Actor Object Reference") (HitInfo :type "HitResult Structure (by ref)"))
  ;[1 1 1] Make Explosion
  (`parent.ReceivePointDamage` Damage DamageType HitLocation HitNormal HitComponent BoneName ShotFromDirection InstigatedBy DamageCauser HitInfo)
  (cast `/Game/UltimateSurvivalPack/Blueprints/DamageType/DT_Bullet` DamageType)
  (`|SpawnActorFromClass` "/Game/UltimateSurvivalPack/Blueprints/Holdable/Others/BP_Explosion.BP_Explosion_C" (`KismetMathLibrary.MakeTransform` (+ (`self.K2_GetActorLocation`) (0.0 0.0 10.0)) (struct) (5.0 5.0 5.0)) "Undefined" "OverrideRootScale" null null :!label _label)
  (`self.K2_DestroyActor`))

(event `self.Player Overlap.OnComponentBeginOverlap`
  (params (OverlappedComponent :type "PrimitiveComponent Object Reference") (OtherActor :type "Actor Object Reference") (OtherComp :type "PrimitiveComponent Object Reference") (OtherBodyIndex :type Integer) (bFromSweep :type Boolean) (SweepResult :type "HitResult Structure (by ref)"))
  ;[1 1 1] Make Explosion
  (`/Engine/EditorBlueprintResources/ActorMacros.Switch Has Authority`
    (:`Authority`
      (goto _label))))

(fn `UserConstructionScript`)