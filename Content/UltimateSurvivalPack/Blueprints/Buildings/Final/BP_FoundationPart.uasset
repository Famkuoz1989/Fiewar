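; Square foundation building part for the survival pack's building system, defining where other parts can attach to it.
; Each getter returns hardcoded transforms, one per side, for adjacent foundations, floors, angled variants, walls and roofs, plus a single centered ground point.
; Floors, walls and roofs sit raised above the origin while neighboring foundations stay level; special locations return nothing.
; It also reports its part type; the event graph and construction script are empty.
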(fn `Get Angled Floor Locations`
  (returns (Locations :type "Array of Transform Structure"))
  (return (`|MakeArray` (`KismetMathLibrary.MakeTransform` (0.0 -197.5 50.0)) (`KismetMathLibrary.MakeTransform` (197.5 0.0 50.0) (struct :`Yaw` 90.0)) (`KismetMathLibrary.MakeTransform` (0.0 197.5 50.0) (struct :`Yaw` 180.0)) (`KismetMathLibrary.MakeTransform` (-197.5 0.0 50.0) (struct :`Yaw` 270.0)))))

(fn `Get Angled Foundation Locations`
  (returns (Locations :type "Array of Transform Structure"))
  (return (`|MakeArray` (`KismetMathLibrary.MakeTransform` (0.0 -197.5 0.0)) (`KismetMathLibrary.MakeTransform` (197.5 0.0 0.0) (struct :`Yaw` 90.0)) (`KismetMathLibrary.MakeTransform` (0.0 197.5 0.0) (struct :`Yaw` 180.0)) (`KismetMathLibrary.MakeTransform` (-197.5 0.0 0.0) (struct :`Yaw` 270.0)))))

(fn `Get Floor Locations`
  (returns (Locations :type "Array of Transform Structure"))
  (return (`|MakeArray` (`KismetMathLibrary.MakeTransform` (250.0 0.0 50.0)) (`KismetMathLibrary.MakeTransform` (0.0 -250.0 50.0)) (`KismetMathLibrary.MakeTransform` (-250.0 0.0 50.0)) (`KismetMathLibrary.MakeTransform` (0.0 250.0 50.0)))))

(fn `Get Foundation Locations`
  (returns (Locations :type "Array of Transform Structure"))
  (return (`|MakeArray` (`KismetMathLibrary.MakeTransform` (250.0 0.0 0.0)) (`KismetMathLibrary.MakeTransform` (0.0 250.0 0.0)) (`KismetMathLibrary.MakeTransform` (-250.0 0.0 0.0) (struct :`Yaw` 180.0)) (`KismetMathLibrary.MakeTransform` (0.0 -250.0 0.0)))))

(fn `Get Ground Locations`
  (returns (Locations :type "Array of Transform Structure"))
  (return (`|MakeArray` (`KismetMathLibrary.MakeTransform` (0.0 0.0 50.0)) :!type "Transform Structure")))

(fn `Get Part Type`
  (returns (`Building Part` :type "/Game/UltimateSurvivalPack/Blueprints/Enum/E_BuildingPart Enum"))
  (return "NewEnumerator0"))

(fn `Get Roof Locations`
  (returns (Locations :type "Array of Transform Structure"))
  (return (`|MakeArray` (`KismetMathLibrary.MakeTransform` (125.0 0.0 50.0)) (`KismetMathLibrary.MakeTransform` (0.0 125.0 50.0) (struct :`Yaw` 90.0)) (`KismetMathLibrary.MakeTransform` (-125.0 0.0 50.0) (struct :`Yaw` 180.0)) (`KismetMathLibrary.MakeTransform` (0.0 -125.0 50.0) (struct :`Yaw` -90.0)))))

(fn `Get Special Locations`
  (returns (Locations :type "Array of Transform Structure"))
  (return))

(fn `Get Wall Locations`
  (returns (Locations :type "Array of Transform Structure"))
  (return (`|MakeArray` (`KismetMathLibrary.MakeTransform` (125.0 0.0 50.0) (struct :`Yaw` 180.0)) (`KismetMathLibrary.MakeTransform` (0.0 125.0 50.0) (struct :`Yaw` -90.0)) (`KismetMathLibrary.MakeTransform` (-125.0 0.0 50.0)) (`KismetMathLibrary.MakeTransform` (0.0 -125.0 50.0) (struct :`Yaw` 90.0)))))

(fn `UserConstructionScript`)