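; Interactable wooden door for the survival building system that swings its mesh open and closed with a timeline.
; Interaction checks cupboard access through the parent actor's building component, allowing anyone if that component is absent, then flips DoorStatus.
; DoorStatus's OnRep plays or reverses the swing, with a DoOnce blocking re-triggering until the server resets it when the animation finishes.
; It also supplies the Open/Close prompt and highlights via custom depth when selected.
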(event `self.ReceiveBeginPlay`
  (`self.Toggle Doors` (`self.Door Status`)))

(event `Toggle Doors`
  (params (Toggle :type Boolean))
  (if Toggle
    (bind (_direction _alpha) (`Timeline|Door Animation` :!label _label)
      (:`Update`
        (`SceneComponent.K2_SetRelativeRotation` (`self.StaticMesh`) (`KismetMathLibrary.MakeRotator` 0.0 0.0 (* _alpha 90.0)) false false))
      (:`Finished`
        (`/Engine/EditorBlueprintResources/ActorMacros.Switch Has Authority`
          (:`Authority`
            (`self.Reset`)))))
    (else
      (goto _label :!via `Reverse`))))

(event `/Game/UltimateSurvivalPack/Blueprints/Interface/BPI_InventorySystem.On Interacted`
  (params (Executor :type "Controller Object Reference"))
  (`self.Can Access` Executor
    (:`True`
      (`/Engine/EditorBlueprintResources/StandardMacros.DoOnce` false :!label _label_2
        (:`Completed`
          (set `self.Door Status` (not (`self.Door Status`))))))))

(event `Reset`
  (goto _label_2 :!via `Reset`))

(event `/Game/UltimateSurvivalPack/Blueprints/Interface/BPI_InventorySystem.Toggle Selected`
  (params (Toggle :type Boolean))
  (bind _staticmesh (`self.StaticMesh`))
  (bind _staticmesh_2 (`self.StaticMesh`))
  (if Toggle
    (`PrimitiveComponent.SetRenderCustomDepth` _staticmesh_2 true)
    (`PrimitiveComponent.SetCustomDepthStencilValue` _staticmesh_2 1)
    (else
      (`PrimitiveComponent.SetRenderCustomDepth` _staticmesh false)
      (`PrimitiveComponent.SetCustomDepthStencilValue` _staticmesh 0))))

(fn `Get Interaction Data`
  (returns (`Interaction Text` :type Text))
  (return (select `bool` (`self.Door Status`) :`false` "Open Door" :`true` "Close Door" :!type "Text")))

(fn `Get Team ID`
  (returns (`Team ID` :type Byte))
  (return 0))

(fn `Local Can Overlap`
  (returns (Success :type Boolean))
  (return false))

(fn `OnRep_Door Status`
  (`self.Toggle Doors` (`self.Door Status`)))

(fn `UserConstructionScript`)