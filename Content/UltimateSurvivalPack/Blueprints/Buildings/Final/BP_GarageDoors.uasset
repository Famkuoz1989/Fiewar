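; Interactable garage door for the building system that swings open and closed on a timeline-driven pitch rotation.
; Interaction checks cupboard access on the parent's building component, then flips DoorStatus, whose OnRep plays or reverses the animation.
; A DoOnce blocks repeat toggles until the animation finishes on authority, and a box trace prevents closing onto vehicles.
; Collision is disabled during movement, and selection highlights the mesh through custom depth stencil.
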(event `Toggle Doors`
  (params (Toggle :type Boolean))
  (`PrimitiveComponent.SetCollisionEnabled` (`self.StaticMesh`) "NoCollision")
  (if Toggle
    (bind (_direction _alpha) (`Timeline|Door Animation` :!label _label)
      (:`Update`
        (`SceneComponent.K2_SetRelativeRotation` (`self.StaticMesh`) (`KismetMathLibrary.MakeRotator` 0.0 (* _alpha -110.0)) false false))
      (:`Finished`
        (`/Engine/EditorBlueprintResources/ActorMacros.Switch Has Authority`
          (:`Authority`
            (`self.Reset`))
          (:`Remote`
            _))
        (`PrimitiveComponent.SetCollisionEnabled` (`self.StaticMesh`) "QueryAndPhysics")))
    (else
      (goto _label :!via `Reverse`))))

(event `/Game/UltimateSurvivalPack/Blueprints/Interface/BPI_InventorySystem.On Interacted`
  (params (Executor :type "Controller Object Reference"))
  (bind _returnvalue (`self.K2_GetActorLocation`))
  (`self.Can Access` Executor
    (:`True`
      (`/Engine/EditorBlueprintResources/StandardMacros.DoOnce` false :!label _label_2
        (:`Completed`
          (if (`self.Door Status`)
            (bind (_outhit _returnvalue_2) (`KismetSystemLibrary.BoxTraceSingleForObjects` _returnvalue (- _returnvalue (0.0 0.0 215.0)) (21.0 150.0 0.0) (`self.K2_GetActorRotation`) (`|MakeArray` "ObjectTypeQuery5" :!type "EObjectTypeQuery Enum")))
            (if _returnvalue_2
              (`self.Reset`)
              (else
                (set `self.Door Status` (not (`self.Door Status`)) :!label _label_3)))
            (else
              (goto _label_3))))))))

(event `Reset`
  (goto _label_2 :!via `Reset`))

(event `/Game/UltimateSurvivalPack/Blueprints/Interface/BPI_InventorySystem.Toggle Selected`
  (params (Toggle :type Boolean))
  (bind _staticmesh (`self.StaticMesh`))
  (bind _staticmesh_2 (`self.StaticMesh`))
  (if Toggle
    (`PrimitiveComponent.SetRenderCustomDepth` _staticmesh_2 true)
    (`PrimitiveComponent.SetCustomDepthStencilValue` _staticmesh_2 1)
    (else
      (`PrimitiveComponent.SetRenderCustomDepth` _staticmesh false)
      (`PrimitiveComponent.SetCustomDepthStencilValue` _staticmesh 0))))

(fn `Get Interaction Data`
  (returns (`Interaction Text` :type Text))
  (return (select `bool` (`self.Door Status`) :`false` "Open Door" :`true` "Close Door" :!type "Text")))

(fn `Get Team ID`
  (returns (`Team ID` :type Byte))
  (return 0))

(fn `Local Can Overlap`
  (returns (Success :type Boolean))
  (return false))

(fn `OnRep_Door Status`
  (`self.Toggle Doors` (`self.Door Status`)))

(fn `UserConstructionScript`)