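; Angled (triangular) foundation piece for the survival pack's building system, defining where other parts can attach to it.
; Getter functions report its part type and return three hardcoded transforms, one per side, for each neighbour type: square and angled foundations, floors, walls and roofs.
; Foundations attach at base height, while floors, walls and roofs sit raised above it.
; Ground and special locations return nothing, and the event graph and construction script are empty.
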(fn `Get Angled Floor Locations`
  (returns (Locations :type "Array of Transform Structure"))
  (return (`|MakeArray` (`KismetMathLibrary.MakeTransform` (-125.5 -72.5 50.0) (struct :`Yaw` -60.0)) (`KismetMathLibrary.MakeTransform` (125.5 -72.5 50.0) (struct :`Yaw` 60.0)) (`KismetMathLibrary.MakeTransform` (0.0 145.0 50.0) (struct :`Yaw` 180.0)))))

(fn `Get Angled Foundation Locations`
  (returns (Locations :type "Array of Transform Structure"))
  (return (`|MakeArray` (`KismetMathLibrary.MakeTransform` (-125.5 -72.5 0.0) (struct :`Yaw` -60.0)) (`KismetMathLibrary.MakeTransform` (125.5 -72.5 0.0) (struct :`Yaw` 60.0)) (`KismetMathLibrary.MakeTransform` (0.0 145.0 0.0) (struct :`Yaw` 180.0)))))

(fn `Get Floor Locations`
  (returns (Locations :type "Array of Transform Structure"))
  (return (`|MakeArray` (`KismetMathLibrary.MakeTransform` (-170.5 -98.5 50.0) (struct :`Yaw` -60.0)) (`KismetMathLibrary.MakeTransform` (0.0 197.5 50.0)) (`KismetMathLibrary.MakeTransform` (172.5 -97.5 50.0) (struct :`Yaw` -30.0)))))

(fn `Get Foundation Locations`
  (returns (Locations :type "Array of Transform Structure"))
  (return (`|MakeArray` (`KismetMathLibrary.MakeTransform` (-170.5 -98.5 0.0) (struct :`Yaw` -60.0)) (`KismetMathLibrary.MakeTransform` (0.0 197.5 0.0)) (`KismetMathLibrary.MakeTransform` (172.5 -97.5 0.0) (struct :`Yaw` 60.0)))))

(fn `Get Ground Locations`
  (returns (Locations :type "Array of Transform Structure"))
  (return))

(fn `Get Part Type`
  (returns (`Building Part` :type "/Game/UltimateSurvivalPack/Blueprints/Enum/E_BuildingPart Enum"))
  (return "NewEnumerator7"))

(fn `Get Roof Locations`
  (returns (Locations :type "Array of Transform Structure"))
  (return (`|MakeArray` (`KismetMathLibrary.MakeTransform` (0.0 70.0 50.0) (struct :`Yaw` 90.0)) (`KismetMathLibrary.MakeTransform` (60.5 -35.0 50.0) (struct :`Yaw` -30.0)) (`KismetMathLibrary.MakeTransform` (-60.5 -35.0 50.0) (struct :`Yaw` -150.0)))))

(fn `Get Special Locations`
  (returns (Locations :type "Array of Transform Structure"))
  (return))

(fn `Get Wall Locations`
  (returns (Locations :type "Array of Transform Structure"))
  (return (`|MakeArray` (`KismetMathLibrary.MakeTransform` (0.0 70.0 50.0) (struct :`Yaw` -90.0)) (`KismetMathLibrary.MakeTransform` (60.5 -35.0 50.0) (struct :`Yaw` 150.0)) (`KismetMathLibrary.MakeTransform` (-60.5 -35.0 50.0) (struct :`Yaw` 30.0)))))

(fn `UserConstructionScript`)