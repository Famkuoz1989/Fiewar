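; Parent Blueprint for harvestable buildings that grow through staged meshes and can be harvested or destroyed.
; Growth uses actor lifespan: on expiry, the authority spawns the same class at the next stage, transferring building component data.
; Interacting at the final stage scatters chance-rolled item drops; earlier interaction just destroys it, and both remove the saved building.
; Stage and elapsed growth time persist through SurvivalGamemode build saves.
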(event `self.ReceiveBeginPlay`
  (bind _returnvalue (`self.GetComponentByClass` "/Game/UltimateSurvivalPack/Blueprints/Buildings/Parent/BP_BuildingComponent.BP_BuildingComponent_C"))
  (bind ((`HarvestableStages_3_6500A21C48D3CEBEB49AFA8AF2653873` _harvestablestages)) (break `/Game/UltimateSurvivalPack/Blueprints/Structs/S_HarvestableData` (`self.Harvestable Data`)))
  (bind _build_id (`/Game/UltimateSurvivalPack/Blueprints/Buildings/Parent/BP_BuildingComponent.Build ID` _returnvalue))
  ;[1 1 1] Set Life Span
  (`KismetSystemLibrary.Delay` 0.0)
  (`self.Load Stage` (`self.Current Stage`))
  (`/Engine/EditorBlueprintResources/ActorMacros.Switch Has Authority`
    (:`Authority`
      (if (<= (`KismetArrayLibrary.Array_LastIndex` _harvestablestages) (`self.Current Stage`))
        ;[1 1 1] Save Last Stage Harvestable
        (`/Engine/EditorBlueprintResources/StandardMacros.IsValid` _returnvalue
          (:`Is Valid`
            (bind _assurvival_gamemode (cast `/Game/UltimateSurvivalPack/Blueprints/SurvivalGamemode` (`GameplayStatics.GetGameMode`)))
            (bind (_saved_data _returnvalue_2) (`/Game/UltimateSurvivalPack/Blueprints/SurvivalGamemode.Get Saved Build Data` _assurvival_gamemode _build_id))
            (if _returnvalue_2
              ;;[1 1 1] Save Data
              (bind _structout (setmembers `/Game/UltimateSurvivalPack/Blueprints/Structs/S_BuildSave` :`StructRef` _saved_data :`Custom Float` (`|MakeArray` (`KismetMathLibrary.Conv_IntToDouble` (`self.Current Stage`)) 0.0 :!type "Float (single-precision)")))
              (`/Game/UltimateSurvivalPack/Blueprints/SurvivalGamemode.Save Existing Building` _assurvival_gamemode _build_id _structout))))
        (else
          (`self.SetLifeSpan` (`KismetMathLibrary.FClamp` (- (`KismetMathLibrary.Conv_IntToDouble` (`.GrowthTime_5_B8A89A414F14770DA75F77A924154985` (break `/Game/UltimateSurvivalPack/Blueprints/Structs/S_HarvestableStages` (`|GetArrayItem` _harvestablestages (`self.Current Stage`))))) (`self.Saved Time`)) 1.0 9999999.0)))))))

(event `/Game/UltimateSurvivalPack/Blueprints/Interface/BPI_InventorySystem.Toggle Selected`
  (params (Toggle :type Boolean))
  (bind _staticmesh (`self.StaticMesh`))
  (bind _staticmesh_2 (`self.StaticMesh`))
  ;[1 1 1] On Selected
  (if Toggle
    (`PrimitiveComponent.SetRenderCustomDepth` _staticmesh_2 true)
    (`PrimitiveComponent.SetCustomDepthStencilValue` _staticmesh_2 1)
    (else
      (`PrimitiveComponent.SetRenderCustomDepth` _staticmesh false)
      (`PrimitiveComponent.SetCustomDepthStencilValue` _staticmesh 0))))

(event `/Game/UltimateSurvivalPack/Blueprints/Interface/BPI_InventorySystem.On Interacted`
  (params (Executor :type "Controller Object Reference"))
  (bind (_harvestablestages _itemstodrop) (break `/Game/UltimateSurvivalPack/Blueprints/Structs/S_HarvestableData` (`self.Harvestable Data`)))
  (`/Engine/EditorBlueprintResources/StandardMacros.DoOnce` false
    (:`Completed`
      (if (>= (`self.Current Stage`) (`KismetArrayLibrary.Array_LastIndex` _harvestablestages))
        (`self.Drop Items` _itemstodrop)
        (`self.K2_DestroyActor`)
        (else
          (set `self.Force Destroy` true)
          (`self.K2_DestroyActor`))))))

(event `self.ReceiveDestroyed`
  (bind _returnvalue (`self.GetComponentByClass` "/Game/UltimateSurvivalPack/Blueprints/Buildings/Parent/BP_BuildingComponent.BP_BuildingComponent_C"))
  (bind _returnvalue_2 (`self.GetComponentByClass` "/Game/UltimateSurvivalPack/Blueprints/Buildings/Parent/BP_BuildingComponent.BP_BuildingComponent_C"))
  (bind _build_id (`/Game/UltimateSurvivalPack/Blueprints/Buildings/Parent/BP_BuildingComponent.Build ID` _returnvalue))
  ;[1 1 1] Event Destroyed
  (`/Engine/EditorBlueprintResources/ActorMacros.Switch Has Authority`
    (:`Authority`
      (if (not (`self.Force Destroy`))
        (if (< (`self.Current Stage`) (`KismetArrayLibrary.Array_LastIndex` (`.HarvestableStages_3_6500A21C48D3CEBEB49AFA8AF2653873` (break `/Game/UltimateSurvivalPack/Blueprints/Structs/S_HarvestableData` (`self.Harvestable Data`)))))
          (bind _returnvalue_3 (`|SpawnActorFromClass` (`GameplayStatics.GetObjectClass` self) (`self.GetTransform`) "Undefined" "SelectDefaultAtRuntime" null (+ (`self.Current Stage`) 1) 0.0 null))
          ;[1 1 1] Add Build Component From Old Component
          (bind _returnvalue_4 (`AddComponent|NODE_AddBP_BuildingComponent-0` :`self` _returnvalue_3))
          (set `/Game/UltimateSurvivalPack/Blueprints/Buildings/Parent/BP_BuildingComponent.Build ID` _build_id _returnvalue_4)
          (set `/Game/UltimateSurvivalPack/Blueprints/Buildings/Parent/BP_BuildingComponent.Build Data` (`/Game/UltimateSurvivalPack/Blueprints/Buildings/Parent/BP_BuildingComponent.Build Data` _returnvalue) _returnvalue_4)
          (set `/Game/UltimateSurvivalPack/Blueprints/Buildings/Parent/BP_BuildingComponent.Attached Actors` (`/Game/UltimateSurvivalPack/Blueprints/Buildings/Parent/BP_BuildingComponent.Attached Actors` _returnvalue) _returnvalue_4)
          ;[1 1 1] Reference New Actor
          (bind _assurvival_gamemode (cast `/Game/UltimateSurvivalPack/Blueprints/SurvivalGamemode` (`GameplayStatics.GetGameMode`)))
          (`BlueprintMapLibrary.Map_Add` (`/Game/UltimateSurvivalPack/Blueprints/SurvivalGamemode.Building Actors` _assurvival_gamemode) _build_id _returnvalue_3)
          (else
            ;[1 1 1] Remove Building From Save
            (`/Engine/EditorBlueprintResources/StandardMacros.IsValid` _returnvalue_2 :!label _label
              (:`Is Valid`
                (bind _assurvival_gamemode_2 (cast `/Game/UltimateSurvivalPack/Blueprints/SurvivalGamemode` (`GameplayStatics.GetGameMode`)))
                (`/Game/UltimateSurvivalPack/Blueprints/SurvivalGamemode.Remove Building` _assurvival_gamemode_2 (`/Game/UltimateSurvivalPack/Blueprints/Buildings/Parent/BP_BuildingComponent.Build ID` _returnvalue_2))))))
        (else
          (goto _label))))))

(event `self.ReceiveEndPlay`
  (params (EndPlayReason :type "EEndPlayReason Enum" :default "Destroyed"))
  (bind _returnvalue (`self.GetComponentByClass` "/Game/UltimateSurvivalPack/Blueprints/Buildings/Parent/BP_BuildingComponent.BP_BuildingComponent_C"))
  (bind _build_id (`/Game/UltimateSurvivalPack/Blueprints/Buildings/Parent/BP_BuildingComponent.Build ID` _returnvalue))
  (switch `EEndPlayReason` EndPlayReason
    (:`LevelTransition`
      _)
    (:`EndPlayInEditor`
      _)
    (:`Quit`
      _))
  (`/Engine/EditorBlueprintResources/StandardMacros.IsValid` _returnvalue
    (:`Is Valid`
      (bind _assurvival_gamemode (cast `/Game/UltimateSurvivalPack/Blueprints/SurvivalGamemode` (`GameplayStatics.GetGameMode`)))
      (bind (_saved_data _returnvalue_2) (`/Game/UltimateSurvivalPack/Blueprints/SurvivalGamemode.Get Saved Build Data` _assurvival_gamemode _build_id))
      (if _returnvalue_2
        ;[1 1 1] Save Data
        (bind _structout (setmembers `/Game/UltimateSurvivalPack/Blueprints/Structs/S_BuildSave` :`StructRef` _saved_data :`Custom Float` (`|MakeArray` (`KismetMathLibrary.Conv_IntToDouble` (`self.Current Stage`)) (+ (`self.GetGameTimeSinceCreation`) (`self.Saved Time`)) :!type "Float (single-precision)")))
        (`/Game/UltimateSurvivalPack/Blueprints/SurvivalGamemode.Save Existing Building Directly` _assurvival_gamemode _build_id _structout)))))

(fn `Drop Items`
  (params (Array :type "Array of /Game/UltimateSurvivalPack/Blueprints/Structs/S_DropItem Structure"))
  (for _array_element Array
    (bind (_itemid _minimumamount _maximumamount _chanceofspawning) (break `/Game/UltimateSurvivalPack/Blueprints/Structs/S_DropItem` _array_element))
    (if (<= (`KismetMathLibrary.RandomFloatInRange` 0.0 100.0) _chanceofspawning)
      (bind _returnvalue (`|SpawnActorFromClass` "/Game/UltimateSurvivalPack/Blueprints/BP_InventoryItem.BP_InventoryItem_C" (`KismetMathLibrary.MakeTransform` (+ (`KismetSystemLibrary.GetComponentBounds` (`self.StaticMesh`)) (0.0 0.0 10.0)) (.rotation (`self.GetTransform`)) (.scale (`self.GetTransform`))) "Undefined" "OverrideRootScale" null (make `/Game/UltimateSurvivalPack/Blueprints/Structs/S_InventoryItem` _itemid (`KismetMathLibrary.RandomIntegerInRange` _minimumamount _maximumamount) -1) null null))
      (`PrimitiveComponent.AddImpulse` (`/Game/UltimateSurvivalPack/Blueprints/BP_InventoryItem.Item Mesh` _returnvalue) (* (`KismetMathLibrary.RandomUnitVector`) (`KismetMathLibrary.RandomFloatInRange` 75.0 150.0)) "None" true))))

(fn `Get Interaction Data`
  (returns (`Interaction Text` :type Text))
  (if (>= (`self.Current Stage`) (`KismetArrayLibrary.Array_LastIndex` (`.HarvestableStages_3_6500A21C48D3CEBEB49AFA8AF2653873` (break `/Game/UltimateSurvivalPack/Blueprints/Structs/S_HarvestableData` (`self.Harvestable Data`)))))
    (return (`|FormatText` "Harvest {Name}" (`self.Name`)))
    (else
      (return (`|FormatText` "Destroy {Name}" (`self.Name`))))))

(fn `Get Team ID`
  (returns (`Team ID` :type Byte))
  (return 0))

(fn `Load Stage`
  (params (Stage :type Integer))
  (`StaticMeshComponent.SetStaticMesh` (`self.StaticMesh`) (`.Mesh_2_0A8788E245A70711D7885D99C17B05F7` (break `/Game/UltimateSurvivalPack/Blueprints/Structs/S_HarvestableStages` (`|GetArrayItem` (`.HarvestableStages_3_6500A21C48D3CEBEB49AFA8AF2653873` (break `/Game/UltimateSurvivalPack/Blueprints/Structs/S_HarvestableData` (`self.Harvestable Data`))) Stage)))))

(fn `Local Can Overlap`
  (returns (Success :type Boolean))
  (return false))

(fn `UserConstructionScript`)