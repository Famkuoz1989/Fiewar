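; Environment harvestable that drops items and awards skill experience when interacted with, then regrows after a delay.
; Interaction sets the replicated IsGrowing flag and clears it after the first stage's growth time, flushing net dormancy on both changes.
; Its OnRep hides the plant by clearing the mesh with impact particles and sound, or restores the first stage's mesh.
; BeginPlay loads stage zero or clears the mesh according to that flag.
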(event `self.ReceiveBeginPlay`
  ;[1 1 1] Begin Play Load
  (if (not (`self.Is Growing`))
    (`self.Load Stage` 0)
    (else
      (`StaticMeshComponent.SetStaticMesh` (`self.StaticMesh`) null))))

(event `/Game/UltimateSurvivalPack/Blueprints/Interface/BPI_InventorySystem.On Interacted`
  (params (Executor :type "Controller Object Reference"))
  ;[1 1 1] On Interacted
  (if (not (`self.Is Growing`))
    ;;[1 1 1] Drop Items
    (`self.Drop Items` (`.ItemsToDrop_11_D6FCA423474F33007BCD3FB01B4B586E` (break `/Game/UltimateSurvivalPack/Blueprints/Structs/S_HarvestableData` (`self.Harvestable Data`))))
    ;;[1 1 1] Add Skill Epxperience
    (`/Game/UltimateSurvivalPack/Blueprints/Components/BP_SkillTreeComponent.Add Experience` (`/Game/UltimateSurvivalPack/Blueprints/BFL_UMSPack.Get Skill Component` Executor) "NewEnumerator0" 75)
    ;;[1 1 1] Update And Replicate
    (set `self.Is Growing` true)
    (`self.FlushNetDormancy`)
    (`KismetSystemLibrary.Delay` (`KismetMathLibrary.Conv_IntToDouble` (`.GrowthTime_5_B8A89A414F14770DA75F77A924154985` (break `/Game/UltimateSurvivalPack/Blueprints/Structs/S_HarvestableStages` (`|GetArrayItem` (`.HarvestableStages_3_6500A21C48D3CEBEB49AFA8AF2653873` (break `/Game/UltimateSurvivalPack/Blueprints/Structs/S_HarvestableData` (`self.Harvestable Data`))))))))
    (set `self.Is Growing` false)
    (`self.FlushNetDormancy`)))

(fn `OnRep_Is Growing`
  (bind _returnvalue (+ (`self.K2_GetActorLocation`) (0.0 0.0 35.0)))
  (if (`self.Is Growing`)
    (`StaticMeshComponent.SetStaticMesh` (`self.StaticMesh`) null)
    (`GameplayStatics.SpawnEmitterAtLocation` "/Game/UltimateSurvivalPack/Demo/Particles/P_ImpactStuff.P_ImpactStuff" _returnvalue (struct) (1.0 1.0 1.0) true "AutoRelease")
    (`GameplayStatics.PlaySoundAtLocation` "/Game/UltimateSurvivalPack/Demo/Audio/Impact/CUE_HitImpact.CUE_HitImpact" _returnvalue (struct) 1.0 1.0 0.0 "/Game/UltimateSurvivalPack/Blueprints/Attenuation/SA_Footsteps.SA_Footsteps" "/Game/UltimateSurvivalPack/Blueprints/Other/SC_Environment.SC_Environment" null null)
    (else
      (`StaticMeshComponent.SetStaticMesh` (`self.StaticMesh`) (`.Mesh_2_0A8788E245A70711D7885D99C17B05F7` (break `/Game/UltimateSurvivalPack/Blueprints/Structs/S_HarvestableStages` (`|GetArrayItem` (`.HarvestableStages_3_6500A21C48D3CEBEB49AFA8AF2653873` (break `/Game/UltimateSurvivalPack/Blueprints/Structs/S_HarvestableData` (`self.Harvestable Data`))))))))))

(fn `UserConstructionScript`
  (`parent.UserConstructionScript`))