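; Actor component for placed buildings that manages health, melee hit feedback, tool repairs, build/destroy effects and cupboard privilege checks.
; Non-harvestable owners bind damage and destruction events; surviving damage saves health through SurvivalGamemode, while zero health destroys the actor.
; On the server, destruction removes the building record, destroys attached buildings by ID, and clears linked respawn points and cupboard links.
; Smoke puffs scale with the owner's bounds.
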(event `self.ReceiveBeginPlay`
  (bind _returnvalue (`self.GetOwner`))
  ;[1 0.02604 0.02604] Harvestables have it's own Destroy Logic
  (cast `/Game/UltimateSurvivalPack/Blueprints/Buildings/Harvestable/Parent/BP_Harvestable` (`self.GetOwner`)
    (:`CastFailed`
      ;[1 1 1] Bind On Destroyed
      (add `Actor.OnDestroyed` _returnvalue (delegate `On Destroyed`))
      (add `Actor.OnTakeAnyDamage` _returnvalue (delegate `On Damaged`))
      (if (!= (`Actor.GetOwner` (`self.GetOwner`)) null)
        (`self.Spawn Build Emmiter`)
        (`GameplayStatics.SpawnSoundAtLocation` "/Game/UltimateSurvivalPack/Demo/Audio/SFX/CUE_Finish_Building.CUE_Finish_Building" (`Actor.K2_GetActorLocation` (`self.GetOwner`)) (struct) 1.0 1.0 0.0 "/Game/UltimateSurvivalPack/Blueprints/Attenuation/SA_Explosion.SA_Explosion" null)))))

(event `On Destroyed`
  (params (DestroyedActor :type "Actor Object Reference"))
  (`|ExecutionSequence`
    (:`then_0`
      (`self.Spawn Build Emmiter`)
      (`GameplayStatics.SpawnSoundAtLocation` "/Game/UltimateSurvivalPack/Demo/Audio/Impact/CUE_BuildingDestroyed.CUE_BuildingDestroyed" (`Actor.K2_GetActorLocation` (`self.GetOwner`)) (struct) 1.0 1.0 0.0 "/Game/UltimateSurvivalPack/Blueprints/Attenuation/SA_Explosion.SA_Explosion" null))
    (:`then_1`
      (if (`Actor.HasAuthority` DestroyedActor)
        ;[1 1 1] Remove Building
        (bind _assurvival_gamemode (cast `/Game/UltimateSurvivalPack/Blueprints/SurvivalGamemode` (`GameplayStatics.GetGameMode`)))
        (`/Game/UltimateSurvivalPack/Blueprints/SurvivalGamemode.Remove Building` _assurvival_gamemode (`self.Build ID`))
        ;[1 1 1] Destroy Attached Actors
        (for _array_element (`self.Attached Actors`)
          (bind _building_actors (`/Game/UltimateSurvivalPack/Blueprints/SurvivalGamemode.Building Actors` _assurvival_gamemode))
          (bind _value (`BlueprintMapLibrary.Map_Find` _building_actors _array_element))
          (`/Engine/EditorBlueprintResources/StandardMacros.IsValid` _value
            (:`Is Valid`
              (bind _asbp_harvestable (cast `/Game/UltimateSurvivalPack/Blueprints/Buildings/Harvestable/Parent/BP_Harvestable` _value) ; Force Destroy On Harvestables
                (:`then`
                  (set `/Game/UltimateSurvivalPack/Blueprints/Buildings/Harvestable/Parent/BP_Harvestable.Force Destroy` true _asbp_harvestable))
                (:`CastFailed`
                  _))
              (`Actor.K2_DestroyActor` _value)
              (`BlueprintMapLibrary.Map_Remove` _building_actors _array_element))))
        ;[1 0.4862 0.3355] Check for Additive Removal Components
        (`self.Check Respawnpoint Removal`)
        (`self.Check Cupboard Removal`)))))

(event `On Damaged`
  (params (DamagedActor :type "Actor Object Reference") (Damage :type "Float (single-precision)") (DamageType :type "DamageType Object Reference") (InstigatedBy :type "Controller Object Reference") (DamageCauser :type "Actor Object Reference"))
  (bind _returnvalue (`/Game/UltimateSurvivalPack/Blueprints/BFL_UMSPack.Get Inventory Component` InstigatedBy))
  (bind _returnvalue_2 (`Actor.K2_GetActorLocation` DamageCauser))
  (cast `/Game/UltimateSurvivalPack/Blueprints/DamageType/DT_Melee` DamageType
    (:`then`
      (`/Engine/EditorBlueprintResources/StandardMacros.IsValid` _returnvalue
        (:`Is Valid`
          (`/Game/UltimateSurvivalPack/Blueprints/Components/BP_PlayerInventoryComponent.Spawn Damage Widget` _returnvalue _returnvalue_2 Damage "None" null)
          (`self.MULTICAST Hit Effect` _returnvalue_2))
        (:`Is Not Valid`
          _)))
    (:`CastFailed`
      _))
  (`self.Handled Damage` Damage))

(event `MULTICAST Hit Effect`
  (params (Location :type "Vector Structure"))
  (`GameplayStatics.SpawnSoundAtLocation` "/Game/UltimateSurvivalPack/Demo/Audio/Impact/CUE_HitImpact.CUE_HitImpact" Location (struct) 1.0 1.0 0.0 null null))

(event `Set Cupboard`
  (params (`Cupboard ID` :type String))
  ;[0.1586 0.5606 1] Set New Cupboard
  (set `self.Cupboard ID` `Cupboard ID`)
  ;;[1 1 1] Save Data
  (bind _assurvival_gamemode (cast `/Game/UltimateSurvivalPack/Blueprints/SurvivalGamemode` (`GameplayStatics.GetGameMode`)))
  (bind (_saved_data _returnvalue) (`/Game/UltimateSurvivalPack/Blueprints/SurvivalGamemode.Get Saved Build Data` _assurvival_gamemode (`self.Build ID`)))
  (if _returnvalue
    (bind _structout (setmembers `/Game/UltimateSurvivalPack/Blueprints/Structs/S_BuildSave` :`StructRef` _saved_data :`Cupboard` (`self.Cupboard ID`)))
    (`/Game/UltimateSurvivalPack/Blueprints/SurvivalGamemode.Save Existing Building` _assurvival_gamemode (`self.Build ID`) _structout)))

(event `SERVER Repair`
  (params (`Repair Tool Reference` :type "/Game/UltimateSurvivalPack/Blueprints/Holdable/HoldableActors/Parent/BP_Holdable Object Reference"))
  (bind _returnvalue (`Actor.GetOwner` `Repair Tool Reference`))
  (bind _returnvalue_2 (`self.GetOwner`))
  (bind (_build_data_buildtype _build_data_ghostmesh _build_data_collisiontransform _build_data_finalbuildingclass _build_data_health _build_data_repairaddhealth) (break `/Game/UltimateSurvivalPack/Blueprints/Structs/S_Building` (`self.Build Data`)))
  (bind (_item_data_id _item_data_amount _item_data_cachedindex) (break `/Game/UltimateSurvivalPack/Blueprints/Structs/S_InventoryItem` (`/Game/UltimateSurvivalPack/Blueprints/Holdable/HoldableActors/Parent/BP_Holdable.Item Data` `Repair Tool Reference`)))
  (bind _returnvalue_3 (`/Game/UltimateSurvivalPack/Blueprints/BFL_UMSPack.Get Inventory Component` _returnvalue))
  ;[1 1 1] Server request add health (repair tool)
  (`/Engine/EditorBlueprintResources/StandardMacros.IsValid` `Repair Tool Reference`
    (:`Is Valid`
      (if (and (> _build_data_repairaddhealth 0.0) (`/Game/UltimateSurvivalPack/Blueprints/Components/BP_PlayerInventoryComponent.Has Durability` _returnvalue_3 _item_data_cachedindex))
        (`/Game/UltimateSurvivalPack/Blueprints/Components/BP_PlayerInventoryComponent.Decerase Durability` _returnvalue_3 _item_data_cachedindex 0.05)
        (set `self.Health` (`KismetMathLibrary.FClamp` (+ (`self.Health`) (`KismetMathLibrary.Abs` _build_data_repairaddhealth)) 0.0 (`self.Maximum Health`)))
        (`Actor.ForceNetUpdate` _returnvalue_2)
        (`Actor.FlushNetDormancy` _returnvalue_2)
        (`/Game/UltimateSurvivalPack/Blueprints/Components/BP_Player_ExperienceComponent.CLIENT Add Notification` (`/Game/UltimateSurvivalPack/Blueprints/BFL_UMSPack.Get Leveling Component` _returnvalue) (make `/Game/UltimateSurvivalPack/Blueprints/Structs/S_Notification` "Repairing Building" (`KismetStringLibrary.Concat_StrStr` "Added " (`KismetStringLibrary.Conv_IntToString` (`KismetMathLibrary.FTrunc` _build_data_repairaddhealth)) " health to building")))))))

(fn `Add Attached Actor`
  (params (`Build ID` :type String))
  (`KismetArrayLibrary.Array_Add` (`self.Attached Actors`) `Build ID`))

(fn `Check Cupboard Removal`
  (bind _asbp_cupboard (cast `/Game/UltimateSurvivalPack/Blueprints/Buildings/Final/BP_Cupboard` (`self.GetOwner`))
    (:`then`
      ;[1 1 1] Only For Cupboard Actors
      (bind _assurvival_gamemode (cast `/Game/UltimateSurvivalPack/Blueprints/SurvivalGamemode` (`GameplayStatics.GetGameMode`)))
      (for _array_element (`/Game/UltimateSurvivalPack/Blueprints/Buildings/Final/BP_Cupboard.Privilege Buildings` _asbp_cupboard)
        (bind _value (`BlueprintMapLibrary.Map_Find` (`/Game/UltimateSurvivalPack/Blueprints/SurvivalGamemode.Building Actors` _assurvival_gamemode) _array_element))
        (`/Engine/EditorBlueprintResources/StandardMacros.IsValid` _value
          (:`Is Valid`
            (`self.Set Cupboard` (`Actor.GetComponentByClass` _value "BP_BuildingComponent_C") "")))))
    (:`CastFailed`
      ;[1 1 1] Remove Building From Cupboard
      (bind _assurvival_gamemode_2 (cast `/Game/UltimateSurvivalPack/Blueprints/SurvivalGamemode` (`GameplayStatics.GetGameMode`)))
      (bind _asbp_cupboard_2 (cast `/Game/UltimateSurvivalPack/Blueprints/Buildings/Final/BP_Cupboard` (`BlueprintMapLibrary.Map_Find` (`/Game/UltimateSurvivalPack/Blueprints/SurvivalGamemode.Building Actors` _assurvival_gamemode_2) (`self.Cupboard ID`))))
      (`/Game/UltimateSurvivalPack/Blueprints/Buildings/Final/BP_Cupboard.Remove Building` _asbp_cupboard_2 (`self.Build ID`)))))

(fn `Check Respawnpoint Removal`
  (bind _asbp_game_instance_umsp (cast `/Game/UltimateSurvivalPack/Blueprints/BP_GameInstance_UMSP` (`GameplayStatics.GetGameInstance`)))
  (bind _players_save (`/Game/UltimateSurvivalPack/Blueprints/Save/SAV_ServerData.Players Save` (`/Game/UltimateSurvivalPack/Blueprints/BP_GameInstance_UMSP.Player Save` _asbp_game_instance_umsp)))
  (bind _keys (`BlueprintMapLibrary.Map_Keys` _players_save))
  (for _array_element _keys
    (bind _value (`BlueprintMapLibrary.Map_Find` _players_save _array_element))
    (if (`KismetStringLibrary.EqualEqual_StrStr` (`.RespawnBuilding_59_A83F0582498F7FEB78B520800AEB0C27` (break `/Game/UltimateSurvivalPack/Blueprints/Structs/S_PlayerSave` _value)) (`self.Build ID`))
      (bind _structout (setmembers `/Game/UltimateSurvivalPack/Blueprints/Structs/S_PlayerSave` :`StructRef` _value :`Respawn Point` (0.0 0.0 0.0) :`Respawn Building` ""))
      (`/Game/UltimateSurvivalPack/Blueprints/BP_GameInstance_UMSP.Save Player Data` _asbp_game_instance_umsp _array_element _structout))))

(fn `Handled Damage`
  (params (Damage :type "Float (double-precision)"))
  (bind _returnvalue (`self.GetOwner`))
  (bind _output_get (set `self.Health` (- (`self.Health`) Damage)))
  (`Actor.ForceNetUpdate` _returnvalue)
  (`Actor.FlushNetDormancy` _returnvalue)
  (if (<= _output_get 0.0)
    (`Actor.K2_DestroyActor` (`self.GetOwner`))
    (return)
    (else
      (bind _assurvival_gamemode (cast `/Game/UltimateSurvivalPack/Blueprints/SurvivalGamemode` (`GameplayStatics.GetGameMode`)))
      (bind (_saved_data _returnvalue_2) (`/Game/UltimateSurvivalPack/Blueprints/SurvivalGamemode.Get Saved Build Data` _assurvival_gamemode (`self.Build ID`)))
      (if _returnvalue_2
        (bind (_builddata _transform _onattachedactor _worldname _inventory _customfloat _customstring _cupboard) (break `/Game/UltimateSurvivalPack/Blueprints/Structs/S_BuildSave` _saved_data))
        (`/Game/UltimateSurvivalPack/Blueprints/SurvivalGamemode.Save Existing Building` _assurvival_gamemode (`self.Build ID`) (make `/Game/UltimateSurvivalPack/Blueprints/Structs/S_BuildSave` _builddata _transform _onattachedactor _worldname _inventory _customfloat _customstring _cupboard (`self.Health`)))))))

(fn `Is In Cupboard`
  (params (`Player ID` :type String))
  (returns (Return :type Boolean))
  (bind _assurvival_gamemode (cast `/Game/UltimateSurvivalPack/Blueprints/SurvivalGamemode` (`GameplayStatics.GetGameMode`)))
  (bind (_value _returnvalue) (`BlueprintMapLibrary.Map_Find` (`/Game/UltimateSurvivalPack/Blueprints/SurvivalGamemode.Building Actors` _assurvival_gamemode) (`self.Cupboard ID`)))
  (if _returnvalue
    (`/Engine/EditorBlueprintResources/StandardMacros.IsValid` _value
      (:`Is Valid`
        (bind _asbp_cupboard (cast `/Game/UltimateSurvivalPack/Blueprints/Buildings/Final/BP_Cupboard` _value)
          (:`then`
            (return (`KismetArrayLibrary.Array_Contains` (`/Game/UltimateSurvivalPack/Blueprints/Buildings/Final/BP_Cupboard.Privilege Players` _asbp_cupboard) (`local.Player ID`))))
          (:`CastFailed`
            _)))
      (:`Is Not Valid`
        _))
    (return true)
    (else
      (return true))))

(fn `OnRep_Build Data`
  ;[1 1 1] Update health
  (set `self.Maximum Health` (`.Health_24_A0BD453941DAB13B0A4FDD99102D5C21` (break `/Game/UltimateSurvivalPack/Blueprints/Structs/S_Building` (`self.Build Data`)))))

(fn `Spawn Build Emmiter`
  (bind _returnvalue (`self.GetOwner`))
  (bind (_origin _boxextent) (`Actor.GetActorBounds` _returnvalue false true))
  (bind _returnvalue_2 (+ (.x _boxextent) (.y _boxextent) (.z _boxextent)))
  (bind _returnvalue_3 (`NiagaraFunctionLibrary.SpawnSystemAtLocation` "/Game/UltimateSurvivalPack/Demo/Particles/Niagara/PSN_Smoke_Puff.PSN_Smoke_Puff" _origin (`Actor.K2_GetActorRotation` _returnvalue)))
  (`/Engine/EditorBlueprintResources/StandardMacros.IsValid` _returnvalue_3
    (:`Is Valid`
      (`NiagaraComponent.SetVariableInt` _returnvalue_3 "Spawn Count" (`KismetMathLibrary.FTrunc` (`KismetMathLibrary.FClamp` (/ _returnvalue_2 75.0) 0.0 10.0)))
      (`NiagaraComponent.SetVariableFloat` _returnvalue_3 "Emitter Scale" (/ _returnvalue_2 300.0))
      (`NiagaraComponent.SetVariableVec3` _returnvalue_3 "Spawn Dimension" _boxextent)
      (return))))