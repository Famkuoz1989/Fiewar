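; AN_SwimEffect is an animation notify that plays swimming splash and sound effects for a character.
; Outside dedicated servers, it reads IsDiving from the owner's BP_PlayerComponent and spawns small Niagara water splashes at both hand sockets only when not diving.
; The swim sound cue plays at the left hand socket whether diving or not, using the footsteps attenuation settings.
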(fn `Received_Notify`
  (params (MeshComp :type "SkeletalMeshComponent Object Reference") (Animation :type "AnimSequenceBase Object Reference") (EventReference :type "AnimNotifyEventReference Structure (by ref)"))
  (returns (ReturnValue :type Boolean))
  (locals (`L Bone Location` :type "Vector Structure" :default (0.0 0.0 0.0)) (`L Owner` :type "Actor Object Reference") (`L Hit` :type "HitResult Structure") (`L Player Component` :type "/Game/UltimateSurvivalPack/Blueprints/Components/BP_PlayerComponent Object Reference"))
  (bind _returnvalue (`SceneComponent.GetSocketLocation` (`local.MeshComp`) "hand_l"))
  (if (not (`KismetSystemLibrary.IsDedicatedServer`))
    (bind _output_get (set `local.L Owner` (`ActorComponent.GetOwner` MeshComp)))
    (bind _output_get_2 (set `local.L Player Component` (`Actor.GetComponentByClass` _output_get "/Game/UltimateSurvivalPack/Blueprints/Components/BP_PlayerComponent.BP_PlayerComponent_C")))
    (if (not (`/Game/UltimateSurvivalPack/Blueprints/Components/BP_PlayerComponent.Is Diving` _output_get_2))
      (`NiagaraFunctionLibrary.SpawnSystemAtLocation` "/Game/UltimateSurvivalPack/Demo/Particles/Niagara/NS_WaterSplash_Small.NS_WaterSplash_Small" _returnvalue)
      (`NiagaraFunctionLibrary.SpawnSystemAtLocation` "/Game/UltimateSurvivalPack/Demo/Particles/Niagara/NS_WaterSplash_Small.NS_WaterSplash_Small" (`SceneComponent.GetSocketLocation` (`local.MeshComp`) "hand_r")))
    (`GameplayStatics.SpawnSoundAtLocation` "/Game/UltimateSurvivalPack/Demo/Audio/SFX/CUE_Swim.CUE_Swim" _returnvalue (struct) 1.0 1.0 0.0 "/Game/UltimateSurvivalPack/Blueprints/Attenuation/SA_Footsteps.SA_Footsteps" null)))