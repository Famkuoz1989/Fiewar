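; Anim notify that plays zombie footstep sounds at a configurable bone when an enemy animation triggers it, skipped on dedicated servers.
; A short downward object trace from the bone checks WorldDynamic hits for the foliage surface type.
; A foliage hit adds a rustle sound at the owner's location, layered over the footstep played at the bone with adjustable volume and pitch.
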(fn `Foliage Hit Filter`
  (params (Hit :type "Array of HitResult Structure"))
  (returns (Foliage :type Boolean))
  (locals (`L Foliage Overlap` :type Boolean))
  (for _array_element Hit
    (if (`|EnumEquality` (`GameplayStatics.GetSurfaceType` _array_element) "SurfaceType3")
      (set `local.L Foliage Overlap` true)
      (return true)))
  (return (`local.L Foliage Overlap`)))

(fn `Received_Notify`
  (params (MeshComp :type "SkeletalMeshComponent Object Reference") (Animation :type "AnimSequenceBase Object Reference") (EventReference :type "AnimNotifyEventReference Structure (by ref)"))
  (returns (ReturnValue :type Boolean))
  (locals (`L Bone Location` :type "Vector Structure" :default (0.0 0.0 0.0)) (`L Owner` :type "Actor Object Reference"))
  (if (not (`KismetSystemLibrary.IsDedicatedServer`))
    (set `local.L Owner` (`ActorComponent.GetOwner` MeshComp))
    (set `local.L Bone Location` (`SceneComponent.GetSocketLocation` MeshComp (`self.Bone Name`)))
    ;[1 1 1] Spawn Foliage Sound
    (bind (_outhits _returnvalue) (`KismetSystemLibrary.LineTraceMultiForObjects` (`local.L Bone Location`) (- (`local.L Bone Location`) (0.0 0.0 50.0)) (`|MakeArray` "ObjectTypeQuery2" :!type "EObjectTypeQuery Enum")))
    (if _returnvalue
      (bind _foliage (`self.Foliage Hit Filter` _outhits))
      (if _foliage
        (`GameplayStatics.SpawnSoundAtLocation` "/Game/UltimateSurvivalPack/Demo/Audio/SFX/CUE_InFoliage.CUE_InFoliage" (`Actor.K2_GetActorLocation` (`local.L Owner`)) (struct) (`self.Volume Multiplier`) 1.0 0.0 "/Game/UltimateSurvivalPack/Blueprints/Attenuation/SA_Footsteps.SA_Footsteps" null)))
    ;[1 1 1] Spawn Footstep Sound
    (`GameplayStatics.SpawnSoundAtLocation` "/Game/UltimateSurvivalPack/Demo/Audio/SFX/Zombie/CUE_Zombie_Footstep.CUE_Zombie_Footstep" (`local.L Bone Location`) (struct) (`self.Volume Multiplier`) (`self.Pitch Multiplier`) 0.0 "/Game/UltimateSurvivalPack/Blueprints/Attenuation/SA_Footsteps.SA_Footsteps" null)
    (return true)))