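; Spherical temperature zone that changes the outside temperature felt by the local player while inside it.
; LocalOverlap writes the zone's Temperature to OutsideTemperature on the player component, and restores that component's class default on exit.
; LocalCanOverlap tests player controller 0's pawn by squared distance against InSphereRadius.
; The construction script forces unit actor scale and sizes the sphere to that radius.
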(event `/Game/UltimateSurvivalPack/Blueprints/Interface/BPI_InventorySystem.Local Overlap`
  (params (Overlap :type Boolean))
  (bind _returnvalue (`/Game/UltimateSurvivalPack/Blueprints/BFL_UMSPack.Get Player Component` (`/Game/UltimateSurvivalPack/Blueprints/Components/BP_PlayerInventoryComponent.Human Player Character` (`/Game/UltimateSurvivalPack/Blueprints/BFL_UMSPack.Get Inventory Component` (`GameplayStatics.GetPlayerController` 0)))))
  (if Overlap
    (set `/Game/UltimateSurvivalPack/Blueprints/Components/BP_PlayerComponent.Outside Temperature` (`self.Temperature`) _returnvalue)
    (else
      (set `/Game/UltimateSurvivalPack/Blueprints/Components/BP_PlayerComponent.Outside Temperature` (defaults `Object` (`GameplayStatics.GetObjectClass` _returnvalue)) _returnvalue))))

(fn `Get Interaction Data`
  (returns (`Interaction Text` :type Text))
  (return ""))

(fn `Get Team ID`
  (returns (`Team ID` :type Byte))
  (return 0))

(fn `Local Can Overlap`
  (returns (Success :type Boolean))
  (bind _in_sphere_radius (`self.In Sphere Radius`))
  (return (< (`self.GetSquaredDistanceTo` (`Controller.K2_GetPawn` (`GameplayStatics.GetPlayerController` 0))) (* _in_sphere_radius _in_sphere_radius))))

(fn `UserConstructionScript`
  (`self.SetActorScale3D` (1.0 1.0 1.0)) ; Failsafe
  (`SphereComponent.SetSphereRadius` (`self.Sphere`) (`self.In Sphere Radius`) false))