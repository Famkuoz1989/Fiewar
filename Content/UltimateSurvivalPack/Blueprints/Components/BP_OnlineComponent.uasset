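; BP_OnlineComponent is an actor component that provides multiplayer text chat between players.
; SendChatMessage rejects empty text, otherwise passes the player's name and message in white to a server event, returning whether it sent.
; The server loops over all PlayerControllers and calls a client event on each one's online component.
; Each client then adds the message to the chat widget obtained from the component's owner.
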(event `SERVER Send Chat Message`
  (params (Name :type String) (Message :type Text) (`Message Color` :type "LinearColor Structure"))
  ;[0.3739 0.5374 1 1 64] Chat System
  ;;[1 1 1] Find All Players And Send Them Message
  (bind _outactors (`GameplayStatics.GetAllActorsOfClass` "/Script/Engine.PlayerController"))
  (for _array_element _outactors
    (bind _bp_onlinecomponent (`/Game/UltimateSurvivalPack/LobbySystem/Blueprints/BFL_LobbySystem.Get Online Component` _array_element))
    (`/Engine/EditorBlueprintResources/StandardMacros.IsValid` _bp_onlinecomponent
      (:`Is Valid`
        (`self.CLIENT Receive Chat Message` _bp_onlinecomponent (select `bool` (`KismetStringLibrary.EqualEqual_StrStr` Name) :`false` Name :`true` "") Message `Message Color`)))))

(event `CLIENT Receive Chat Message`
  (params (`Sender Name` :type String) (Message :type Text) (`Message Color` :type "LinearColor Structure"))
  ;[0.3739 0.5374 1 1 64] Chat System
  ;;[1 1 1] Write Message To Widget
  (bind _chat_widget_reference (message `/Game/UltimateSurvivalPack/Blueprints/Interface/BPI_OnlineSystem.Get Chat Widget` (`self.GetOwner`)))
  (`/Engine/EditorBlueprintResources/StandardMacros.IsValid` _chat_widget_reference
    (:`Is Valid`
      (`/Game/UltimateSurvivalPack/LobbySystem/Widget/W_Chat.Add Chat Message` _chat_widget_reference `Sender Name` Message `Message Color`))))

(fn `Send Chat Message`
  (params (Player :type "PlayerController Object Reference") (Message :type Text))
  (returns (Return :type Boolean))
  ;[1 1 1] Request server to send message if not Null
  (if (`KismetTextLibrary.NotEqual_TextText` Message "")
    (`self.SERVER Send Chat Message` (`/Game/UltimateSurvivalPack/LobbySystem/Blueprints/BFL_LobbySystem.Get Player Name` Player) Message (struct :`R` 1.0 :`G` 1.0 :`B` 1.0 :`A` 1.0))
    (return true)
    (else
      (return false))))