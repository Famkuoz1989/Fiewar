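; Chest inventory component for storage actors, with optional random loot filled from a loot table or, failing that, the item table.
; Changes refresh players who have this storage open, prune stale viewers and, for building pieces, save contents through SurvivalGamemode.
; Destroying the owner closes the local player's menu if this storage is open; on authority it can also spawn a stash holding the remaining items.
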(event `Reinitialize`
  ;[1 0.1552 0.195] Initialization
  (`self.Create Inventory`))

(event `self.ReceiveBeginPlay`
  ;[1 0.1552 0.195] Initialization
  (add `Actor.OnDestroyed` (`self.GetOwner`) (delegate `Event Destroyed`))
  (`self.Create Inventory`))

(event `Event Destroyed`
  (params (DestroyedActor :type "Actor Object Reference"))
  (bind _returnvalue (`GameplayStatics.GetPlayerController` 0))
  ;[1 1 1] On Destroyed
  (if (== self (`/Game/UltimateSurvivalPack/Blueprints/Components/BP_PlayerInventoryComponent.Current Opened Storage` (`/Game/UltimateSurvivalPack/Blueprints/BFL_UMSPack.Get Inventory Component` _returnvalue)))
    (`/Game/UltimateSurvivalPack/Blueprints/Components/BP_MissionComponent.Close Inventory Menu` (`/Game/UltimateSurvivalPack/Blueprints/BFL_UMSPack.Get Mission Component` _returnvalue))))

(event `Update All Clients Inventory`
  (bind _returnvalue (`Actor.GetComponentByClass` (`self.GetOwner`) "/Game/UltimateSurvivalPack/Blueprints/Buildings/Parent/BP_BuildingComponent.BP_BuildingComponent_C"))
  (bind _build_id (`/Game/UltimateSurvivalPack/Blueprints/Buildings/Parent/BP_BuildingComponent.Build ID` _returnvalue))
  ;[1 1 1] Update Chest
  ;;[1 1 1] Update On All Clients
  (`self.Update Inventory To All Clients`)
  (`self.Storage Updated`)
  ;;[1 1 1] Save New Chest Data to Save Component
  (`/Engine/EditorBlueprintResources/StandardMacros.IsValid` _returnvalue
    (:`Is Valid`
      (bind _assurvival_gamemode (cast `/Game/UltimateSurvivalPack/Blueprints/SurvivalGamemode` (`GameplayStatics.GetGameMode`)))
      (bind (_saved_data _returnvalue_2) (`/Game/UltimateSurvivalPack/Blueprints/SurvivalGamemode.Get Saved Build Data` _assurvival_gamemode _build_id))
      (if _returnvalue_2
        (bind ((`BuildData_2_700EB4E148DBEF7281188785324662CA` _builddata) (`Transform_6_227D833D45720C2C90F11EB731C1BBAA` _transform) (`OnAttachedActor_9_07069BCA4FEF9223D5BEC6BA5C09F0C5` _onattachedactor) (`WorldName_11_6840022640BD07C9638712B3FDD0588F` _worldname) (`CustomFloat_21_2B1EE62141F1CF01B611A4BB124FA5E8` _customfloat) (`CustomString_25_358AA98E4F4B4693E56F5CB4422E5AF2` _customstring) (`Cupboard_28_E77CCD52410AEBABC31F47A904A01FB2` _cupboard)) (break `/Game/UltimateSurvivalPack/Blueprints/Structs/S_BuildSave` _saved_data))
        (`/Game/UltimateSurvivalPack/Blueprints/SurvivalGamemode.Save Existing Building` _assurvival_gamemode _build_id (make `/Game/UltimateSurvivalPack/Blueprints/Structs/S_BuildSave` _builddata _transform _onattachedactor _worldname (`self.Inventory`) _customfloat _customstring _cupboard (`/Game/UltimateSurvivalPack/Blueprints/Buildings/Parent/BP_BuildingComponent.Health` _returnvalue)))))))

(event `self.ReceiveEndPlay`
  (params (EndPlayReason :type "EEndPlayReason Enum" :default "Destroyed"))
  ;[1 1 1] On End Play
  (`parent.ReceiveEndPlay` EndPlayReason)
  (switch `EEndPlayReason` EndPlayReason
    (:`Destroyed`
      ;;[1 1 1] Switch on Authority
      (if (`Actor.HasAuthority` (`self.GetOwner`))
        (`self.Spawn Destroyed Items`)))))

(fn `Create Inventory`
  (locals (`L Randomized Item Names` :type "Array of Name") (`L Index` :type Integer))
  (bind _inventory (`self.Inventory`))
  (bind _l_index (`local.L Index`))
  (bind _inventory_2 (`self.Inventory`))
  (`parent.Create Inventory`)
  (if (> (`self.Random Loot Spawn Count`) 0)
    (bind _random_loot_data_table (`self.Random Loot Data Table`)
      (:`then`
        (bind _outrownames (`DataTableFunctionLibrary.GetDataTableRowNames` _random_loot_data_table))
        (bind _output_get (set `local.L Randomized Item Names` _outrownames))
        (`KismetArrayLibrary.Array_Shuffle` _output_get)
        (if (> (`KismetArrayLibrary.Array_LastIndex` (`local.L Randomized Item Names`)) 0)
          (for _index (range (+ (`KismetMathLibrary.Clamp` (`self.Random Loot Spawn Count`) 0 (`KismetArrayLibrary.Array_LastIndex` (`local.L Randomized Item Names`))) 1))
            (bind _returnvalue (`|GetDataTableRow` _random_loot_data_table (`|GetArrayItem` (`local.L Randomized Item Names`) _index))
              (:`then`
                (bind (_id _minimumspawnamount _maximumspawnamount _chance) (break `/Game/UltimateSurvivalPack/Blueprints/Structs/S_ItemSpawner` _returnvalue))
                (if (>= _chance (`KismetMathLibrary.RandomFloatInRange` 0.0 1.0))
                  _
                  (else
                    _))
                (if (`KismetArrayLibrary.Array_IsValidIndex` _inventory (`local.L Index`))
                  (`KismetArrayLibrary.Array_Set` _inventory _l_index (make `/Game/UltimateSurvivalPack/Blueprints/Structs/S_InventoryItem` _id (`KismetMathLibrary.RandomIntegerInRange` _minimumspawnamount _maximumspawnamount) _l_index self))
                  (`/Engine/EditorBlueprintResources/StandardMacros.IncrementInt` (`local.L Index`))))))))
      (:`else`
        (bind _outrownames_2 (`DataTableFunctionLibrary.GetDataTableRowNames` "/Game/UltimateSurvivalPack/Blueprints/Datatable/Inventory/DT_ItemData.DT_ItemData"))
        (for _index_2 (range (`self.Random Loot Spawn Count`))
          (if (`KismetArrayLibrary.Array_IsValidIndex` _inventory_2 _index_2)
            (bind _output (`|GetArrayItem` _outrownames_2 (`KismetMathLibrary.RandomIntegerInRange` 0 (`KismetArrayLibrary.Array_LastIndex` _outrownames_2))))
            (`KismetArrayLibrary.Array_Set` _inventory_2 _index_2 (make `/Game/UltimateSurvivalPack/Blueprints/Structs/S_InventoryItem` _output (`KismetMathLibrary.RandomIntegerInRange` 1 (`.MaximumStack_21_39EA4E634AD2ADBC0EA36C92000AFBC7` (break `/Game/UltimateSurvivalPack/Blueprints/Structs/S_InventoryItemData` (`.Item Data` (`/Game/UltimateSurvivalPack/Blueprints/BFL_Inventory.Get Item Data from ID` _output))))) _index_2 self))))))))

(fn `Remove Item`
  (params (`At Index` :type Integer) (Amount :type Integer) (`From Inventory` :type "/Game/UltimateSurvivalPack/Blueprints/Components/BP_MasterInventoryComponent Object Reference"))
  (bind (_id _amount _cachedindex _inventoryreference _custominteger _durability _additionaldata) (break `/Game/UltimateSurvivalPack/Blueprints/Structs/S_InventoryItem` (`|GetArrayItem` (`self.Inventory`) `At Index`)))
  (if (>= Amount _amount)
    (`KismetArrayLibrary.Array_Set` (`self.Inventory`) (`local.At Index`) (make `/Game/UltimateSurvivalPack/Blueprints/Structs/S_InventoryItem` "None" 0 (`local.At Index`) (`local.From Inventory`)))
    (else
      (`KismetArrayLibrary.Array_Set` (`self.Inventory`) (`local.At Index`) (make `/Game/UltimateSurvivalPack/Blueprints/Structs/S_InventoryItem` _id (- _amount (`local.Amount`)) (`local.At Index`) (`local.From Inventory`) _custominteger _durability _additionaldata)))))

(fn `Remove Items`
  (params (`Item ID` :type Name) (Amount :type Integer) (`Update Storage` :type Boolean :default true))
  (locals (`L Remaining Amount` :type Integer) (`L Index` :type Integer) (`L Current Item` :type "/Game/UltimateSurvivalPack/Blueprints/Structs/S_InventoryItem Structure") (`Item ID` :type Name) (`L Updated` :type Boolean) (`L Update Indexes` :type "Array of Integer"))
  (bind (_l_current_item_id _l_current_item_amount _l_current_item_cachedindex _l_current_item_inventoryreference _l_current_item_custominteger _l_current_item_durability _l_current_item_additionaldata) (break `/Game/UltimateSurvivalPack/Blueprints/Structs/S_InventoryItem` (`local.L Current Item`)))
  (`|ExecutionSequence`
    (:`then_0`
      (set `local.L Remaining Amount` Amount)
      (for (_array_element _array_index) (`self.Inventory`)
        (bind _output_get (set `local.L Current Item` _array_element))
        (set `local.L Index` _array_index)
        (bind ((`ID_2_1F4451EE4759095BA0D31BB237483A5E` _id) (`Amount_5_1F2975454CE296A7C7033BA39535256F` _amount)) (break `/Game/UltimateSurvivalPack/Blueprints/Structs/S_InventoryItem` _output_get))
        (if (== (`local.Item ID`) _id)
          (if (<= _amount (`local.L Remaining Amount`))
            (bind _returnvalue (- (`local.L Remaining Amount`) (`KismetMathLibrary.Clamp` _amount 0 (`local.L Remaining Amount`))))
            (set `local.L Remaining Amount` _returnvalue)
            (`KismetArrayLibrary.Array_Set` (`self.Inventory`) (`local.L Index`) (make `/Game/UltimateSurvivalPack/Blueprints/Structs/S_InventoryItem` "None" 0 (`local.L Index`) self))
            (`KismetArrayLibrary.Array_Add` (`local.L Update Indexes`) (`local.L Index`))
            (else
              (set `local.L Remaining Amount` _returnvalue)
              (`KismetArrayLibrary.Array_Set` (`self.Inventory`) (`local.L Index`) (make `/Game/UltimateSurvivalPack/Blueprints/Structs/S_InventoryItem` _l_current_item_id (- _l_current_item_amount 1) _l_current_item_cachedindex self _l_current_item_custominteger _l_current_item_durability _l_current_item_additionaldata))
              (`KismetArrayLibrary.Array_Add` (`local.L Update Indexes`) (`local.L Index`))))
          (if (<= (`local.L Remaining Amount`) 0)
            (if (`local.Update Storage`)
              (`self.Update All Clients Inventory`))
            (return)
            (else
              (set `local.L Updated` true)))))
      (if (and (`local.L Updated`) (`local.Update Storage`))
        (`self.Update All Clients Inventory` self)))
    (:`then_1`
      (return))))

(fn `Spawn Destroyed Items`
  (if (`self.Enable Spawn Items Destroyed`)
    ;[1 1 1] Can create death bag
    (if (`self.Has Any Items in Inventory`)
      ;[1 1 1] Spawn Storage on Controlled Pawn Loc
      (bind _returnvalue (`|SpawnActorFromClass` "/Game/UltimateSurvivalPack/Blueprints/Buildings/BP_StorageStash.BP_StorageStash_C" (`KismetMathLibrary.MakeTransform` (`Actor.K2_GetActorLocation` (`self.GetOwner`))) "AdjustIfPossibleButAlwaysSpawn" "OverrideRootScale" null null))
      (bind _bp_chestinventorycomponent (`/Game/UltimateSurvivalPack/Blueprints/Buildings/BP_StorageStash.BP_ChestInventoryComponent` _returnvalue))
      ;[1 1 1] Initialize and replace inventory
      (set `/Game/UltimateSurvivalPack/Blueprints/Components/BP_MasterInventoryComponent.Inventory Size` (+ (`self.Inventory Size`) 4) _bp_chestinventorycomponent)
      (`self.Reinitialize` _bp_chestinventorycomponent)
      (for (_array_element _array_index) (`self.Inventory`)
        (`KismetArrayLibrary.Array_Set` (`/Game/UltimateSurvivalPack/Blueprints/Components/BP_MasterInventoryComponent.Inventory` _bp_chestinventorycomponent) _array_index (make `/Game/UltimateSurvivalPack/Blueprints/Structs/S_InventoryItem` (break `/Game/UltimateSurvivalPack/Blueprints/Structs/S_InventoryItem` _array_element) (`.Amount_5_1F2975454CE296A7C7033BA39535256F` (break `/Game/UltimateSurvivalPack/Blueprints/Structs/S_InventoryItem` _array_element)) _array_index _bp_chestinventorycomponent (`.CustomInteger_14_C4B91C704D98E5A3B3B6D1B77CFE476E` (break `/Game/UltimateSurvivalPack/Blueprints/Structs/S_InventoryItem` _array_element)) (`.Durability_17_EACE862B4A67C4626DE918B12D7D20BB` (break `/Game/UltimateSurvivalPack/Blueprints/Structs/S_InventoryItem` _array_element))) true)))))

(fn `Update Inventory To All Clients`
  (locals (`L Player Components` :type "Array of /Game/UltimateSurvivalPack/Blueprints/Components/BP_PlayerInventoryComponent Object Reference"))
  (bind _output_get (set `local.L Player Components` (`self.Controlling Components`)))
  ;[1 1 1] Loop each client that has interacted with chest, dump if not valid (disconnected)
  (for _array_element _output_get
    (`/Engine/EditorBlueprintResources/StandardMacros.IsValid` _array_element
      (:`Is Valid`
        (if (== (`/Game/UltimateSurvivalPack/Blueprints/Components/BP_PlayerInventoryComponent.Current Opened Storage` _array_element) self)
          (`/Game/UltimateSurvivalPack/Blueprints/Components/BP_PlayerInventoryComponent.Open Chest Inventory` _array_element self false (`self.Inventory`))
          (else
            (`KismetArrayLibrary.Array_RemoveItem` (`self.Controlling Components`) _array_element :!label _label))))
      (:`Is Not Valid`
        (goto _label))))
  (return))