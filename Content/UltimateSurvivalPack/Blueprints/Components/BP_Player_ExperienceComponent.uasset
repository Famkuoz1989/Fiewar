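; Controller-owned component that tracks the player's XP and level, loading them from the game instance's save on local BeginPlay.
; AddExperience clamps total XP against formula-based level thresholds, loops level changes, updates level suffixes, then saves through the inventory component.
; CLIENT events push XP and notifications to the mission component's HUD.
; Debug-messaged switches control level loss, multi-level gain caps and per-level or cumulative XP display.
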(event `Update Values`
  ;[1 1 1] Main Events
  ;;[0.4969 1 0.4969] Update Values on Network
)

(event `Add Experience`
  (params (Experience :type Integer) (`Enable Notification` :type Boolean) (Notification :type "/Game/UltimateSurvivalPack/Blueprints/Structs/S_Notification Structure"))
  ;[1 1 1] Main Events
  ;;[0.498 1 0.498] Add Experience Event
  (bind (_current_xp _maximum_xp _minimum_xp) (`self.On Experience Changed` Experience))
  (`self.CLIENT Update Experience Widget` (`self.Level`) _current_xp _maximum_xp _minimum_xp)
  (`self.Update Values`)
  (`/Game/UltimateSurvivalPack/Blueprints/Components/BP_MasterInventoryComponent.Save Player Data` (`/Game/UltimateSurvivalPack/Blueprints/BFL_UMSPack.Get Inventory Component` (`self.GetOwner`)))
  (if `Enable Notification`
    (`self.CLIENT Add Notification` Notification)))

(event `Reset Experience`
  ;[1 1 1] Main Events
  ;;[0.498 1 0.498] Restart Experience Event
  (if (`self.Decrease Level`)
    (`self.Add Experience` (* (`self.Total Experience Points`) -1))
    (`self.Debug Message` "Experience has been reset" (struct :`R` 0.1 :`G` 1.0 :`B` 0.1 :`A` 1.0) 4.0)
    (else
      (`self.Debug Message` "You can't reset experience when you have Decerasing Level = Disabled \nEnable it by pressing [ Y ]" (struct :`R` 1.0 :`G` 0.2 :`B` 0.2 :`A` 1.0) 4.0))))

(event `Switch Decrease Level`
  ;[1 1 1] Main Events
  ;;[0.498 1 0.498] Toggle Decrease Level Event
  (bind _output_get (set `self.Decrease Level` (not (`self.Decrease Level`))))
  (`self.Debug Message` (select `bool` _output_get :`false` "You are no longer able to decerase level" :`true` "You are now able to decerase level") (struct :`G` 0.701961 :`B` 1.0 :`A` 1.0) 4.0))

(event `Set Level Skipping`
  (bind _returnvalue (+ (`self.Level Skipping`) 1))
  ;[1 1 1] Main Events
  ;;[0.498 1 0.498] Set Level skipping
  (if (> _returnvalue 5)
    (set `self.Level Skipping` 1)
    (`self.Debug Message` "Level skipping has been disabled" (struct :`R` 0.1 :`G` 1.0 :`B` 0.1 :`A` 1.0) 4.0)
    (else
      (bind _output_get (set `self.Level Skipping` _returnvalue))
      (`self.Debug Message` (`KismetStringLibrary.Concat_StrStr` "Level Skipping has been set to " (`KismetStringLibrary.Conv_IntToString` _output_get)) (struct :`G` 0.701961 :`B` 1.0 :`A` 1.0) 4.0))))

(event `CLIENT Load Component`
  (params (`Current Level` :type Integer) (`Experience Points` :type Integer) (`Actual Experience Points` :type Integer) (`Maximum Experience` :type Integer) (`Minimum Experience` :type Integer))
  (bind _hud (`/Game/UltimateSurvivalPack/Blueprints/Components/BP_MissionComponent.HUD` (`/Game/UltimateSurvivalPack/Blueprints/BFL_UMSPack.Get Mission Component` (`self.GetOwner`))))
  ;[1 1 1] Load Component on Client
  (bind _output_get (set `self.Level` `Current Level`))
  (set `self.Total Experience Points` `Experience Points`)
  (`/Engine/EditorBlueprintResources/StandardMacros.IsValid` _hud
    (:`Is Valid`
      (`/Game/UltimateSurvivalPack/Widget/W_HUD.Add Experience` _hud _output_get `Actual Experience Points` `Maximum Experience` `Minimum Experience`))))

(event `SERVER Initialize`
  (bind (_maximum_total_xp _minimum_total_xp _maximum_current_xp _minimum_current_xp _actual_current_xp) (`self.Get Level Information` (`self.Level`)))
  ;[1 1 1] Begin PLay
  (bind _asbp_game_instance_umsp (cast `/Game/UltimateSurvivalPack/Blueprints/BP_GameInstance_UMSP` (`GameplayStatics.GetGameInstance`)))
  (bind _player_save (`/Game/UltimateSurvivalPack/Blueprints/BP_GameInstance_UMSP.Player Save` _asbp_game_instance_umsp))
  (`/Engine/EditorBlueprintResources/StandardMacros.IsValid` _player_save
    (:`Is Valid`
      (bind ((`Level_16_83D6146A4E52593645A0B2B8A361A480` _level) (`TotalExperiencePoints_18_5A66592D4AD144AE29DA819A39A6CD8C` _totalexperiencepoints)) (break `/Game/UltimateSurvivalPack/Blueprints/Structs/S_PlayerSave` (`BlueprintMapLibrary.Map_Find` (`/Game/UltimateSurvivalPack/Blueprints/Save/SAV_ServerData.Players Save` _player_save) (`/Game/UltimateSurvivalPack/LobbySystem/Blueprints/BFL_LobbySystem.Get Player Unique ID` (cast `PlayerController` (`self.GetOwner`) :!pure true)))))
      (set `self.Level` _level)
      (set `self.Total Experience Points` _totalexperiencepoints)
      (`self.CLIENT Load Component` (`self.Level`) (`self.Total Experience Points`) _actual_current_xp _maximum_current_xp _minimum_current_xp))))

(event `CLIENT Update Experience Widget`
  (params (`Current Level` :type Integer) (`Actual Experience Points` :type Integer) (`Maximum Experience` :type Integer) (`Minimum Experience` :type Integer))
  (bind _hud (`/Game/UltimateSurvivalPack/Blueprints/Components/BP_MissionComponent.HUD` (`/Game/UltimateSurvivalPack/Blueprints/BFL_UMSPack.Get Mission Component` (`self.GetOwner`))))
  ;[1 1 1] Refresh XP Widget
  (set `self.Level` `Current Level`)
  (`/Engine/EditorBlueprintResources/StandardMacros.IsValid` _hud
    (:`Is Valid`
      (`/Game/UltimateSurvivalPack/Widget/W_HUD.Add Experience` _hud `Current Level` `Actual Experience Points` `Maximum Experience` `Minimum Experience`))))

(event `self.ReceiveBeginPlay`
  ;[1 1 1] Begin PLay
  (if (`Controller.IsLocalController` (cast `Controller` (`self.GetOwner`) :!pure true))
    (`self.SERVER Initialize`)))

(event `CLIENT Add Notification`
  (params (Notification :type "/Game/UltimateSurvivalPack/Blueprints/Structs/S_Notification Structure"))
  (bind _hud (`/Game/UltimateSurvivalPack/Blueprints/Components/BP_MissionComponent.HUD` (`/Game/UltimateSurvivalPack/Blueprints/BFL_UMSPack.Get Mission Component` (`self.GetOwner`))))
  ;[1 1 1] Add Notication Widget
  (`/Engine/EditorBlueprintResources/StandardMacros.IsValid` _hud
    (:`Is Valid`
      (`/Game/UltimateSurvivalPack/Widget/W_HUD.Create Notification` _hud Notification))))

(event `Switch Experience Level Mode`
  ;[1 1 1] Change Experience Calculation Mode
  (bind _output_get (set `self.Restart Points on Levelup` (not (`self.Restart Points on Levelup`))))
  (`self.Debug Message` (select `bool` _output_get :`false` "Points are now kept when player Levels up" :`true` "Points are now set to 0 when player Levels up") (struct :`G` 0.7 :`B` 1.0 :`A` 1.0) 4.0)
  (`self.Add Experience` 0) ; Only For Refreshing Level Mode
)

(fn `Debug Message`
  (params (Message :type String) (TextColor :type "LinearColor Structure") (Duration :type "Float (double-precision)"))
  (if (`self.Enable Debug Messages`)
    (`KismetSystemLibrary.PrintString` (`KismetStringLibrary.Concat_StrStr` "[AMLS] " Message) true true TextColor Duration)
    (`GameplayStatics.PlaySound2D` "/Engine/VREditor/Sounds/VR_click2.VR_click2" 0.2 0.5 0.0 null null)))

(fn `Find Level Suffix`
  (params (Level :type Integer))
  (returns (Suffix :type Text))
  (locals (`L Current Array Element` :type "/Game/UltimateSurvivalPack/Blueprints/Structs/S_Level Structure") (`L Current Suffix` :type Text))
  (for (_array_element _array_index) (`self.Level Suffixes`)
    (bind _output_get (set `local.L Current Array Element` _array_element))
    (bind _returnvalue (>= (`local.Level`) (`.FromLevel_2_CE6A64F64E4499F64FBCEB9BC76B487A` (break `/Game/UltimateSurvivalPack/Blueprints/Structs/S_Level` _output_get))))
    (bind _returnvalue_2 (+ _array_index 1))
    (if (select `bool` (< _returnvalue_2 (`KismetArrayLibrary.Array_Length` (`self.Level Suffixes`))) :`false` _returnvalue :`true` (and _returnvalue (< (`local.Level`) (`.FromLevel_2_CE6A64F64E4499F64FBCEB9BC76B487A` (break `/Game/UltimateSurvivalPack/Blueprints/Structs/S_Level` (`|GetArrayItem` (`self.Level Suffixes`) _returnvalue_2))))))
      (`|ExecutionSequence`
        (:`then_0`
          (set `local.L Current Suffix` (`.Suffix_8_C9C420B14E5257FF7096859CC9BE7A04` (break `/Game/UltimateSurvivalPack/Blueprints/Structs/S_Level` (`local.L Current Array Element`)))))
        (:`then_1`
          (break)))))
  (return (`local.L Current Suffix`)))

(fn `Get Character Component`
  (returns (ReturnValue :type "/Game/UltimateSurvivalPack/Blueprints/Components/BP_PlayerComponent Object Reference"))
  (return (`Actor.GetComponentByClass` (`/Game/UltimateSurvivalPack/Blueprints/BFL_UMSPack.Get Human Player Character` (cast `Controller` (`self.GetOwner`) :!pure true)) "/Game/UltimateSurvivalPack/Blueprints/Components/BP_PlayerComponent.BP_PlayerComponent_C")))

(fn `Get Level Information`
  (params (Level :type Integer))
  (returns (`Maximum Total XP` :type Integer) (`Minimum Total XP` :type Integer) (`Maximum Current XP` :type Integer) (`Minimum Current XP` :type Integer) (`Actual Current XP` :type Integer))
  (bind _returnvalue (* (`self.Maximum Experience Range`) Level))
  (bind _returnvalue_2 (* (- Level 1) (`KismetMathLibrary.FTrunc` (* (`self.Maximum Experience Range`) (* Level 0.5)))))
  (bind _returnvalue_3 (+ _returnvalue_2 _returnvalue))
  (return _returnvalue_3 _returnvalue_2 (select `bool` (`self.Restart Points on Levelup`) :`false` _returnvalue_3 :`true` _returnvalue) (select `bool` (`self.Restart Points on Levelup`) :`false` _returnvalue_2) (select `bool` (`self.Restart Points on Levelup`) :`false` (`self.Total Experience Points`) :`true` (- (`self.Total Experience Points`) _returnvalue_2))))

(fn `On Experience Changed`
  (params (XP :type Integer))
  (returns (`Current XP` :type Integer) (`Maximum XP` :type Integer) (`Minimum XP` :type Integer) (Success :type Boolean))
  (bind _level (`self.Level`))
  (bind _level_skipping (`self.Level Skipping`))
  (bind (_maximum_total_xp _minimum_total_xp _maximum_current_xp) (`self.Get Level Information` (`self.Level`)))
  (bind (_maximum_total_xp_2 _minimum_total_xp_2 _maximum_current_xp_2 _minimum_current_xp _actual_current_xp) (`self.Get Level Information` (`self.Level`)))
  (bind (_maximum_total_xp_3 _minimum_total_xp_3 _maximum_current_xp_3 _minimum_current_xp_2 _actual_current_xp_2) (`self.Get Level Information` (`self.Level`)))
  (bind (_maximum_total_xp_4 _minimum_total_xp_4 _maximum_current_xp_4 _minimum_current_xp_3 _actual_current_xp_3) (`self.Get Level Information` (`self.Level`)))
  ;[1 1 1] Is not equal 0
  (if (!= XP 0)
    ;[1 1 1] Calculate new experience points
    (set `self.Total Experience Points` (`KismetMathLibrary.Clamp` (+ (`local.XP`) (`self.Total Experience Points`)) (select `bool` (`self.Decrease Level`) :`false` (`.Minimum Total XP` (`self.Get Level Information` (`self.Level`)))) (`self.Get Level Information` (`KismetMathLibrary.Clamp` (select `bool` (> _level_skipping 1) :`false` (`self.Maximum Level`) :`true` (+ (`self.Level`) (- _level_skipping 1))) 1 (`self.Maximum Level`)))))
    ;[1 1 1] Is Experience Incerasing
    (if (> (`local.XP`) 0)
      ;[1 1 1] Experience Incerase
      ;;[1 1 1] Is current XP higher than Maximum range multiplied by level
      (if (>= (`self.Total Experience Points`) _maximum_total_xp_3) :!label _label
        (if (< (`self.Level`) (`self.Maximum Level`))
          ;;[1 1 1] Set Level
          (set `self.Level` (+ (`KismetMathLibrary.Clamp` (`self.Level`) 1 (`self.Maximum Level`)) 1))
          ;;[1 1 1] Set Current Level Suffix
          (set `self.Level Suffix` (`self.Find Level Suffix` _level))
          ;;[1 1 1] Create Notification On Level Up
          (if (`self.Enable Levelup Notifycation`)
            (`self.CLIENT Add Notification` (make `/Game/UltimateSurvivalPack/Blueprints/Structs/S_Notification` "Level up!" (`KismetStringLibrary.Concat_StrStr` "You have now reached Level " (`KismetStringLibrary.Conv_IntToString` _level))))
            (goto _label)
            (else
              (goto _label)))
          (else
            ;;[0.5 1 0.35] Return
            (return _maximum_current_xp _maximum_current_xp _minimum_total_xp true) ; Reaching Maximum Level and it's maximum Experience Points
          ))
        (else
          ;;[0.5 1 0.35] Return
          (return _actual_current_xp_2 _maximum_current_xp_3 _minimum_current_xp_2 true)))
      (else
        ;[1 1 1] Experience Decerase
        (if (< (`self.Total Experience Points`) (`.Minimum Total XP` (`self.Get Level Information` (`self.Level`)))) :!label _label_2
          (if (`self.Decrease Level`)
            ;;[1 1 1] Set Level
            (set `self.Level` (- (`KismetMathLibrary.Clamp` (`self.Level`) 1 (`self.Maximum Level`)) 1))
            ;;[1 1 1] Set Current Level Suffix
            (set `self.Level Suffix` (`self.Find Level Suffix` (`self.Level`)))
            (goto _label_2))
          (else
            ;;[0.5 1 0.35] Return
            (return _actual_current_xp _maximum_current_xp_2 _minimum_current_xp true)))))
    (else
      ;[1 0.1 0.1] Return Failed
      (return _actual_current_xp_3 _maximum_current_xp_4 _minimum_current_xp_3 false))))