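; BP_Environmental is a mineable environment resource that loses health to damage, drops items when depleted and respawns after a timeout.
; Point damage is scaled by a per-damage-type multiplier, ignoring unlisted types, while any damage multicasts a hit sound.
; Depletion spawns chance-based items with random amounts around a spawn point.
; Mined replicates through a dormancy flush, and its OnRep swaps normal and destroyed meshes; damage widget logic is disconnected.
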(event `self.ReceiveAnyDamage`
  (params (Damage :type "Float (single-precision)") (DamageType :type "DamageType Object Reference") (InstigatedBy :type "Controller Object Reference") (DamageCauser :type "Actor Object Reference"))
  ;[1 1 1] Spawn Sound On Damage
  (`parent.ReceiveAnyDamage` Damage DamageType InstigatedBy DamageCauser)
  (`self.Multicast Spawn Sound`))

(event `Multicast Spawn Sound`
  ;[1 1 1] Spawn Sound On Damage
  (`GameplayStatics.SpawnSoundAtLocation` (`self.Sound`) (`self.K2_GetActorLocation`) (struct) 1.0 1.0 0.0 "/Game/UltimateSurvivalPack/Blueprints/Attenuation/SA_Footsteps.SA_Footsteps" null))

(event `self.ReceivePointDamage`
  (params (Damage :type "Float (single-precision)") (DamageType :type "DamageType Object Reference") (HitLocation :type "Vector Structure") (HitNormal :type "Vector Structure") (HitComponent :type "PrimitiveComponent Object Reference") (BoneName :type Name) (ShotFromDirection :type "Vector Structure") (InstigatedBy :type "Controller Object Reference") (DamageCauser :type "Actor Object Reference") (HitInfo :type "HitResult Structure (by ref)"))
  (bind (_value _returnvalue) (`BlueprintMapLibrary.Map_Find` (`self.Damage Types Multiplier`) (`GameplayStatics.GetObjectClass` DamageType)))
  ;[0 0 0] On Damaged
  ;;[1 1 1] Determine if Can be Damaged, decerase health
  (if (> (`self.Health`) 0.0)
    (if _returnvalue
      (bind _output_get (set `self.Health` (`KismetMathLibrary.FClamp` (- (`self.Health`) (* Damage _value)) 0.0 (`self.Maximum Health`))))
      (if (<= _output_get 0.0)
        ;;[1 1 1] If health is 0, flush network and call mined
        (set `self.Mined` true)
        (set `self.bCanBeDamaged` false)
        (`self.FlushNetDormancy`)
        (`self.ForceNetUpdate`)
        ;;[1 1 1] Spawn Item
        (`self.Drop Items`)
        ;;[1 1 1] Init Respawn and Flush Network
        (`KismetSystemLibrary.RetriggerableDelay` (`self.Respawn Timeout`))
        (set `self.Health` (`self.Maximum Health`))
        (set `self.Mined` false)
        (set `self.bCanBeDamaged` true)
        (`self.FlushNetDormancy`)
        (`self.ForceNetUpdate`)))))

(event `On Mined`
  ;[1 1 1] Networked Events
  (`StaticMeshComponent.SetStaticMesh` (`self.StaticMesh`) (`self.Destroyed Mesh`)))

(event `Respawn`
  ;[1 1 1] Networked Events
  (`StaticMeshComponent.SetStaticMesh` (`self.StaticMesh`) (`self.Normal Mesh`)))

(fn `Drop Items`
  (for _array_element (`self.Mined Item ID`)
    (bind (_itemid _minimumamount _maximumamount _chanceofspawning) (break `/Game/UltimateSurvivalPack/Blueprints/Structs/S_DropItem` _array_element))
    (if (<= (`KismetMathLibrary.RandomFloatInRange` 0.0 100.0) _chanceofspawning)
      (`|SpawnActorFromClass` "/Game/UltimateSurvivalPack/Blueprints/BP_InventoryItem.BP_InventoryItem_C" (`KismetMathLibrary.MakeTransform` (`KismetMathLibrary.RandomPointInBoundingBox` (`SceneComponent.K2_GetComponentLocation` (`self.Item Spawn location`)) (50.0 50.0 50.0))) "AdjustIfPossibleButAlwaysSpawn" "OverrideRootScale" null (make `/Game/UltimateSurvivalPack/Blueprints/Structs/S_InventoryItem` _itemid (`KismetMathLibrary.RandomIntegerInRange` _minimumamount _maximumamount)) null null)))
  (return))

(fn `OnRep_Mined`
  (if (`self.Mined`)
    (`self.On Mined`)
    (else
      (`self.Respawn`))))

(fn `UserConstructionScript`
  ;[1 1 1] Set Default mesh
  (`StaticMeshComponent.SetStaticMesh` (`self.StaticMesh`) (`self.Normal Mesh`))
  ;[1 1 1] Used for mining tools to determine if hit collision can be mined
  (`KismetArrayLibrary.Array_AddUnique` (`self.Tags`) "Mineable"))