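; BP_CarSpawner spawns a vehicle of a configurable class at its own location and yaw when RequestRespawn is called.
; After a short random delay, a non-zero CarLimit gates spawning on the world's BP_Buggy count and a box trace for blocking vehicles.
; A zero limit skips both checks.
; The spawned vehicle receives random health and a reference back to this spawner.
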(event `/Game/UltimateSurvivalPack/Blueprints/Interface/BPI_Spawning.Request Respawn`
  (bind _returnvalue (`self.K2_GetActorLocation`))
  (bind (_returnvalue_roll _returnvalue_pitch _returnvalue_yaw) (`KismetMathLibrary.BreakRotator` (`self.K2_GetActorRotation`)))
  ;[1 1 1] On requested respanw spawn car
  (`KismetSystemLibrary.Delay` (`KismetMathLibrary.RandomFloatInRange` 0.0 0.1))
  (if (!= (`self.Car Limit`) 0)
    (bind _outactors (`GameplayStatics.GetAllActorsOfClass` "/Game/UltimateSurvivalPack/Blueprints/VehicleBP/BP_Buggy.BP_Buggy_C"))
    (if (<= (`KismetArrayLibrary.Array_Length` _outactors) (`KismetMathLibrary.Conv_ByteToInt` (`self.Car Limit`)))
      (bind (_outhit _returnvalue_2) (`KismetSystemLibrary.BoxTraceSingleForObjects` _returnvalue _returnvalue (200.0 200.0 50.0) (struct) (`|MakeArray` "ObjectTypeQuery5" :!type "EObjectTypeQuery Enum")))
      (if (not _returnvalue_2)
        (`|SpawnActorFromClass` (`self.Vehicle Class`) (`KismetMathLibrary.MakeTransform` (`self.K2_GetActorLocation`) (`KismetMathLibrary.MakeRotator` 0.0 0.0 _returnvalue_yaw)) "AlwaysSpawn" "SelectDefaultAtRuntime" null 30.0 3.0 "" false (`KismetMathLibrary.RandomFloatInRange` 200.0 700.0) 700.0 (-1.0 -1.0 -1.0) self null :!label _label)))
    (else
      (goto _label))))

(fn `UserConstructionScript`)