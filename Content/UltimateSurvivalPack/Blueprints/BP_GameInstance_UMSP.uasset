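; Game instance for the survival pack that owns the persistent save of players, buildings and vehicles.
; On Init it loads or creates the SAV_ServerData PlayerSave object and sets resolution quality and a frame cap.
; Helper functions edit its maps and write to the slot, often gated by IsCurrentLevelSaveable, with retriggerable delays batching player and building saves.
; New buildings get random numeric IDs, rerolled on collision.
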(event `self.ReceiveInit`
  (`parent.ReceiveInit`)
  (`|ExecutionSequence`
    (:`then_0`
      (bind _returnvalue (`GameplayStatics.LoadGameFromSlot` "PlayerSave"))
      (`/Engine/EditorBlueprintResources/StandardMacros.IsValid` _returnvalue
        (:`Is Valid`
          (bind _assav_server_data (cast `/Game/UltimateSurvivalPack/Blueprints/Save/SAV_ServerData` _returnvalue))
          (set `self.Player Save` _assav_server_data))
        (:`Is Not Valid`
          (bind _returnvalue_2 (`GameplayStatics.CreateSaveGameObject` "/Game/UltimateSurvivalPack/Blueprints/Save/SAV_ServerData.SAV_ServerData_C"))
          (set `self.Player Save` _returnvalue_2))))
    (:`then_1`
      (`KismetSystemLibrary.ExecuteConsoleCommand` "sg.resolutionquality 100" null)
      (`KismetSystemLibrary.ExecuteConsoleCommand` "t.maxfps 144" null))))

(event `Save Building`
  (params (`Build ID` :type "String (by ref)") (`New Save` :type "/Game/UltimateSurvivalPack/Blueprints/Structs/S_BuildSave Structure (by ref)"))
  (`BlueprintMapLibrary.Map_Add` (`/Game/UltimateSurvivalPack/Blueprints/Save/SAV_ServerData.Build Saves` (`self.Player Save`)) `Build ID` `New Save`)
  (if (`/Game/UltimateSurvivalPack/Blueprints/BFL_UMSPack.Is Current Level Saveable`)
    (`KismetSystemLibrary.RetriggerableDelay` 0.2)
    (`GameplayStatics.SaveGameToSlot` (`self.Player Save`) "PlayerSave")))

(event `Save Building Directly`
  (params (`Build ID` :type "String (by ref)") (`New Save` :type "/Game/UltimateSurvivalPack/Blueprints/Structs/S_BuildSave Structure (by ref)"))
  (`BlueprintMapLibrary.Map_Add` (`/Game/UltimateSurvivalPack/Blueprints/Save/SAV_ServerData.Build Saves` (`self.Player Save`)) `Build ID` `New Save`)
  (if (`/Game/UltimateSurvivalPack/Blueprints/BFL_UMSPack.Is Current Level Saveable`)
    (`GameplayStatics.SaveGameToSlot` (`self.Player Save`) "PlayerSave")))

(event `Save Game Delayed`
  (`KismetSystemLibrary.RetriggerableDelay` 1.0)
  (`GameplayStatics.SaveGameToSlot` (`self.Player Save`) "PlayerSave"))

(fn `Add New Building`
  (params (`Build Data` :type "/Game/UltimateSurvivalPack/Blueprints/Structs/S_BuildSave Structure"))
  (returns (`Build ID` :type String))
  (locals (`L Normal ID` :type Integer :default 0))
  (bind _output_get (set `local.L Normal ID` (`KismetMathLibrary.RandomInteger` 999999999) :!label _label))
  (if (not (`.ReturnValue` (`BlueprintMapLibrary.Map_Find` (`/Game/UltimateSurvivalPack/Blueprints/Save/SAV_ServerData.Build Saves` (`self.Player Save`)) (`KismetStringLibrary.Conv_IntToString` _output_get))))
    (`BlueprintMapLibrary.Map_Add` (`/Game/UltimateSurvivalPack/Blueprints/Save/SAV_ServerData.Build Saves` (`self.Player Save`)) (`KismetStringLibrary.Conv_IntToString` (`local.L Normal ID`)) (make `/Game/UltimateSurvivalPack/Blueprints/Structs/S_BuildSave` :`Build Data` `Build Data_BuildData_2_700EB4E148DBEF7281188785324662CA` :`Transform` `Build Data_Transform_6_227D833D45720C2C90F11EB731C1BBAA` :`On Attached Actor` `Build Data_OnAttachedActor_9_07069BCA4FEF9223D5BEC6BA5C09F0C5` :`World Name` `Build Data_WorldName_11_6840022640BD07C9638712B3FDD0588F` :`Health` `Build Data_Health_35_3685E417491C5C60374FFFA4E51A29DB`))
    (if (`/Game/UltimateSurvivalPack/Blueprints/BFL_UMSPack.Is Current Level Saveable`)
      (`GameplayStatics.SaveGameToSlot` (`self.Player Save`) "PlayerSave"))
    (return (`KismetStringLibrary.Conv_IntToString` (`local.L Normal ID`)))
    (else
      (goto _label))))

(fn `Add Vehicle Save`
  (params (Key :type "String (by ref)") (Value :type "/Game/UltimateSurvivalPack/Blueprints/Structs/S_VehicleSaveData Structure (by ref)"))
  (if (`/Game/UltimateSurvivalPack/Blueprints/BFL_UMSPack.Is Current Level Saveable`)
    (`BlueprintMapLibrary.Map_Add` (`/Game/UltimateSurvivalPack/Blueprints/Save/SAV_ServerData.Vehicle Saves` (`self.Player Save`)) Key Value)
    (`GameplayStatics.SaveGameToSlot` (`self.Player Save`) "PlayerSave")
    (return)
    (else
      (return))))

(fn `Get Saved Data`
  (params (`Build ID` :type String))
  (returns (`Saved Data` :type "/Game/UltimateSurvivalPack/Blueprints/Structs/S_BuildSave Structure") (ReturnValue :type Boolean))
  (bind (_value _returnvalue) (`BlueprintMapLibrary.Map_Find` (`/Game/UltimateSurvivalPack/Blueprints/Save/SAV_ServerData.Build Saves` (`self.Player Save`)) `Build ID`))
  (return _value _returnvalue))

(fn `Remove Building`
  (params (`Build ID` :type String))
  (`BlueprintMapLibrary.Map_Remove` (`/Game/UltimateSurvivalPack/Blueprints/Save/SAV_ServerData.Build Saves` (`self.Player Save`)) `Build ID`)
  (`GameplayStatics.SaveGameToSlot` (`self.Player Save`) "PlayerSave"))

(fn `Remove Vehicle Save`
  (params (Key :type "String (by ref)"))
  (if (`/Game/UltimateSurvivalPack/Blueprints/BFL_UMSPack.Is Current Level Saveable`)
    (`BlueprintMapLibrary.Map_Remove` (`/Game/UltimateSurvivalPack/Blueprints/Save/SAV_ServerData.Vehicle Saves` (`self.Player Save`)) Key)
    (`GameplayStatics.SaveGameToSlot` (`self.Player Save`) "PlayerSave")
    (return)
    (else
      (return))))

(fn `Save Existing Building`
  (params (`Build ID` :type String) (`New Save` :type "/Game/UltimateSurvivalPack/Blueprints/Structs/S_BuildSave Structure"))
  (`self.Save Building` `Build ID` `New Save`))

(fn `Save Player Data`
  (params (`Player ID` :type String) (Save :type "/Game/UltimateSurvivalPack/Blueprints/Structs/S_PlayerSave Structure (by ref)"))
  (`BlueprintMapLibrary.Map_Add` (`/Game/UltimateSurvivalPack/Blueprints/Save/SAV_ServerData.Players Save` (`self.Player Save`)) `Player ID` Save)
  (`self.Save Game Delayed`)
  (return))