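; BP_Fire is a temporary fire hazard actor that damages anything inside its sphere until it burns out.
; The server runs a looping one-second timer that applies point damage, typed as explosion damage, to every actor overlapping the sphere.
; After FireLifeTime, a multicast event plays a timeline that animates the actor's scale as it disappears, and the server destroys the actor when the timeline finishes.
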(event `self.ReceiveBeginPlay`
  (`/Engine/EditorBlueprintResources/ActorMacros.Switch Has Authority`
    (:`Authority`
      (`|ExecutionSequence`
        (:`then_0`
          (`KismetSystemLibrary.Delay` (`self.Fire Life Time`))
          (`self.MULTICAST Fire disappear`))
        (:`then_1`
          (`KismetSystemLibrary.K2_SetTimerDelegate` (delegate `Apply Damage in Radius`) 1.0 true))))))

(event `Apply Damage in Radius`
  (for _array_element (`PrimitiveComponent.GetOverlappingActors` (`self.Sphere`) "/Script/Engine.Actor")
    (`GameplayStatics.ApplyPointDamage` _array_element 10.0 (`self.K2_GetActorLocation`) (`GameplayStatics.MakeHitResult` false) null self "/Game/UltimateSurvivalPack/Blueprints/DamageType/DT_Explosion.DT_Explosion_C")))

(event `MULTICAST Fire Disappear`
  ;[1 1 1] Play Animation
  (bind (_direction _animation) (`Timeline|Animation` :!via `PlayFromStart`)
    (:`Update`
      (`self.SetActorRelativeScale3D` (`KismetMathLibrary.Conv_DoubleToVector` _animation)))
    (:`Finished`
      (`/Engine/EditorBlueprintResources/ActorMacros.Switch Has Authority`
        (:`Authority`
          (`self.K2_DestroyActor`))))))

(fn `UserConstructionScript`)