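; BP_Throwable_Fishing is the thrown end of a fishing holdable's line, launched at the throw velocity and attached by rope to its holdable.
; On water hit it splashes, stops moving and loops a bobbing timeline.
; The authority alternates random wait and catch windows, using ranges from the holdable.
; CatchMode's RepNotify speeds up the bob, and each bob cycle ending during a catch window splashes again.
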(event `self.ReceiveBeginPlay`
  (bind _projectilemovement (`self.ProjectileMovement`))
  (bind _returnvalue (`KismetMathLibrary.VSize` (`self.Throw Velocity`)))
  ;[1 0.2448 0.2448] Simulate Phyiscs and Add Velocity
  (`PrimitiveComponent.IgnoreActorWhenMoving` (`self.ObjectMesh`) (`self.Instigator`) true)
  (set `ProjectileMovementComponent.InitialSpeed` _returnvalue _projectilemovement)
  (set `ProjectileMovementComponent.MaxSpeed` _returnvalue _projectilemovement)
  (set `MovementComponent.Velocity` (`self.Throw Velocity`) _projectilemovement)
  (`/Game/UltimateSurvivalPack/Blueprints/Holdable/HoldableActors/BP_Holdable_FishingRod.Attach Rope` (`self.Holdable Reference`) self))

(event `self.ProjectileMovement.OnProjectileStop`
  (params (ImpactResult :type "HitResult Structure (by ref)")))

(event `/Game/UltimateSurvivalPack/Blueprints/Interface/BPI_InventorySystem.Toggle Selected`
  (params (Toggle :type Boolean))
  (bind _objectmesh (`self.ObjectMesh`))
  (bind _objectmesh_2 (`self.ObjectMesh`))
  (if true
    (if Toggle
      (`PrimitiveComponent.SetRenderCustomDepth` _objectmesh_2 true)
      (`PrimitiveComponent.SetCustomDepthStencilValue` _objectmesh_2 1)
      (else
        (`PrimitiveComponent.SetRenderCustomDepth` _objectmesh false :!label _label)
        (`PrimitiveComponent.SetCustomDepthStencilValue` _objectmesh 0)))
    (else
      (goto _label))))

(event `self.On Water Hit`
  (params (Location :type "Vector Structure"))
  (`NiagaraFunctionLibrary.SpawnSystemAtLocation` "/Game/UltimateSurvivalPack/Demo/Particles/Niagara/NS_WaterSplash_Big.NS_WaterSplash_Big" Location)
  (`GameplayStatics.SpawnSoundAtLocation` "/Game/UltimateSurvivalPack/Demo/Audio/SFX/CUE_WaterSplash.CUE_WaterSplash" Location (struct) 1.0 1.0 0.0 "/Game/UltimateSurvivalPack/Blueprints/Attenuation/SA_Footsteps.SA_Footsteps" null)
  (`self.K2_SetActorLocation` Location)
  (`self.SetActorTickEnabled` false)
  (`ActorComponent.K2_DestroyComponent` (`self.ProjectileMovement`))
  (set `self.Hit Location` (`self.K2_GetActorLocation`))
  (`self.On Landed`))

(event `On Landed`
  (bind (_returnvalue_x _returnvalue_y) (`KismetMathLibrary.BreakVector` (`self.K2_GetActorLocation`)))
  (bind (_hit_location_x _hit_location_y _hit_location_z) (`KismetMathLibrary.BreakVector` (`self.Hit Location`)))
  (bind _hit_location (`self.Hit Location`))
  (`self.Do Catch Function`)
  (bind (_direction _alpha) (`Timeline|Animation` :!label _label_2)
    (:`Update`
      (`self.K2_SetActorLocation` (`KismetMathLibrary.MakeVector` _returnvalue_x _returnvalue_y (`KismetMathLibrary.Lerp` _hit_location_z (- _hit_location_z 10.0) _alpha))))
    (:`Finished`
      (if (`self.Catch Mode`)
        (`NiagaraFunctionLibrary.SpawnSystemAtLocation` "/Game/UltimateSurvivalPack/Demo/Particles/Niagara/NS_WaterSplash_Big.NS_WaterSplash_Big" _hit_location)
        (`GameplayStatics.SpawnSoundAtLocation` "/Game/UltimateSurvivalPack/Demo/Audio/SFX/CUE_WaterSplash.CUE_WaterSplash" _hit_location (struct) 1.0 1.0 0.0 "/Game/UltimateSurvivalPack/Blueprints/Attenuation/SA_Footsteps.SA_Footsteps" null)
        (goto _label_2 :!via `PlayFromStart`)
        (else
          (goto _label_2 :!via `PlayFromStart`))))))

(event `Do Catch Function`
  (bind (_catch_length_min_max_x _catch_length_min_max_y) (`KismetMathLibrary.BreakVector2D` (`/Game/UltimateSurvivalPack/Blueprints/Holdable/HoldableActors/BP_Holdable_FishingRod.Catch Length Min/Max` (`self.Holdable Reference`))))
  (bind (_fishing_length_min_max_x _fishing_length_min_max_y) (`KismetMathLibrary.BreakVector2D` (`/Game/UltimateSurvivalPack/Blueprints/Holdable/HoldableActors/BP_Holdable_FishingRod.Fishing Length Min/Max` (`self.Holdable Reference`))))
  (if (`self.HasAuthority`)
    (`KismetSystemLibrary.Delay` (`KismetMathLibrary.RandomFloatInRange` _fishing_length_min_max_x _fishing_length_min_max_y))
    (set `self.Catch Mode` true)
    (`KismetSystemLibrary.Delay` (`KismetMathLibrary.RandomFloatInRange` _catch_length_min_max_x _catch_length_min_max_y))
    (set `self.Catch Mode` false)
    (`self.Do Catch Function`)))

(fn `Get Interaction Data`
  (returns (`Interaction Text` :type Text))
  (return (select `bool` false :`true` "Pick up Spear." :!type "Text")))

(fn `Get Team ID`
  (returns (`Team ID` :type Byte))
  (return 0))

(fn `Local Can Overlap`
  (returns (Success :type Boolean))
  (return false))

(fn `OnRep_Catch Mode`
  (`TimelineComponent.SetPlayRate` (`self.Animation`) (select `bool` (`self.Catch Mode`) :`false` 1.0 :`true` 5.0)))

(fn `UserConstructionScript`
  (`parent.UserConstructionScript`))