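; Parent actor for thrown objects that fly under physics and splash out when they land in water.
; On BeginPlay the mesh simulates physics at ThrowVelocity, and component hits raise its linear damping.
; On Tick, the authority runs a small sphere trace for BP_Water, then OnWaterHit spawns splash VFX and sound and destroys the actor.
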(event `self.ReceiveBeginPlay`
  ;[1 0.2448 0.2448] Simulate Phyiscs and Add Velocity
  (`PrimitiveComponent.SetSimulatePhysics` (`self.ObjectMesh`) true)
  (`PrimitiveComponent.SetAllPhysicsLinearVelocity` (`self.ObjectMesh`) (`self.Throw Velocity`) false))

(event `self.ObjectMesh.OnComponentHit`
  (params (HitComponent :type "PrimitiveComponent Object Reference") (OtherActor :type "Actor Object Reference") (OtherComp :type "PrimitiveComponent Object Reference") (NormalImpulse :type "Vector Structure") (Hit :type "HitResult Structure (by ref)"))
  (`PrimitiveComponent.SetLinearDamping` (`self.ObjectMesh`) 1.0))

(event `self.ReceiveTick`
  (params (DeltaSeconds :type "Float (single-precision)"))
  (bind _returnvalue (`self.K2_GetActorLocation`))
  ;[0.2777 0.6 1] Water Detection
  (`/Engine/EditorBlueprintResources/ActorMacros.Switch Has Authority`
    (:`Authority`
      (bind (_outhit _returnvalue_2) (`KismetSystemLibrary.SphereTraceSingleForObjects` _returnvalue _returnvalue 5.0 (`|MakeArray` "ObjectTypeQuery7" :!type "EObjectTypeQuery Enum")))
      (if _returnvalue_2
        (bind (_bblockinghit _binitialoverlap _time _distance _location _impactpoint _normal _impactnormal _physmat _hitactor) (`GameplayStatics.BreakHitResult` _outhit))
        (cast `/Game/UltimateSurvivalPack/Blueprints/BP_Water` _hitactor)
        (`self.On Water Hit` _impactpoint)))))

(event `On Water Hit`
  (params (Location :type "Vector Structure"))
  ;[0.3102 1 0.4051] Water Effects
  (`NiagaraFunctionLibrary.SpawnSystemAtLocation` "/Game/UltimateSurvivalPack/Demo/Particles/Niagara/NS_WaterSplash_Big.NS_WaterSplash_Big" Location)
  (`GameplayStatics.SpawnSoundAtLocation` "/Game/UltimateSurvivalPack/Demo/Audio/SFX/CUE_WaterSplash.CUE_WaterSplash" Location (struct) 1.0 1.0 0.0 "/Game/UltimateSurvivalPack/Blueprints/Attenuation/SA_Footsteps.SA_Footsteps" null)
  (`self.K2_DestroyActor`))

(fn `UserConstructionScript`)