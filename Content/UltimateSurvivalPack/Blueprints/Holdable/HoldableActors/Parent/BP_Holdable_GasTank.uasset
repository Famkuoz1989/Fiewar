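; Holdable gas tank that refuels vehicles with the primary action and siphons fuel from them with the aim action, using its inventory item's durability as the fuel store.
; On the owning client, Tick traces from the camera for BPI_VehicleSystem actors, caching the target and showing its fuel in a W_GasTank widget.
; SERVER events send interface messages to that target and adjust durability by the returned amount, with each fill request capped.
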(event `/Game/UltimateSurvivalPack/Blueprints/Interface/BPI_Player.Aiming Action`
  (params (Toggle :type Boolean))
  (if Toggle
    (bind _hit_actor (`self.Hit Actor`)
      (:`then`
        (`self.SERVER Remove Fuel` _hit_actor))
      (:`else`))))

(event `SERVER Remove Fuel`
  (params (Target :type "Object Object Reference"))
  (bind (_item_data_id _item_data_amount _item_data_cachedindex) (break `/Game/UltimateSurvivalPack/Blueprints/Structs/S_InventoryItem` (`self.Item Data`)))
  (bind (_item_data_id_2 _item_data_amount_2 _item_data_cachedindex_2) (break `/Game/UltimateSurvivalPack/Blueprints/Structs/S_InventoryItem` (`self.Item Data`)))
  (bind (_output_id _output_amount _output_cachedindex _output_inventoryreference _output_custominteger _output_durability) (break `/Game/UltimateSurvivalPack/Blueprints/Structs/S_InventoryItem` (`|GetArrayItem` (`/Game/UltimateSurvivalPack/Blueprints/Components/BP_MasterInventoryComponent.Inventory` (`/Game/UltimateSurvivalPack/Blueprints/BFL_UMSPack.Get Inventory Component` (`self.GetOwner`))) _item_data_cachedindex_2)))
  (if (< _output_durability 1.0)
    (bind _add_durability (message `/Game/UltimateSurvivalPack/Blueprints/Interface/BPI_VehicleSystem.Remove Fuel` Target))
    (if (> _add_durability 0.0)
      (`/Game/UltimateSurvivalPack/Blueprints/Components/BP_PlayerInventoryComponent.Decerase Durability` (`/Game/UltimateSurvivalPack/Blueprints/BFL_UMSPack.Get Inventory Component` (`self.GetOwner`)) _item_data_cachedindex (* _add_durability -1.0)))))

(event `/Game/UltimateSurvivalPack/Blueprints/Interface/BPI_Player.Primary Action`
  (params (Pressed :type Boolean))
  (if Pressed
    (bind _hit_actor (`self.Hit Actor`)
      (:`then`
        (`self.SERVER Add Fuel` _hit_actor))
      (:`else`))))

(event `SERVER Add Fuel`
  (params (Target :type "Object Object Reference"))
  (bind (_item_data_id _item_data_amount _item_data_cachedindex) (break `/Game/UltimateSurvivalPack/Blueprints/Structs/S_InventoryItem` (`self.Item Data`)))
  (bind (_item_data_id_2 _item_data_amount_2 _item_data_cachedindex_2) (break `/Game/UltimateSurvivalPack/Blueprints/Structs/S_InventoryItem` (`self.Item Data`)))
  (bind (_output_id _output_amount _output_cachedindex _output_inventoryreference _output_custominteger _output_durability) (break `/Game/UltimateSurvivalPack/Blueprints/Structs/S_InventoryItem` (`|GetArrayItem` (`/Game/UltimateSurvivalPack/Blueprints/Components/BP_MasterInventoryComponent.Inventory` (`/Game/UltimateSurvivalPack/Blueprints/BFL_UMSPack.Get Inventory Component` (`self.GetOwner`))) _item_data_cachedindex_2)))
  (bind _returnvalue (* _output_durability 100.0))
  (if (> _output_durability 0.0)
    (bind _take_durability (message `/Game/UltimateSurvivalPack/Blueprints/Interface/BPI_VehicleSystem.Add Fuel` Target (select `bool` (> _returnvalue 10.0) :`false` _returnvalue :`true` 10.0)))
    (if (> _take_durability 0.0)
      (`/Game/UltimateSurvivalPack/Blueprints/Components/BP_PlayerInventoryComponent.Decerase Durability` (`/Game/UltimateSurvivalPack/Blueprints/BFL_UMSPack.Get Inventory Component` (`self.GetOwner`)) _item_data_cachedindex _take_durability))))

(event `self.ReceiveTick`
  (params (DeltaSeconds :type "Float (single-precision)"))
  (bind _returnvalue (`GameplayStatics.GetPlayerCameraManager` 0))
  (bind _gas_widget (`self.Gas Widget`))
  (bind _returnvalue_2 (`PlayerCameraManager.GetCameraLocation` _returnvalue))
  (`parent.ReceiveTick` DeltaSeconds)
  ;[1 1 1] Switch on local
  (if (`self.Is Owner Local`)
    (bind (_outhit _returnvalue_3) (`KismetSystemLibrary.LineTraceSingle` _returnvalue_2 (+ _returnvalue_2 (* (`KismetMathLibrary.GetForwardVector` (`PlayerCameraManager.GetCameraRotation` _returnvalue)) 1000.0)) "TraceTypeQuery1" false (`|MakeArray` (`self.GetInstigator`) :!type "Actor Object Reference")))
    (if _returnvalue_3
      (bind (_bblockinghit _binitialoverlap _time _distance _location _impactpoint _normal _impactnormal _physmat _hitactor) (`GameplayStatics.BreakHitResult` _outhit))
      (if (`KismetSystemLibrary.DoesImplementInterface` _hitactor "/Game/UltimateSurvivalPack/Blueprints/Interface/BPI_VehicleSystem.BPI_VehicleSystem_C")
        (bind _output_get (set `self.Hit Actor` _hitactor))
        (`Widget.SetVisibility` _gas_widget "HitTestInvisible")
        (bind (_fuel_amount _max_fuel) (message `/Game/UltimateSurvivalPack/Blueprints/Interface/BPI_VehicleSystem.Get Fuel` _output_get))
        (`/Game/UltimateSurvivalPack/Widget/W_GasTank.Set Fuel` _gas_widget _fuel_amount _max_fuel)
        (else
          (`Widget.SetVisibility` (`self.Gas Widget`) "Hidden" :!label _label)
          (set `self.Hit Actor` null)))
      (else
        (goto _label)))))

(event `self.ReceiveBeginPlay`
  (`parent.ReceiveBeginPlay`)
  ;[1 1 1] Switch on local
  (if (`self.Is Owner Local`)
    ;[1 1 1] Create Gastank widget
    (bind _returnvalue (`|CreateWidget` "/Game/UltimateSurvivalPack/Widget/W_GasTank.W_GasTank_C"))
    (bind _output_get (set `self.Gas Widget` _returnvalue))
    (`UserWidget.AddToViewport` _output_get -1)))

(event `self.ReceiveDestroyed`
  (`parent.ReceiveDestroyed`)
  ;[1 1 1] Switch on local
  (if (`self.Is Owner Local`)
    (`Widget.RemoveFromParent` (`self.Gas Widget`))))

(fn `UserConstructionScript`
  (`parent.UserConstructionScript`))