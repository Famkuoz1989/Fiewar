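; Checkpoint objective actor that registers custom markers through the player's mission component and stores itself in its target information at construction.
; At BeginPlay it sets each marker's initial hide-animation state by pawn distance, then polls that distance on a looping timer.
; Paired DoOnce gates turn range changes into CheckpointOverlap calls, an event left empty here.
; DestroyCheckpoint plays the markers' hide animation with destroy-on-hide, once.
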(event `self.ReceiveBeginPlay`
  (`/Engine/EditorBlueprintResources/StandardMacros.IsValid` (`/Game/UltimateSurvivalPack/Blueprints/Components/BP_MissionComponent.HUD` (`/Game/UltimateSurvivalPack/Blueprints/BFL_UMSPack.Get Mission Component` (`GameplayStatics.GetPlayerController` 0)))
    (:`Is Valid`
      (`|ExecutionSequence`
        (:`then_0`
          ;[1 1 1] Add Marker
          (bind _marker_reference (`/Game/UltimateSurvivalPack/Blueprints/Components/BP_MissionComponent.Add Custom Marker` (`/Game/UltimateSurvivalPack/Blueprints/BFL_UMSPack.Get Mission Component` (`GameplayStatics.GetPlayerController` 0)) (`.Marker_11_0442BFA549B64EFAF2A6708C8F3D4046` (break `/Game/UltimateSurvivalPack/Blueprints/Structs/S_TargetInformation` (`self.Target Information`))) self))
          (set `self.Markers` _marker_reference)
          ;[1 1 1] Play Initial Widget Animations
          (for _array_element (`self.Markers`)
            (if (<= (`self.GetDistanceTo` (`Controller.K2_GetPawn` (`GameplayStatics.GetPlayerController` 0)) self) (`self.Overlap Distance`))
              (set `/Game/UltimateSurvivalPack/Widget/W_Marker.Is Hidden?` false _array_element)
              (`/Game/UltimateSurvivalPack/Widget/W_Marker.Play Hide Animation` _array_element "Forward" false)
              (else
                (set `/Game/UltimateSurvivalPack/Widget/W_Marker.Is Hidden?` true _array_element)
                (`/Game/UltimateSurvivalPack/Widget/W_Marker.Play Hide Animation` _array_element "Reverse" false)))))
        (:`then_1`
          (`KismetSystemLibrary.K2_SetTimerDelegate` (delegate `Check Distance`) 0.5 true))))))

(event `Check Distance`
  ;[1 1 1] Check Distance
  (if (<= (`self.GetDistanceTo` (`Controller.K2_GetPawn` (`GameplayStatics.GetPlayerController` 0)) self) (`self.Overlap Distance`))
    (`/Engine/EditorBlueprintResources/StandardMacros.DoOnce` false :!label _label
      (:`Completed`
        (`self.Checkpoint Overlap` true)
        (goto _label_2 :!via `Reset`)))
    (else
      (`/Engine/EditorBlueprintResources/StandardMacros.DoOnce` false :!label _label_2
        (:`Completed`
          (`self.Checkpoint Overlap` false)
          (goto _label :!via `Reset`))))))

(event `Checkpoint Overlap`
  (params (`Overlaping?` :type Boolean)))

(event `Destroy Checkpoint`
  ;[1 1 1] Destroy Checkpoint
  (`/Engine/EditorBlueprintResources/StandardMacros.DoOnce` false
    (:`Completed`
      (for _array_element (`self.Markers`)
        (`/Engine/EditorBlueprintResources/StandardMacros.IsValid` _array_element
          (:`Is Valid`
            (`/Game/UltimateSurvivalPack/Widget/W_Marker.Play Hide Animation` _array_element "Forward" true)))))))

(fn `UserConstructionScript`
  (bind (_targettype _uniqueid _amount _marker) (break `/Game/UltimateSurvivalPack/Blueprints/Structs/S_TargetInformation` (`self.Target Information`)))
  (set `self.Target Information` (make `/Game/UltimateSurvivalPack/Blueprints/Structs/S_TargetInformation` _targettype _uniqueid _amount _marker self)))