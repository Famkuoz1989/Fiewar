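; Player controller for the survival pack that maps hardcoded key and mouse input to gameplay and UI.
; Combat, quickslot, view and building input goes to the inventory component's held item via messages or casts, while menus, map, chat and HUD go through the mission component.
; Possession links the character to the inventory, and unpossessing drops the holdable.
; Also handles skip-revive by lethal self-damage, rain forwarding and a test startup mission.
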(event `Key|LeftMouseButton`
  (params (Key :type "Key Structure"))
  (bind _bp_playerinventorycomponent (`self.BP_PlayerInventoryComponent`))
  (bind _bp_missioncomponent (`self.BP_MissionComponent`))
  (bind _hud (`/Game/UltimateSurvivalPack/Blueprints/Components/BP_MissionComponent.HUD` _bp_missioncomponent))
  (bind _human_player_character (`/Game/UltimateSurvivalPack/Blueprints/Components/BP_PlayerInventoryComponent.Human Player Character` _bp_playerinventorycomponent))
  (bind _holdable_actor (`/Game/UltimateSurvivalPack/Blueprints/Components/BP_PlayerInventoryComponent.Holdable Actor` _bp_playerinventorycomponent))
  ;[1 1 1] Primary Action
  (:`Pressed`
    (if (and (`KismetSystemLibrary.IsValid` _bp_missioncomponent) (`KismetSystemLibrary.IsValid` _hud))
      (if (not (`/Game/UltimateSurvivalPack/Widget/W_HUD.Is Interactable Widget Visible` _hud))
        (`/Engine/EditorBlueprintResources/StandardMacros.IsValid` _holdable_actor
          (:`Is Valid`
            (message `/Game/UltimateSurvivalPack/Blueprints/Interface/BPI_Player.Primary Action` _holdable_actor true))
          (:`Is Not Valid`
            (message `/Game/UltimateSurvivalPack/Blueprints/Interface/BPI_Player.Primary Action` _human_player_character true))))))
  (:`Released`
    (`/Engine/EditorBlueprintResources/StandardMacros.IsValid` _holdable_actor
      (:`Is Valid`
        (message `/Game/UltimateSurvivalPack/Blueprints/Interface/BPI_Player.Primary Action` _holdable_actor false))
      (:`Is Not Valid`
        (message `/Game/UltimateSurvivalPack/Blueprints/Interface/BPI_Player.Primary Action` _human_player_character false)))))

(event `Key|One`
  (params (Key :type "Key Structure"))
  (bind _bp_playerinventorycomponent (`self.BP_PlayerInventoryComponent`))
  ;[1 1 1] Quickslot Usement
  (:`Pressed`
    (`/Game/UltimateSurvivalPack/Blueprints/Components/BP_MasterInventoryComponent.Use Item Call` _bp_playerinventorycomponent 0 _bp_playerinventorycomponent)))

(event `Key|Tab`
  (params (Key :type "Key Structure"))
  ;[1 0.1875 0.1875] All Input
  ;;[1 1 1] Toggle Mission Menu
  (:`Pressed`
    (`/Game/UltimateSurvivalPack/Blueprints/Components/BP_MissionComponent.Toggle Menu` (`self.BP_MissionComponent`) 0)))

(event `Key|Two`
  (params (Key :type "Key Structure"))
  (bind _bp_playerinventorycomponent (`self.BP_PlayerInventoryComponent`))
  ;[1 1 1] Quickslot Usement
  (:`Pressed`
    (`/Game/UltimateSurvivalPack/Blueprints/Components/BP_MasterInventoryComponent.Use Item Call` _bp_playerinventorycomponent 1 _bp_playerinventorycomponent)))

(event `Key|Three`
  (params (Key :type "Key Structure"))
  (bind _bp_playerinventorycomponent (`self.BP_PlayerInventoryComponent`))
  ;[1 1 1] Quickslot Usement
  (:`Pressed`
    (`/Game/UltimateSurvivalPack/Blueprints/Components/BP_MasterInventoryComponent.Use Item Call` _bp_playerinventorycomponent 2 _bp_playerinventorycomponent)))

(event `Key|RightMouseButton`
  (params (Key :type "Key Structure"))
  (bind _holdable_actor (`/Game/UltimateSurvivalPack/Blueprints/Components/BP_PlayerInventoryComponent.Holdable Actor` (`self.BP_PlayerInventoryComponent`)))
  ;[1 0.1875 0.1875] All Input
  ;;[1 1 1] Aiming Action
  (:`Pressed`
    (`/Game/UltimateSurvivalPack/Blueprints/Components/BP_PlayerInventoryComponent.Human Player Character` (`self.BP_PlayerInventoryComponent`)
      (:`then`
        (bind _holdable_actor_2 (`/Game/UltimateSurvivalPack/Blueprints/Components/BP_PlayerInventoryComponent.Holdable Actor` (`self.BP_PlayerInventoryComponent`))
          (:`then`
            (message `/Game/UltimateSurvivalPack/Blueprints/Interface/BPI_Player.Aiming Action` _holdable_actor_2 (not (`/Game/UltimateSurvivalPack/Widget/W_HUD.Is Interactable Widget Visible` (`/Game/UltimateSurvivalPack/Blueprints/Components/BP_MissionComponent.HUD` (`self.BP_MissionComponent`))))))
          (:`else`)))
      (:`else`)))
  (:`Released`
    (`/Engine/EditorBlueprintResources/StandardMacros.IsValid` _holdable_actor
      (:`Is Valid`
        (message `/Game/UltimateSurvivalPack/Blueprints/Interface/BPI_Player.Aiming Action` _holdable_actor false)))))

(event `Key|Four`
  (params (Key :type "Key Structure"))
  (bind _bp_playerinventorycomponent (`self.BP_PlayerInventoryComponent`))
  ;[1 1 1] Quickslot Usement
  (:`Pressed`
    (`/Game/UltimateSurvivalPack/Blueprints/Components/BP_MasterInventoryComponent.Use Item Call` _bp_playerinventorycomponent 3 _bp_playerinventorycomponent)))

(event `self.ReceiveUnPossess`
  (params (UnpossessedPawn :type "Pawn Object Reference"))
  (`parent.ReceiveUnPossess` UnpossessedPawn)
  ;[1 1 1] Is Unpossessed pawn a Player
  (if (`KismetArrayLibrary.Array_Contains` (`Actor.Tags` UnpossessedPawn) "Player")
    (`/Game/UltimateSurvivalPack/Blueprints/Components/BP_PlayerInventoryComponent.Remove Holdable Object` (`self.BP_PlayerInventoryComponent`) false)))

(event `Key|Five`
  (params (Key :type "Key Structure"))
  (bind _bp_playerinventorycomponent (`self.BP_PlayerInventoryComponent`))
  ;[1 1 1] Quickslot Usement
  (:`Pressed`
    (`/Game/UltimateSurvivalPack/Blueprints/Components/BP_MasterInventoryComponent.Use Item Call` _bp_playerinventorycomponent 4 _bp_playerinventorycomponent)))

(event `Key|M`
  (params (Key :type "Key Structure"))
  ;[1 0.1875 0.1875] All Input
  (:`Pressed`
    (`/Game/UltimateSurvivalPack/Blueprints/Components/BP_MissionComponent.Toggle Menu` (`self.BP_MissionComponent`) 1)))

(event `Key|P`
  (params (Key :type "Key Structure"))
  ;[1 0.1875 0.1875] All Input
  (:`Pressed`
    (`/Game/UltimateSurvivalPack/Blueprints/Components/BP_MissionComponent.Toggle Pause Menu` (`self.BP_MissionComponent`) :!label _label)))

(event `Key|Six`
  (params (Key :type "Key Structure"))
  (bind _bp_playerinventorycomponent (`self.BP_PlayerInventoryComponent`))
  ;[1 1 1] Quickslot Usement
  (:`Pressed`
    (`/Game/UltimateSurvivalPack/Blueprints/Components/BP_MasterInventoryComponent.Use Item Call` _bp_playerinventorycomponent 5 _bp_playerinventorycomponent)))

(event `Key|Escape` :paused true
  (params (Key :type "Key Structure"))
  ;[1 0.1875 0.1875] All Input
  (:`Pressed`
    (goto _label)))

(event `Key|Seven`
  (params (Key :type "Key Structure"))
  (bind _bp_playerinventorycomponent (`self.BP_PlayerInventoryComponent`))
  ;[1 1 1] Quickslot Usement
  (:`Pressed`
    (`/Game/UltimateSurvivalPack/Blueprints/Components/BP_MasterInventoryComponent.Use Item Call` _bp_playerinventorycomponent 6 _bp_playerinventorycomponent)))

(event `InputAxisKey|MouseWheelAxis`
  (params (AxisValue :type "Float (single-precision)"))
  ;[1 0.1875 0.1875] All Input
  ;;[1 1 1] Zoom Bigmap
  (`/Game/UltimateSurvivalPack/Blueprints/Components/BP_MissionComponent.Zoom Map` (`self.BP_MissionComponent`) AxisValue))

(event `Key|Eight`
  (params (Key :type "Key Structure"))
  (bind _bp_playerinventorycomponent (`self.BP_PlayerInventoryComponent`))
  ;[1 1 1] Quickslot Usement
  (:`Pressed`
    (`/Game/UltimateSurvivalPack/Blueprints/Components/BP_MasterInventoryComponent.Use Item Call` _bp_playerinventorycomponent 7 _bp_playerinventorycomponent)))

(event `Key|R`
  (params (Key :type "Key Structure"))
  (bind _holdable_actor (`/Game/UltimateSurvivalPack/Blueprints/Components/BP_PlayerInventoryComponent.Holdable Actor` (`self.BP_PlayerInventoryComponent`)))
  ;[1 0.1875 0.1875] All Input
  ;;[1 1 1] Reload If Holdable Class = Range Weapon
  (:`Pressed`
    (`/Engine/EditorBlueprintResources/StandardMacros.IsValid` _holdable_actor
      (:`Is Valid`
        (bind _asbp_holdable_range_weapon (cast `/Game/UltimateSurvivalPack/Blueprints/Holdable/HoldableActors/Parent/BP_Holdable_RangeWeapon` _holdable_actor))
        (`/Game/UltimateSurvivalPack/Blueprints/Holdable/HoldableActors/Parent/BP_Holdable_RangeWeapon.Reload` _asbp_holdable_range_weapon)))))

(event `Key|V`
  (params (Key :type "Key Structure"))
  ;[1 1 1] Quickslot Usement
  (:`Pressed`
    (`/Game/UltimateSurvivalPack/Blueprints/Components/BP_PlayerInventoryComponent.Set Viewmode` (`self.BP_PlayerInventoryComponent`) (not (`/Game/UltimateSurvivalPack/Blueprints/Components/BP_PlayerInventoryComponent.FirstPerson View` (`self.BP_PlayerInventoryComponent`))))))

(event `Key|I`
  (params (Key :type "Key Structure"))
  ;[1 0.1875 0.1875] All Input
  ;;[1 1 1] Input Info Menu
  (:`Pressed`
    (`/Game/UltimateSurvivalPack/Blueprints/Components/BP_MissionComponent.Toggle Menu` (`self.BP_MissionComponent`) 6)))

(event `Key|B`
  (params (Key :type "Key Structure"))
  (bind _holdable_actor (`/Game/UltimateSurvivalPack/Blueprints/Components/BP_PlayerInventoryComponent.Holdable Actor` (`self.BP_PlayerInventoryComponent`)))
  ;[1 0.1875 0.1875] All Input
  ;;[1 1 1] Reload If Holdable Class = Range Weapon
  (:`Pressed`
    (`/Engine/EditorBlueprintResources/StandardMacros.IsValid` _holdable_actor
      (:`Is Valid`
        (bind _asbp_holdable_range_weapon (cast `/Game/UltimateSurvivalPack/Blueprints/Holdable/HoldableActors/Parent/BP_Holdable_RangeWeapon` _holdable_actor))
        (`/Game/UltimateSurvivalPack/Blueprints/Holdable/HoldableActors/Parent/BP_Holdable_RangeWeapon.Change Firemode` _asbp_holdable_range_weapon)))))

(event `Key|MouseScrollUp`
  (params (Key :type "Key Structure"))
  (bind _holdable_actor (`/Game/UltimateSurvivalPack/Blueprints/Components/BP_PlayerInventoryComponent.Holdable Actor` (`self.BP_PlayerInventoryComponent`)))
  ;[1 1 1] Rotate Building Actor
  (:`Pressed`
    (`/Engine/EditorBlueprintResources/StandardMacros.IsValid` _holdable_actor
      (:`Is Valid`
        (bind _asbp_holdable_building (cast `/Game/UltimateSurvivalPack/Blueprints/Holdable/HoldableActors/BP_Holdable_Building` _holdable_actor))
        (`/Game/UltimateSurvivalPack/Blueprints/Holdable/HoldableActors/BP_Holdable_Building.Rotate Actor` _asbp_holdable_building true)))))

(event `Key|MouseScrollDown`
  (params (Key :type "Key Structure"))
  (bind _holdable_actor (`/Game/UltimateSurvivalPack/Blueprints/Components/BP_PlayerInventoryComponent.Holdable Actor` (`self.BP_PlayerInventoryComponent`)))
  ;[1 1 1] Rotate Building Actor
  (:`Pressed`
    (`/Engine/EditorBlueprintResources/StandardMacros.IsValid` _holdable_actor
      (:`Is Valid`
        (bind _asbp_holdable_building (cast `/Game/UltimateSurvivalPack/Blueprints/Holdable/HoldableActors/BP_Holdable_Building` _holdable_actor))
        (`/Game/UltimateSurvivalPack/Blueprints/Holdable/HoldableActors/BP_Holdable_Building.Rotate Actor` _asbp_holdable_building false)))))

(event `SERVER Skip Revive`
  (bind _returnvalue (`self.K2_GetPawn`))
  ;[1 0.1875 0.1875] All Input
  ;;[1 1 1] Is Player In Knocked State?
  (if (`/Game/UltimateSurvivalPack/Blueprints/Components/BP_PlayerInventoryComponent.Is Knocked` (`self.BP_PlayerInventoryComponent`))
    ;;[1 1 1] Apply Self Damage To Switch To Dead State.
    (`GameplayStatics.ApplyDamage` _returnvalue 99999.0 self _returnvalue "/Game/UltimateSurvivalPack/Blueprints/DamageType/DT_InternalDamage.DT_InternalDamage_C")))

(event `Key|Delete`
  (params (Key :type "Key Structure"))
  (bind _hud (`/Game/UltimateSurvivalPack/Blueprints/Components/BP_MissionComponent.HUD` (`self.BP_MissionComponent`)))
  (:`Pressed`
    (`/Engine/EditorBlueprintResources/StandardMacros.FlipFlop`
      (:`A`
        (`Widget.SetVisibility` _hud "Hidden"))
      (:`B`
        (`Widget.SetVisibility` _hud "Visible")))))

(event `Key|X`
  (params (Key :type "Key Structure"))
  ;[1 1 1] Skip Revive
  (:`Pressed`
    (`self.SERVER Skip Revive`)))

(event `Key|Enter`
  (params (Key :type "Key Structure"))
  (bind _bp_playerinventorycomponent (`self.BP_PlayerInventoryComponent`))
  ;[1 1 1] Open Chat
  (:`Pressed`
    (if (and (not (`/Game/UltimateSurvivalPack/Blueprints/Components/BP_PlayerInventoryComponent.Is Knocked` _bp_playerinventorycomponent)) (not (`/Game/UltimateSurvivalPack/Blueprints/Components/BP_PlayerInventoryComponent.Is Dead` _bp_playerinventorycomponent)) (not (`/Game/UltimateSurvivalPack/Widget/W_HUD.Is Interactable Widget Visible` (`/Game/UltimateSurvivalPack/Blueprints/Components/BP_MissionComponent.HUD` (`self.BP_MissionComponent`)))))
      (bind _chat_widget_reference (`self.Get Chat Widget`))
      (`/Game/UltimateSurvivalPack/LobbySystem/Widget/W_Chat.Open Ingame Chat` _chat_widget_reference))))

(event `self.ReceiveBeginPlay`
  (bind _missioncomponent (`/Game/UltimateSurvivalPack/Blueprints/BFL_UMSPack.Get Mission Component` (`GameplayStatics.GetPlayerController` 0)))
  (if (`self.IsLocalController`)
    (bind _returnvalue (`GameplayStatics.GetCurrentLevelName` true))
    (`WidgetBlueprintLibrary.SetInputMode_GameOnly` self)
    (if (`KismetStringLibrary.NotEqual_StrStr` _returnvalue "L_Demo")
      ;[1 1 1] Only For Testing Purposes!
      (`KismetSystemLibrary.Delay` 2.0)
      (`/Engine/EditorBlueprintResources/StandardMacros.IsValid` _missioncomponent
        (:`Is Valid`
          (if (`KismetArrayLibrary.Array_Contains` (`/Game/UltimateSurvivalPack/Blueprints/Components/BP_MissionComponent.Quest Log` _missioncomponent) (make `/Game/UltimateSurvivalPack/Blueprints/Structs/S_MissionDatabase` "/Game/UltimateSurvivalPack/Blueprints/Datatable/Mission/DT_Missions.DT_Missions" "mission:startup"))
            (`/Game/UltimateSurvivalPack/Blueprints/Components/BP_MissionComponent.Start Mission` _missioncomponent "/Game/UltimateSurvivalPack/Blueprints/Datatable/Mission/DT_Missions.DT_Missions" "mission:startup"))))
      (else
        (`KismetArrayLibrary.Array_Clear` (`/Game/UltimateSurvivalPack/Blueprints/Components/BP_MissionComponent.Quest Log` (`/Game/UltimateSurvivalPack/Blueprints/BFL_UMSPack.Get Mission Component` (`GameplayStatics.GetPlayerController` 0))))))))

(event `Key|Delete`
  (params (Key :type "Key Structure"))
  ;[1 1 1] Hide HUD
)

(event `Key|T`
  (params (Key :type "Key Structure"))
  (:`Pressed`
    (bind _holdable_actor (`/Game/UltimateSurvivalPack/Blueprints/Components/BP_PlayerInventoryComponent.Holdable Actor` (`self.BP_PlayerInventoryComponent`))
      (:`then`
        (bind _asbp_holdable_range_weapon (cast `/Game/UltimateSurvivalPack/Blueprints/Holdable/HoldableActors/Parent/BP_Holdable_RangeWeapon` _holdable_actor))
        (`/Game/UltimateSurvivalPack/Blueprints/Holdable/HoldableActors/Parent/BP_Holdable_RangeWeapon.Toggle Upgrade Mode` _asbp_holdable_range_weapon (not (`/Game/UltimateSurvivalPack/Blueprints/Holdable/HoldableActors/Parent/BP_Holdable_RangeWeapon.Upgrade Mode` _asbp_holdable_range_weapon))))
      (:`else`))))

(event `self.ReceivePossess`
  (params (PossessedPawn :type "Pawn Object Reference"))
  (bind _bp_playerinventorycomponent (`self.BP_PlayerInventoryComponent`))
  (`parent.ReceivePossess` PossessedPawn)
  (bind _asthird_person_character (cast `/Game/UltimateSurvivalPack/Blueprints/ThirdPersonCharacter` PossessedPawn))
  (`/Game/UltimateSurvivalPack/Blueprints/Components/BP_PlayerInventoryComponent.Human Player Character` _bp_playerinventorycomponent
    (:`then`)
    (:`else`
      (set `/Game/UltimateSurvivalPack/Blueprints/Components/BP_PlayerInventoryComponent.Human Player Character` _asthird_person_character _bp_playerinventorycomponent))))

(event `/Game/UltimateSurvivalPack/WeatherSystem/Blueprints/BI_MultiplayerDynamicWeatherSystem.On Rain`
  (params (`Raining?` :type Boolean))
  ;[1 1 1] On Rain
  (if (`self.IsLocalController`)
    (message `/Game/UltimateSurvivalPack/WeatherSystem/Blueprints/BI_MultiplayerDynamicWeatherSystem.Toggle Raining` (`/Game/UltimateSurvivalPack/Blueprints/Components/BP_PlayerInventoryComponent.Human Player Character` (`self.BP_PlayerInventoryComponent`)) `Raining?`)))

(fn `Get Chat Widget`
  (returns (`Chat Widget Reference` :type "/Game/UltimateSurvivalPack/LobbySystem/Widget/W_Chat Object Reference"))
  (bind _hud (`/Game/UltimateSurvivalPack/Blueprints/Components/BP_MissionComponent.HUD` (`self.BP_MissionComponent`)))
  (`/Engine/EditorBlueprintResources/StandardMacros.IsValid` _hud
    (:`Is Valid`
      (return (`/Game/UltimateSurvivalPack/Widget/W_PlayerStats.W_Chat` (`/Game/UltimateSurvivalPack/Widget/W_HUD.W_PlayerStats` _hud))))
    (:`Is Not Valid`
      (return null))))

(fn `UserConstructionScript`)