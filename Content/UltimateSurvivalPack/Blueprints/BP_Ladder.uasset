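; Climbable ladder actor that switches a locally controlled third-person character's player component into ladder state while inside its Box trigger.
; Interaction-interface overlap events toggle the Box's overlap generation, and Restart briefly suspends it with a retriggerable delay.
; Leaving the Box restores the default state and launches the character using its last movement input, unrotated by actor rotation, for Y and clamped Z velocity.
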(event `self.BPI_Interaction_BeginOverlap`
  (set `self.Local Overlaping` true)
  (if (`self.Local Overlaping`) :!label _label
    (set `PrimitiveComponent.bGenerateOverlapEvents` true (`self.Box`))
    (else
      (set `PrimitiveComponent.bGenerateOverlapEvents` false (`self.Box`)))))

(event `self.BPI_Interaction_EndOverlap`
  (set `self.Local Overlaping` false)
  (goto _label))

(event `Restart`
  (if (`self.Local Overlaping`)
    (set `PrimitiveComponent.bGenerateOverlapEvents` false (`self.Box`))
    (`KismetSystemLibrary.RetriggerableDelay` 1.0)
    (set `PrimitiveComponent.bGenerateOverlapEvents` (`self.Local Overlaping`) (`self.Box`))))

(event `self.Box.OnComponentBeginOverlap`
  (params (OverlappedComponent :type "PrimitiveComponent Object Reference") (OtherActor :type "Actor Object Reference") (OtherComp :type "PrimitiveComponent Object Reference") (OtherBodyIndex :type Integer) (bFromSweep :type Boolean) (SweepResult :type "HitResult Structure (by ref)"))
  (bind _asthird_person_character (cast `/Game/UltimateSurvivalPack/Blueprints/ThirdPersonCharacter` OtherActor))
  (if (`Pawn.IsLocallyControlled` _asthird_person_character)
    (`/Game/UltimateSurvivalPack/Blueprints/Components/BP_PlayerComponent.Enter Ladder State` (`/Game/UltimateSurvivalPack/Blueprints/ThirdPersonCharacter.BP_PlayerComponent` _asthird_person_character) self)))

(event `self.Box.OnComponentEndOverlap`
  (params (OverlappedComponent :type "PrimitiveComponent Object Reference") (OtherActor :type "Actor Object Reference") (OtherComp :type "PrimitiveComponent Object Reference") (OtherBodyIndex :type Integer))
  (bind _asthird_person_character (cast `/Game/UltimateSurvivalPack/Blueprints/ThirdPersonCharacter` OtherActor))
  (if (`Pawn.IsLocallyControlled` _asthird_person_character)
    (`/Game/UltimateSurvivalPack/Blueprints/Components/BP_PlayerComponent.Enter Default State` (`/Game/UltimateSurvivalPack/Blueprints/ThirdPersonCharacter.BP_PlayerComponent` _asthird_person_character))
    (bind (_returnvalue_x _returnvalue_y _returnvalue_z) (`KismetMathLibrary.BreakVector` (`KismetMathLibrary.LessLess_VectorRotator` (`PawnMovementComponent.GetLastInputVector` (`Character.CharacterMovement` _asthird_person_character)) (`self.K2_GetActorRotation` _asthird_person_character))))
    (`Character.LaunchCharacter` _asthird_person_character (`KismetMathLibrary.MakeVector` 0.0 (* _returnvalue_y 150.0) (`KismetMathLibrary.MapRangeClamped` _returnvalue_z 0.0 1.0 0.0 400.0)) false true)))

(fn `UserConstructionScript`)