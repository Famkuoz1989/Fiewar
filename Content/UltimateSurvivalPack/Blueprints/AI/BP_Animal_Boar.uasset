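; Boar animal AI character that runs its own behavior tree on possession and registers as a navigation invoker on the server.
; Construction picks one of three boar meshes at random.
; Damage adds the instigator's pawn as an enemy target and multicasts a hit sound, plus spine blood splash for non-bullet hits.
; Target updates switch between slow and faster walk speed, and death fades out its audio.
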(event `MULTICAST On Damage`
  (params (Melee :type Boolean))
  ;[1 1 1] On Damage
  (if Melee
    (`NiagaraFunctionLibrary.SpawnSystemAttached` "/Game/UltimateSurvivalPack/Demo/Particles/Niagara/NS_BloodSplash.NS_BloodSplash" (`self.Mesh`) "Spine_01" (0.0 0.0 0.0) (struct) "KeepRelativeOffset" true))
  (`GameplayStatics.PlaySoundAtLocation` "/Game/UltimateSurvivalPack/Demo/Audio/SFX/CUE_Boar_Hit.CUE_Boar_Hit" (`self.K2_GetActorLocation`) (struct) 1.0 1.0 0.0 "/Game/UltimateSurvivalPack/Blueprints/Attenuation/SA_Footsteps.SA_Footsteps" null null null))

(event `self.ReceiveAnyDamage`
  (params (Damage :type "Float (single-precision)") (DamageType :type "DamageType Object Reference") (InstigatedBy :type "Controller Object Reference") (DamageCauser :type "Actor Object Reference"))
  (bind _returnvalue (`Controller.K2_GetPawn` InstigatedBy))
  ;[1 1 1] On Damage Taken
  (`parent.ReceiveAnyDamage` Damage DamageType InstigatedBy DamageCauser)
  (`/Engine/EditorBlueprintResources/StandardMacros.IsValid` _returnvalue
    (:`Is Valid`
      (`|ExecutionSequence`
        (:`then_0`
          (`/Game/UltimateSurvivalPack/Blueprints/Components/BP_AI_DataComponent.Add Enemy Target` (`self.C_AI_DataComponent`) _returnvalue))
        (:`then_1`
          (cast `/Game/UltimateSurvivalPack/Blueprints/DamageType/DT_Bullet` DamageType
            (:`then`
              (`self.MULTICAST On Damage` false))
            (:`CastFailed`
              (`self.MULTICAST On Damage` true))))))))

(event `/Game/UltimateSurvivalPack/Blueprints/Interface/BPI_AI.On Target Updated`
  ;[1 1 1] On target Updated
  (if (<= (`KismetArrayLibrary.Array_Length` (`/Game/UltimateSurvivalPack/Blueprints/Components/BP_AI_DataComponent.Enemy Targets` (`self.C_AI_DataComponent`))) 0)
    (set `CharacterMovementComponent.MaxWalkSpeed` 100.0 (`self.CharacterMovement`))
    (else
      (set `CharacterMovementComponent.MaxWalkSpeed` 300.0 (`self.CharacterMovement`)))))

(event `self.ReceiveBeginPlay`
  (`/Engine/EditorBlueprintResources/ActorMacros.Switch Has Authority`
    (:`Authority`
      (`NavigationSystemV1.RegisterNavigationInvoker` (`NavigationSystemV1.GetNavigationSystem`) self 1500.0 2000.0))))

(event `self.MULTICAST On Dead`
  ;[1 1 1] Multicast on Dead
  (`parent.MULTICAST On Dead`)
  (`AudioComponent.FadeOut` (`self.Audio`) 0.5 0.0 "Linear"))

(event `self.ReceivePossessed`
  (params (NewController :type "Controller Object Reference"))
  ;[1 1 1] On Possessed
  (`parent.ReceivePossessed` NewController)
  (`AIController.RunBehaviorTree` (`AIBlueprintHelperLibrary.GetAIController` (`self.GetOwner`)) "/Game/UltimateSurvivalPack/Blueprints/AI/BT_Animal_Boar.BT_Animal_Boar"))

(fn `UserConstructionScript`
  (`parent.UserConstructionScript`)
  (`SkinnedMeshComponent.SetSkinnedAssetAndUpdate` (`self.Mesh`) (select `int` (`KismetMathLibrary.RandomIntegerInRange` 0 2) :`0` "/Game/UltimateSurvivalPack/Demo/Animals/Boar/SK_Boar_01.SK_Boar_01" :`1` "/Game/UltimateSurvivalPack/Demo/Animals/Boar/SK_Boar_02.SK_Boar_02" :`2` "/Game/UltimateSurvivalPack/Demo/Animals/Boar/SK_Boar_03.SK_Boar_03" :!type "SkeletalMesh Object Reference") true))