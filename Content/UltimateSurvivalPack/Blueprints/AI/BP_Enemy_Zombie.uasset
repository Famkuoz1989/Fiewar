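; Networked zombie enemy that runs BT_Zombie, with a server-chosen random mesh and walk speed.
; Perception and damage instigators feed targets to CAIDataComponent; the Attack action plays a swing, then timed DoAttack damages nearby targets ahead, or their attach parents.
; Damage flags IsHit in the blackboard; non-vehicle hits also cancel pending attacks.
; Multicasts replicate hit reactions, blood and sounds; shielding suppresses only the target hit effect.
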(event `MULTICAST On Vehicle Damage`
  ;[1 1 1] On Vehicle Damage
  (`NiagaraFunctionLibrary.SpawnSystemAttached` "/Game/UltimateSurvivalPack/Demo/Particles/Niagara/NS_BigBloodSplash.NS_BigBloodSplash" (`self.Mesh`) "Spine_01" (0.0 0.0 0.0) (struct) "SnapToTarget" true)
  (`GameplayStatics.PlaySoundAtLocation` "/Game/UltimateSurvivalPack/Demo/Audio/SFX/Zombie/CUE_Zombie_Death.CUE_Zombie_Death" (`self.K2_GetActorLocation`) (struct) 1.0 1.0 0.0 "/Game/UltimateSurvivalPack/Blueprints/Attenuation/SA_Footsteps.SA_Footsteps" null null null))

(event `self.ReceiveAnyDamage`
  (params (Damage :type "Float (single-precision)") (DamageType :type "DamageType Object Reference") (InstigatedBy :type "Controller Object Reference") (DamageCauser :type "Actor Object Reference"))
  (bind _returnvalue (`AIBlueprintHelperLibrary.GetBlackboard` (`AIBlueprintHelperLibrary.GetAIController` self)))
  ;[1 1 1] On Damaged
  (`parent.ReceiveAnyDamage` Damage DamageType InstigatedBy DamageCauser)
  (`/Engine/EditorBlueprintResources/StandardMacros.IsValid` InstigatedBy
    (:`Is Valid`
      (`/Game/UltimateSurvivalPack/Blueprints/Components/BP_AI_DataComponent.Add Enemy Target` (`self.C_AI_DataComponent`) (`Controller.K2_GetPawn` InstigatedBy)))
    (:`Is Not Valid`
      _))
  (`|ExecutionSequence`
    (:`then_0`
      (if (`KismetArrayLibrary.Array_Contains` (`|MakeArray` "/Game/UltimateSurvivalPack/Blueprints/DamageType/DT_Melee.DT_Melee_C" "/Game/UltimateSurvivalPack/Blueprints/DamageType/DT_PickaxeTool.DT_PickaxeTool_C" "/Game/UltimateSurvivalPack/Blueprints/DamageType/DT_AxeTool.DT_AxeTool_C" :!type "DamageType Class Reference") (`GameplayStatics.GetObjectClass` DamageType))
        (`self.MULTICAST On Damage` (`/Game/UltimateSurvivalPack/Blueprints/Components/BP_AI_DataComponent.Is Alive` (`self.C_AI_DataComponent`)) :!label _label)
        (`KismetSystemLibrary.K2_ClearAndInvalidateTimerHandle` (`self.Attack Timer`))
        (else
          (cast `/Game/UltimateSurvivalPack/Blueprints/DamageType/DT_Vehicle` DamageType
            (:`then`
              (`self.MULTICAST On Vehicle Damage`))
            (:`CastFailed`
              (if (== (`KismetMathLibrary.RandomIntegerInRange` 0 5) 5)
                (goto _label)
                (else
                  (goto _label))))))))
    (:`then_1`
      ;[1 1 1] Set BT
      (`BlackboardComponent.SetValueAsBool` _returnvalue "IsHit" true)
      (`KismetSystemLibrary.RetriggerableDelay` 1.0)
      (`BlackboardComponent.SetValueAsBool` _returnvalue "IsHit" false))))

(event `self.ReceivePossessed`
  (params (NewController :type "Controller Object Reference"))
  ;[1 1 1] Run Zombie Behavior on Possessed
  (`parent.ReceivePossessed` NewController)
  (`AIController.RunBehaviorTree` (`AIBlueprintHelperLibrary.GetAIController` (`self.GetOwner`)) "/Game/UltimateSurvivalPack/Blueprints/AI/BT_Zombie.BT_Zombie")
  ;[1 1 1] Set Random Walk Speed
  (set `CharacterMovementComponent.MaxWalkSpeed` (select `int` (`KismetMathLibrary.RandomIntegerInRange` 0 1) :`0` 200.0 :`1` 400.0) (`self.CharacterMovement`)))

(event `MULTICAST On Damage`
  (params (`Is Alive` :type Boolean))
  ;[1 1 1] Do Hit Effect on MUTLICAST
  (`self.PlayAnimMontage` "/Game/UltimateSurvivalPack/Demo/Character/Animations/Zombie/Montage/React_Heavy_Front_Montage.React_Heavy_Front_Montage")
  (`NiagaraFunctionLibrary.SpawnSystemAttached` "/Game/UltimateSurvivalPack/Demo/Particles/Niagara/NS_BloodSplash.NS_BloodSplash" (`self.Mesh`) "Spine_01" (0.0 0.0 0.0) (struct) "KeepRelativeOffset" true true "AutoRelease")
  (`GameplayStatics.PlaySoundAtLocation` (select `bool` `Is Alive` :`false` "/Game/UltimateSurvivalPack/Demo/Audio/SFX/Zombie/CUE_Zombie_Death.CUE_Zombie_Death" :`true` "/Game/UltimateSurvivalPack/Demo/Audio/SFX/Zombie/CUE_ZombieHit.CUE_ZombieHit" :!type "SoundBase Object Reference") (`self.K2_GetActorLocation`) (struct) 1.0 1.0 0.0 "/Game/UltimateSurvivalPack/Blueprints/Attenuation/SA_Footsteps.SA_Footsteps" "/Game/UltimateSurvivalPack/Blueprints/Other/SC_Environment.SC_Environment" null null))

(event `self.ReceiveBeginPlay`
  ;[1 1 1] Begin Play (Set Skeletal Mesh)
  (`/Engine/EditorBlueprintResources/ActorMacros.Switch Has Authority`
    (:`Authority`
      (bind _output_get (set `self.Mesh Number` (`KismetMathLibrary.RandomIntegerInRange` 0 4)))
      (`self.MULTICAST Set Mesh` _output_get))
    (:`Remote`
      (`SkinnedMeshComponent.SetSkinnedAssetAndUpdate` (`self.Mesh`) (select `int` (`self.Mesh Number`) :`0` "/Game/UltimateSurvivalPack/Demo/Character/Zombie/SK_Zombie_01.SK_Zombie_01" :`1` "/Game/UltimateSurvivalPack/Demo/Character/Zombie/SK_Zombie_02.SK_Zombie_02" :`2` "/Game/UltimateSurvivalPack/Demo/Character/Zombie/SK_Zombie_03.SK_Zombie_03" :`3` "/Game/UltimateSurvivalPack/Demo/Character/Zombie/SK_Zombie_04.SK_Zombie_04" :`4` "/Game/UltimateSurvivalPack/Demo/Character/Zombie/SK_Zombie_05.SK_Zombie_05" :!type "SkeletalMesh Object Reference") true))))

(event `MULTICAST Set Mesh`
  (params (`Mesh Number` :type Integer))
  ;[1 1 1] Set Mesh On Multicast
  (`SkinnedMeshComponent.SetSkinnedAssetAndUpdate` (`self.Mesh`) (select `int` `Mesh Number` :`0` "/Game/UltimateSurvivalPack/Demo/Character/Zombie/SK_Zombie_01.SK_Zombie_01" :`1` "/Game/UltimateSurvivalPack/Demo/Character/Zombie/SK_Zombie_02.SK_Zombie_02" :`2` "/Game/UltimateSurvivalPack/Demo/Character/Zombie/SK_Zombie_03.SK_Zombie_03" :`3` "/Game/UltimateSurvivalPack/Demo/Character/Zombie/SK_Zombie_04.SK_Zombie_04" :`4` "/Game/UltimateSurvivalPack/Demo/Character/Zombie/SK_Zombie_05.SK_Zombie_05" :!type "SkeletalMesh Object Reference") true))

(event `MULTICAST Hit Target`
  (params (Location :type "Vector Structure"))
  ;[1 1 1] Multicast Hit Target
  (`GameplayStatics.PlaySoundAtLocation` "/Game/UltimateSurvivalPack/Demo/Audio/SFX/CUE_BodyHit.CUE_BodyHit" Location (struct) 1.0 1.0 0.0 "/Game/UltimateSurvivalPack/Blueprints/Attenuation/SA_Footsteps.SA_Footsteps" null null null)
  (`NiagaraFunctionLibrary.SpawnSystemAtLocation` "/Game/UltimateSurvivalPack/Demo/Particles/Niagara/NS_BloodSplash.NS_BloodSplash" Location))

(event `self.AIPerception.OnTargetPerceptionUpdated`
  (params (Actor :type "Actor Object Reference") (Stimulus :type "AIStimulus Structure"))
  ;[1 1 1] On Updated Perception
  (`/Game/UltimateSurvivalPack/Blueprints/Components/BP_AI_DataComponent.On Perception Updated` (`self.C_AI_DataComponent`) Actor Stimulus))

(fn `DoAttack`
  (bind (_returnvalue_roll _returnvalue_pitch _returnvalue_yaw) (`KismetMathLibrary.BreakRotator` (`self.K2_GetActorRotation`)))
  (for _array_element (`/Game/UltimateSurvivalPack/Blueprints/Components/BP_AI_DataComponent.Enemy Targets` (`self.C_AI_DataComponent`))
    (bind _returnvalue (`self.GetAttachParentActor` _array_element))
    (bind _returnvalue_2 (`KismetSystemLibrary.IsValid` _returnvalue))
    (bind _returnvalue_3 (select `bool` _returnvalue_2 :`false` _array_element :`true` _returnvalue))
    (bind _returnvalue_4 (`self.K2_GetActorLocation` _array_element))
    (bind (_returnvalue_roll_2 _returnvalue_pitch_2 _returnvalue_yaw_2) (`KismetMathLibrary.BreakRotator` (`KismetMathLibrary.FindLookAtRotation` (`self.K2_GetActorLocation`) _returnvalue_4)))
    (if (and (< (`self.GetDistanceTo` _returnvalue_3) (select `bool` _returnvalue_2 :`false` 150.0 :`true` 400.0)) (< (`KismetMathLibrary.Abs` (- _returnvalue_yaw _returnvalue_yaw_2)) 90.0))
      (`GameplayStatics.ApplyDamage` _returnvalue_3 20.0 (`self.GetController`) self "/Game/UltimateSurvivalPack/Blueprints/DamageType/DT_Melee.DT_Melee_C")
      (bind _ascharacter (cast `Character` _array_element :!pure true))
      (`/Engine/EditorBlueprintResources/StandardMacros.IsValid` _ascharacter
        (:`Is Valid`
          (bind _returnvalue_5 (`/Game/UltimateSurvivalPack/Blueprints/BFL_UMSPack.Get Player Component` _ascharacter))
          (`/Engine/EditorBlueprintResources/StandardMacros.IsValid` _returnvalue_5
            (:`Is Valid`
              (bind _holdable_actor (`/Game/UltimateSurvivalPack/Blueprints/Components/BP_PlayerComponent.Holdable Actor` _returnvalue_5)
                (:`then`
                  (bind _asbp_holdable_meele_weapon_one_handed (cast `/Game/UltimateSurvivalPack/Blueprints/Holdable/HoldableActors/Parent/BP_Holdable_MeeleWeapon_OneHanded` _holdable_actor)
                    (:`then`
                      (if (not (`/Game/UltimateSurvivalPack/Blueprints/Holdable/HoldableActors/Parent/BP_Holdable_MeeleWeapon_OneHanded.Is Shielding` _asbp_holdable_meele_weapon_one_handed))
                        (`self.MULTICAST Hit Target` _returnvalue_4 :!label _label)))
                    (:`CastFailed`
                      (goto _label))))
                (:`else`
                  (goto _label))))
            (:`Is Not Valid`
              (goto _label))))
        (:`Is Not Valid`
          (goto _label))))))

(fn `Perform AI Action`
  (params (Action :type Name))
  (returns (Success :type Boolean))
  (switch `name` Action
    (:`Default`
      (return false))
    (:`Attack`
      (`self.MULTICAST Play Montage` "/Game/UltimateSurvivalPack/Demo/Character/Animations/Zombie/Montage/Enemy_Anim_Sword_Combat_Swing_Montage.Enemy_Anim_Sword_Combat_Swing_Montage")
      (`KismetSystemLibrary.K2_ClearAndInvalidateTimerHandle` (`self.Attack Timer`))
      (bind _returnvalue (`KismetSystemLibrary.K2_SetTimer` null "DoAttack" 0.2))
      (set `self.Attack Timer` _returnvalue)
      (return true))))

(fn `UserConstructionScript`
  (`parent.UserConstructionScript`))