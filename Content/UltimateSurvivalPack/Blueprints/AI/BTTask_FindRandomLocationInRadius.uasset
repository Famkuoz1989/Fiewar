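; Behavior tree task that picks a random navigable roaming destination for an AI pawn and writes it to a blackboard key.
; If the pawn's AI data component references an enemy camp, it searches within that camp's area sphere.
; Otherwise it searches within a set radius around the pawn's own location.
; It finishes with success when a point is found, or failure when none is.
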(event `self.ReceiveExecuteAI`
  (params (OwnerController :type "AIController Object Reference") (ControlledPawn :type "Pawn Object Reference"))
  (bind _returnvalue (`Actor.GetComponentByClass` ControlledPawn "/Game/UltimateSurvivalPack/Blueprints/Components/BP_AI_DataComponent.BP_AI_DataComponent_C"))
  ;[1 1 1] Determine is has AI Component
  (`/Engine/EditorBlueprintResources/StandardMacros.IsValid` _returnvalue
    (:`Is Valid`
      ;[1 1 1] If valid and has an enemy camp reference, get location only inside the area radius
      (bind _enemycamp (`/Game/UltimateSurvivalPack/Blueprints/Components/BP_AI_DataComponent.EnemyCamp` _returnvalue)
        (:`then`
          (bind (_randomlocation _returnvalue_2) (`NavigationSystemV1.K2_GetRandomLocationInNavigableRadius` (`Actor.K2_GetActorLocation` _enemycamp) (`SphereComponent.SphereRadius` (`/Game/UltimateSurvivalPack/Blueprints/BP_EnemyCamp.Area Collision` _enemycamp)) null null))
          (if _returnvalue_2
            (`BTFunctionLibrary.SetBlackboardValueAsVector` (`self.Destination Key`) _randomlocation)
            (`self.FinishExecute` true)
            (else
              ;[1 1 1] If not Valid, roam
              (`self.FinishExecute` false))))
        (:`else`
          (bind (_randomlocation_2 _returnvalue_3) (`NavigationSystemV1.K2_GetRandomLocationInNavigableRadius` (`Actor.K2_GetActorLocation` ControlledPawn) (`self.Radius`) null null :!label _label))
          (if _returnvalue_3
            (`BTFunctionLibrary.SetBlackboardValueAsVector` (`self.Destination Key`) _randomlocation_2)
            (`self.FinishExecute` true)
            (else
              (`self.FinishExecute` false))))))
    (:`Is Not Valid`
      (goto _label))))