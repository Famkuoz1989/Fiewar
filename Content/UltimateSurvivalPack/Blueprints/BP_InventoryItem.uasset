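; World pickup actor for an inventory item, taking its mesh from item data by ID and showing weapon attachments for ranged weapons.
; Interaction adds what fits to the executor's inventory, then either destroys the actor and starts any spawner's respawn timeout, or keeps the leftover amount.
; Selection toggles a custom-depth highlight.
; Tick sphere-traces for water to play splash effects, and switches itself off after a splash or once the item settles.
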(event `self.ReceiveBeginPlay`
  (bind _returnvalue (`self.K2_GetActorLocation`))
  (bind _item_data_id (break `/Game/UltimateSurvivalPack/Blueprints/Structs/S_InventoryItem` (`self.Item Data`)))
  (bind (_bisvalid _item_data) (`/Game/UltimateSurvivalPack/Blueprints/BFL_Inventory.Get Item Data from ID` _item_data_id))
  ;[1 1 1] Begin Play
  (`PrimitiveComponent.SetSimulatePhysics` (`self.Item Mesh`) (== (`self.Spawner Reference`) null))
  ;;[1 1 1] Set Preview Mesh
  (if _bisvalid
    (`StaticMeshComponent.SetStaticMesh` (`self.Item Mesh`) (`.ItemMesh_32_5AC0B44A4BF0D4ECC34C868B2CFC9CF3` (break `/Game/UltimateSurvivalPack/Blueprints/Structs/S_InventoryItemData` _item_data)))
    (`self.Load Attachments`)
    ;[1 1 1] Is Already In Water?
    (bind (_outhit _returnvalue_2) (`KismetSystemLibrary.SphereTraceSingleForObjects` _returnvalue _returnvalue 10.0 (`|MakeArray` "ObjectTypeQuery7" :!type "EObjectTypeQuery Enum")))
    (if _returnvalue_2
      (`self.SetActorTickEnabled` false))
    (else
      (`self.K2_DestroyActor`))))

(event `/Game/UltimateSurvivalPack/Blueprints/Interface/BPI_InventorySystem.Toggle Selected`
  (params (Toggle :type Boolean))
  (bind _item_mesh (`self.Item Mesh`))
  (bind _item_mesh_2 (`self.Item Mesh`))
  ;[1 1 1] On Selected
  (if Toggle
    (`PrimitiveComponent.SetRenderCustomDepth` _item_mesh_2 true)
    (`PrimitiveComponent.SetCustomDepthStencilValue` _item_mesh_2 1)
    (else
      (`PrimitiveComponent.SetRenderCustomDepth` _item_mesh false)
      (`PrimitiveComponent.SetCustomDepthStencilValue` _item_mesh 0))))

(event `/Game/UltimateSurvivalPack/Blueprints/Interface/BPI_InventorySystem.On Interacted`
  (params (Executor :type "Controller Object Reference"))
  (bind _returnvalue (`/Game/UltimateSurvivalPack/Blueprints/BFL_UMSPack.Get Inventory Component` Executor))
  (bind (_item_data_id _item_data_amount) (break `/Game/UltimateSurvivalPack/Blueprints/Structs/S_InventoryItem` (`self.Item Data`)))
  (bind (_item_data_id_2 _item_data_amount_2 _item_data_cachedindex _item_data_inventoryreference _item_data_custominteger _item_data_durability _item_data_additionaldata) (break `/Game/UltimateSurvivalPack/Blueprints/Structs/S_InventoryItem` (`self.Item Data`)))
  (bind _item_data_id_3 (break `/Game/UltimateSurvivalPack/Blueprints/Structs/S_InventoryItem` (`self.Item Data`)))
  (bind (_item_data_id_4 _item_data_amount_3) (break `/Game/UltimateSurvivalPack/Blueprints/Structs/S_InventoryItem` (`self.Item Data`)))
  (bind (_item_data_id_5 _item_data_amount_4) (break `/Game/UltimateSurvivalPack/Blueprints/Structs/S_InventoryItem` (`self.Item Data`)))
  ;[1 1 1] Find Free Space
  (bind _found_space (`/Game/UltimateSurvivalPack/Blueprints/Components/BP_MasterInventoryComponent.Find Free Space for Item` _returnvalue _item_data_id_3 -1 (`|MakeArray`)))
  (if (> _found_space 0)
    ;[1 1 1] Calculate add amount and double check for success
    (bind _success (`/Game/UltimateSurvivalPack/Blueprints/Components/BP_MasterInventoryComponent.Add Item` _returnvalue (make `/Game/UltimateSurvivalPack/Blueprints/Structs/S_InventoryItem` _item_data_id (`KismetMathLibrary.Clamp` _found_space 0 _item_data_amount) 0 null _item_data_custominteger _item_data_durability _item_data_additionaldata)))
    (if _success
      ;[1 1 1] Decide, if the item can be taken and destroyed, or only modified amount
      (if (>= _found_space _item_data_amount_3)
        (bind _spawner_reference (`self.Spawner Reference`)
          (:`then`
            (`/Game/UltimateSurvivalPack/Blueprints/BP_ItemSpawner.Start Respawn Timeout` _spawner_reference))
          (:`else`
            _))
        (`self.K2_DestroyActor`)
        (else
          (set `self.Item Data` (make `/Game/UltimateSurvivalPack/Blueprints/Structs/S_InventoryItem` _item_data_id_5 (- _item_data_amount_4 _found_space))))))))

(event `self.ReceiveTick`
  (params (DeltaSeconds :type "Float (single-precision)"))
  (bind _returnvalue (`self.K2_GetActorLocation`))
  (bind _item_mesh (`self.Item Mesh`))
  (`|ExecutionSequence`
    (:`then_0`
      (bind (_outhit _returnvalue_2) (`KismetSystemLibrary.SphereTraceSingleForObjects` _returnvalue _returnvalue 10.0 (`|MakeArray` "ObjectTypeQuery7" :!type "EObjectTypeQuery Enum")))
      (if _returnvalue_2
        (`NiagaraFunctionLibrary.SpawnSystemAtLocation` "/Game/UltimateSurvivalPack/Demo/Particles/Niagara/NS_WaterSplash_Big.NS_WaterSplash_Big" (`self.K2_GetActorLocation`))
        (`GameplayStatics.SpawnSoundAtLocation` "/Game/UltimateSurvivalPack/Demo/Audio/SFX/CUE_WaterSplash.CUE_WaterSplash" (`self.K2_GetActorLocation`) (struct) 0.75 1.0 0.0 "/Game/UltimateSurvivalPack/Blueprints/Attenuation/SA_Footsteps.SA_Footsteps" null)
        (`self.SetActorTickEnabled` false)
        (set `PrimitiveComponent.bIgnoreRadialImpulse` true _item_mesh)
        (set `PrimitiveComponent.bIgnoreRadialForce` false _item_mesh)))
    (:`then_1`
      (`/Engine/EditorBlueprintResources/StandardMacros.DoOnce` false :!label _label
        (:`Completed`
          (`|ExecutionSequence`
            (:`then_0`
              (`KismetSystemLibrary.Delay` 2.0)
              (if (< (`KismetMathLibrary.VSize` (`self.GetVelocity`)) 10.0)
                (`self.SetActorTickEnabled` false)))
            (:`then_1`
              (goto _label :!via `Reset`))))))))

(fn `Get Interaction Data`
  (returns (`Interaction Text` :type Text))
  (bind (_item_data_id _item_data_amount) (break `/Game/UltimateSurvivalPack/Blueprints/Structs/S_InventoryItem` (`self.Item Data`)))
  (bind (_bisvalid _item_data) (`/Game/UltimateSurvivalPack/Blueprints/BFL_Inventory.Get Item Data from ID` _item_data_id))
  (if _bisvalid
    (return (`|FormatText` "Pickup {amount}x {Itemname}" _item_data_amount (`.Name_22_1F2975454CE296A7C7033BA39535256F` (break `/Game/UltimateSurvivalPack/Blueprints/Structs/S_InventoryItemData` _item_data))))
    (else
      (return ""))))

(fn `Get Team ID`
  (returns (`Team ID` :type Byte))
  (return 0))

(fn `Load Attachments`
  (bind (_item_data_id _item_data_amount _item_data_cachedindex _item_data_inventoryreference _item_data_custominteger _item_data_durability _item_data_additionaldata) (break `/Game/UltimateSurvivalPack/Blueprints/Structs/S_InventoryItem` (`self.Item Data`)))
  (bind (_item_data_id_2 _item_data_amount_2 _item_data_cachedindex_2 _item_data_inventoryreference_2 _item_data_custominteger_2 _item_data_durability_2 _item_data_additionaldata_2) (break `/Game/UltimateSurvivalPack/Blueprints/Structs/S_InventoryItem` (`self.Item Data`)))
  (bind (_bisvalid _item_data) (`/Game/UltimateSurvivalPack/Blueprints/BFL_Inventory.Get Item Data from ID` _item_data_id_2))
  (if _bisvalid
    ;[1 1 1] If item is rangeweapon and has attachments, apply them
    (if (and (`KismetMathLibrary.ClassIsChildOf` (`.HoldableClass_29_8A6F0EC8424460490B303C8F6E7391CD` (break `/Game/UltimateSurvivalPack/Blueprints/Structs/S_InventoryItemData` _item_data)) "/Game/UltimateSurvivalPack/Blueprints/Holdable/HoldableActors/Parent/BP_Holdable_RangeWeapon.BP_Holdable_RangeWeapon_C") (> (`KismetArrayLibrary.Array_Length` _item_data_additionaldata_2) 0))
      (bind _outrownames (`DataTableFunctionLibrary.GetDataTableRowNames` "/Game/UltimateSurvivalPack/Blueprints/Datatable/DT_WeaponAttachments.DT_WeaponAttachments"))
      ;;[1 1 1] Loop data and check attachment validity
      (for _array_element _item_data_additionaldata
        (bind _returnvalue (`KismetMathLibrary.Conv_ByteToInt` _array_element))
        (if (`KismetArrayLibrary.Array_IsValidIndex` _outrownames _returnvalue)
          (bind _returnvalue_2 (`|GetDataTableRow` "/Game/UltimateSurvivalPack/Blueprints/Datatable/DT_WeaponAttachments.DT_WeaponAttachments" (`|GetArrayItem` _outrownames _returnvalue))
            (:`then`
              (bind ((`AttachedSkeletalMesh_15_CFA1CAA849B266DEE4D384AE8614F55D` _attachedskeletalmesh) (`AttachtoSocketName_13_753B484B449EADBF418FAFA76F8BFEC9` _attachtosocketname) (`AttachTransform_17_3DF2AC03464CEBCA85671E8A04049FDB` _attachtransform)) (break `/Game/UltimateSurvivalPack/Blueprints/Structs/S_WeaponAttachment` _returnvalue_2))
              (`/Engine/EditorBlueprintResources/StandardMacros.IsValid` _attachedskeletalmesh
                (:`Is Valid`
                  (bind _returnvalue_3 (`AddComponent|NODE_AddStaticMeshComponent-1` :`bManualAttachment` true :`RelativeTransform` _attachtransform))
                  (`StaticMeshComponent.SetStaticMesh` _returnvalue_3 _attachedskeletalmesh)
                  (`SceneComponent.K2_AttachToComponent` _returnvalue_3 (`self.Item Mesh`) _attachtosocketname "SnapToTarget" "SnapToTarget" "SnapToTarget" true))))))))))

(fn `Local Can Overlap`
  (returns (Success :type Boolean))
  (return false))

(fn `UserConstructionScript`
  (bind (_item_data_id _item_data_amount _item_data_cachedindex _item_data_inventoryreference _item_data_custominteger _item_data_durability _item_data_additionaldata) (break `/Game/UltimateSurvivalPack/Blueprints/Structs/S_InventoryItem` (`self.Item Data`)))
  (bind (_item_data_id_2 _item_data_amount_2) (break `/Game/UltimateSurvivalPack/Blueprints/Structs/S_InventoryItem` (`self.Item Data`)))
  (bind (_bisvalid _item_data) (`/Game/UltimateSurvivalPack/Blueprints/BFL_Inventory.Get Item Data from ID` _item_data_id_2))
  (bind ((`MaximumStack_21_39EA4E634AD2ADBC0EA36C92000AFBC7` _maximumstack) (`ItemMesh_32_5AC0B44A4BF0D4ECC34C868B2CFC9CF3` _itemmesh)) (break `/Game/UltimateSurvivalPack/Blueprints/Structs/S_InventoryItemData` _item_data))
  (if _bisvalid
    (`StaticMeshComponent.SetStaticMesh` (`self.Item Mesh`) _itemmesh)
    (if (> _item_data_amount_2 _maximumstack)
      ;[1 1 1] Item Data stack Failsafe
      (set `self.Item Data` (make `/Game/UltimateSurvivalPack/Blueprints/Structs/S_InventoryItem` _item_data_id _maximumstack _item_data_cachedindex _item_data_inventoryreference _item_data_custominteger _item_data_durability _item_data_additionaldata)))))