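; Survival game mode that persists placed buildings and vehicles per level through the PlayerSave in BP_GameInstance_UMSP.
; On BeginPlay it respawns the current level's saved buildings, restoring attachment links, storage inventories, and refinery, harvestable and cupboard state.
; It also triggers car spawner respawns, then spawns saved vehicles only where a box trace finds no vehicle.
; Save and remove functions forward to the game instance, with BuildingActors mapping build IDs to actors.
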(event `self.ReceiveBeginPlay`
  (`self.Load Buildings`)
  (`self.Load Vehicles`))

(fn `Get Saved Build Data`
  (params (`Build ID` :type String))
  (returns (`Saved Data` :type "/Game/UltimateSurvivalPack/Blueprints/Structs/S_BuildSave Structure") (ReturnValue :type Boolean))
  (bind _asbp_game_instance_umsp (cast `/Game/UltimateSurvivalPack/Blueprints/BP_GameInstance_UMSP` (`GameplayStatics.GetGameInstance`)))
  (bind (_saved_data _returnvalue) (`/Game/UltimateSurvivalPack/Blueprints/BP_GameInstance_UMSP.Get Saved Data` _asbp_game_instance_umsp `Build ID`))
  (return _saved_data _returnvalue))

(fn `Load Buildings`
  (locals (`L World Name` :type String) (`L Spawned Actor` :type "Actor Object Reference") (`L Save Data` :type "/Game/UltimateSurvivalPack/Blueprints/Structs/S_BuildSave Structure"))
  (bind ((`Inventory_15_455E05174F564C8EFC99DEB244083EC8` _inventory) (`CustomFloat_21_2B1EE62141F1CF01B611A4BB124FA5E8` _customfloat) (`CustomString_25_358AA98E4F4B4693E56F5CB4422E5AF2` _customstring)) (break `/Game/UltimateSurvivalPack/Blueprints/Structs/S_BuildSave` (`local.L Save Data`)))
  (bind _returnvalue (`self.GetComponentByClass` (`local.L Spawned Actor`) "/Game/UltimateSurvivalPack/Blueprints/Components/BP_MasterInventoryComponent.BP_MasterInventoryComponent_C"))
  (bind _returnvalue_2 (`GameplayStatics.GetCurrentLevelName` true))
  (set `local.L World Name` _returnvalue_2)
  (bind _asbp_game_instance_umsp (cast `/Game/UltimateSurvivalPack/Blueprints/BP_GameInstance_UMSP` (`GameplayStatics.GetGameInstance`)))
  (bind _build_saves (`/Game/UltimateSurvivalPack/Blueprints/Save/SAV_ServerData.Build Saves` (`/Game/UltimateSurvivalPack/Blueprints/BP_GameInstance_UMSP.Player Save` _asbp_game_instance_umsp)))
  (bind _keys (`BlueprintMapLibrary.Map_Keys` _build_saves))
  (bind _values (`BlueprintMapLibrary.Map_Values` _build_saves))
  (for (_array_element _array_index) _values
    (bind _output_get (set `local.L Save Data` _array_element))
    (bind ((`BuildData_2_700EB4E148DBEF7281188785324662CA` _builddata) (`Transform_6_227D833D45720C2C90F11EB731C1BBAA` _transform) (`OnAttachedActor_9_07069BCA4FEF9223D5BEC6BA5C09F0C5` _onattachedactor) (`WorldName_11_6840022640BD07C9638712B3FDD0588F` _worldname) (`Inventory_15_455E05174F564C8EFC99DEB244083EC8` _inventory_2) (`Cupboard_28_E77CCD52410AEBABC31F47A904A01FB2` _cupboard) (`Health_35_3685E417491C5C60374FFFA4E51A29DB` _health)) (break `/Game/UltimateSurvivalPack/Blueprints/Structs/S_BuildSave` _output_get))
    (if (`KismetStringLibrary.EqualEqual_StrStr` _worldname (`local.L World Name`))
      ;[1 1 1] Spawn Building and Set Data
      (bind _returnvalue_3 (`|SpawnActorFromClass` (`.FinalBuildingClass_9_4326F1B541E7F202FC5966BCF6E0D317` (break `/Game/UltimateSurvivalPack/Blueprints/Structs/S_Building` _builddata)) _transform "Undefined" "SelectDefaultAtRuntime" null null))
      (bind _output_get_2 (set `local.L Spawned Actor` _returnvalue_3))
      (bind _returnvalue_4 (`AddComponent|NODE_AddBP_BuildingComponent-0` :`self` _output_get_2))
      (bind _output_get_3 (set `/Game/UltimateSurvivalPack/Blueprints/Buildings/Parent/BP_BuildingComponent.Build ID` (`|GetArrayItem` _keys _array_index) _returnvalue_4))
      (set `/Game/UltimateSurvivalPack/Blueprints/Buildings/Parent/BP_BuildingComponent.Build Data` _builddata _returnvalue_4)
      (set `/Game/UltimateSurvivalPack/Blueprints/Buildings/Parent/BP_BuildingComponent.Cupboard ID` _cupboard _returnvalue_4)
      (set `/Game/UltimateSurvivalPack/Blueprints/Buildings/Parent/BP_BuildingComponent.Health` _health _returnvalue_4)
      (`BlueprintMapLibrary.Map_Add` (`self.Building Actors`) _output_get_3 (`local.L Spawned Actor`))
      (bind (_value _returnvalue_5) (`BlueprintMapLibrary.Map_Find` (`self.Building Actors`) _onattachedactor))
      (if _returnvalue_5
        (`/Game/UltimateSurvivalPack/Blueprints/Buildings/Parent/BP_BuildingComponent.Add Attached Actor` (`self.GetComponentByClass` _value "/Game/UltimateSurvivalPack/Blueprints/Buildings/Parent/BP_BuildingComponent.BP_BuildingComponent_C") _output_get_3))
      ;[1 1 1] Set Inventory To Storages
      (`/Engine/EditorBlueprintResources/StandardMacros.IsValid` _returnvalue
        (:`Is Valid`
          (for (_array_element_2 _array_index_2) _inventory_2
            (bind (_id _amount _cachedindex _inventoryreference _custominteger _durability) (break `/Game/UltimateSurvivalPack/Blueprints/Structs/S_InventoryItem` _array_element_2))
            (`KismetArrayLibrary.Array_Set` (`/Game/UltimateSurvivalPack/Blueprints/Components/BP_MasterInventoryComponent.Inventory` _returnvalue) _array_index_2 (make `/Game/UltimateSurvivalPack/Blueprints/Structs/S_InventoryItem` _id _amount _cachedindex _returnvalue _custominteger _durability) true))
          ;[1 1 1] Load Rafinery
          (bind _asbp_rafinery (cast `/Game/UltimateSurvivalPack/Blueprints/Buildings/Final/BP_Rafinery` (`local.L Spawned Actor`)))
          (for _array_element_3 _customstring
            (`KismetArrayLibrary.Array_Add` (`/Game/UltimateSurvivalPack/Blueprints/Buildings/Final/BP_Rafinery.Slot Items` _asbp_rafinery) (`KismetStringLibrary.Conv_StringToName` _array_element_3)))
          (for (_array_element_4 _array_index_3) _customfloat
            (if (> _array_index_3 0)
              (`KismetArrayLibrary.Array_Add` (`/Game/UltimateSurvivalPack/Blueprints/Buildings/Final/BP_Rafinery.Slot Time` _asbp_rafinery) (`KismetMathLibrary.FTrunc` _array_element_4))))
          (if (`KismetArrayLibrary.Array_IsValidIndex` _customfloat)
            (bind _output_get_4 (set `/Game/UltimateSurvivalPack/Blueprints/Buildings/Final/BP_Rafinery.Current Fuel Time` (`KismetMathLibrary.FTrunc` (`|GetArrayItem` _customfloat)) _asbp_rafinery))
            (if (> _output_get_4 0)
              (`self.SetActorTickEnabled` _asbp_rafinery true)
              (set `/Game/UltimateSurvivalPack/Blueprints/Buildings/Final/BP_Rafinery.Active` true _asbp_rafinery)
              (else
                (`/Game/UltimateSurvivalPack/Blueprints/Buildings/Final/BP_Rafinery.On Storage Updated` _asbp_rafinery)))))
        (:`Is Not Valid`
          ;[1 1 1] Sat Harvestable Data
          (bind _asbp_harvestable (cast `/Game/UltimateSurvivalPack/Blueprints/Buildings/Harvestable/Parent/BP_Harvestable` (`local.L Spawned Actor`))
            (:`then`
              (if (> (`KismetArrayLibrary.Array_Length` _customfloat) 0)
                (set `/Game/UltimateSurvivalPack/Blueprints/Buildings/Harvestable/Parent/BP_Harvestable.Current Stage` (`KismetMathLibrary.FTrunc` (`|GetArrayItem` _customfloat)) _asbp_harvestable)
                (set `/Game/UltimateSurvivalPack/Blueprints/Buildings/Harvestable/Parent/BP_Harvestable.Saved Time` (`|GetArrayItem` _customfloat 1) _asbp_harvestable)))
            (:`CastFailed`
              ;[1 1 1] Set Cupboard Data
              (bind _asbp_cupboard (cast `/Game/UltimateSurvivalPack/Blueprints/Buildings/Final/BP_Cupboard` (`local.L Spawned Actor`)))
              (for _array_element_5 _inventory
                (`KismetArrayLibrary.Array_AddUnique` (`/Game/UltimateSurvivalPack/Blueprints/Buildings/Final/BP_Cupboard.Privilege Players` _asbp_cupboard) (`KismetStringLibrary.Conv_NameToString` (`.ID_2_1F4451EE4759095BA0D31BB237483A5E` (break `/Game/UltimateSurvivalPack/Blueprints/Structs/S_InventoryItem` _array_element_5)))))
              (set `/Game/UltimateSurvivalPack/Blueprints/Buildings/Final/BP_Cupboard.Privilege Buildings` _customstring _asbp_cupboard))))))))

(fn `Load Vehicles`
  (bind _outactors (`GameplayStatics.GetAllActorsOfClass` "/Game/UltimateSurvivalPack/Blueprints/BP_CarSpawner.BP_CarSpawner_C"))
  (for _array_element _outactors
    (`/Game/UltimateSurvivalPack/Blueprints/BP_CarSpawner.Request Respawn` _array_element))
  (bind _asbp_game_instance_umsp (cast `/Game/UltimateSurvivalPack/Blueprints/BP_GameInstance_UMSP` (`GameplayStatics.GetGameInstance`)))
  (bind _vehicle_saves (`/Game/UltimateSurvivalPack/Blueprints/Save/SAV_ServerData.Vehicle Saves` (`/Game/UltimateSurvivalPack/Blueprints/BP_GameInstance_UMSP.Player Save` _asbp_game_instance_umsp)))
  (bind _keys (`BlueprintMapLibrary.Map_Keys` _vehicle_saves))
  (bind _values (`BlueprintMapLibrary.Map_Values` _vehicle_saves))
  (bind _returnvalue (`GameplayStatics.GetCurrentLevelName` true))
  (for (_array_element_2 _array_index) _keys
    (bind (_health _maximumhealth _color _fuelamount _transform _levelname _vehicleclass) (break `/Game/UltimateSurvivalPack/Blueprints/Structs/S_VehicleSaveData` (`|GetArrayItem` _values _array_index)))
    (if (`KismetStringLibrary.EqualEqual_StrStr` _returnvalue _levelname)
      (bind _location (.location _transform))
      (bind (_outhit _returnvalue_2) (`KismetSystemLibrary.BoxTraceSingleForObjects` _location _location (200.0 100.0 100.0) (.rotation _transform) (`|MakeArray` "ObjectTypeQuery5" :!type "EObjectTypeQuery Enum")))
      (if (not _returnvalue_2)
        (`|SpawnActorFromClass` _vehicleclass _transform "AdjustIfPossibleButAlwaysSpawn" "SelectDefaultAtRuntime" null _fuelamount 3.0 _array_element_2 false _health _maximumhealth _color null null)))))

(fn `Remove Building`
  (params (`Build ID` :type String))
  (bind _asbp_game_instance_umsp (cast `/Game/UltimateSurvivalPack/Blueprints/BP_GameInstance_UMSP` (`GameplayStatics.GetGameInstance`)))
  (`/Game/UltimateSurvivalPack/Blueprints/BP_GameInstance_UMSP.Remove Building` _asbp_game_instance_umsp (`local.Build ID`))
  (`BlueprintMapLibrary.Map_Remove` (`self.Building Actors`) (`local.Build ID`)))

(fn `Remove Vehicle Save`
  (params (`Vehicle ID` :type String))
  (bind _asbp_game_instance_umsp (cast `/Game/UltimateSurvivalPack/Blueprints/BP_GameInstance_UMSP` (`GameplayStatics.GetGameInstance`)))
  (`BlueprintMapLibrary.Map_Remove` (`/Game/UltimateSurvivalPack/Blueprints/Save/SAV_ServerData.Vehicle Saves` (`/Game/UltimateSurvivalPack/Blueprints/BP_GameInstance_UMSP.Player Save` _asbp_game_instance_umsp)) `Vehicle ID`))

(fn `Save Existing Building`
  (params (`Build ID` :type String) (`New Save` :type "/Game/UltimateSurvivalPack/Blueprints/Structs/S_BuildSave Structure"))
  (bind _asbp_game_instance_umsp (cast `/Game/UltimateSurvivalPack/Blueprints/BP_GameInstance_UMSP` (`GameplayStatics.GetGameInstance`)))
  (`/Game/UltimateSurvivalPack/Blueprints/BP_GameInstance_UMSP.Save Existing Building` _asbp_game_instance_umsp (`local.Build ID`) `New Save`))

(fn `Save Existing Building Directly`
  (params (`Build ID` :type String) (`New Save` :type "/Game/UltimateSurvivalPack/Blueprints/Structs/S_BuildSave Structure"))
  (bind _asbp_game_instance_umsp (cast `/Game/UltimateSurvivalPack/Blueprints/BP_GameInstance_UMSP` (`GameplayStatics.GetGameInstance`)))
  (`/Game/UltimateSurvivalPack/Blueprints/BP_GameInstance_UMSP.Save Building Directly` _asbp_game_instance_umsp (`local.Build ID`) `New Save`))

(fn `Save New Building`
  (params (`Build Data` :type "/Game/UltimateSurvivalPack/Blueprints/Structs/S_Building Structure") (`Spawned Actor` :type "Actor Object Reference") (Transform :type "Transform Structure") (`Placed On Actor` :type "Actor Object Reference"))
  (returns (`Build ID` :type String))
  (locals (`L World Name` :type String))
  (bind _returnvalue (`self.GetComponentByClass` (`local.Placed On Actor`) "/Game/UltimateSurvivalPack/Blueprints/Buildings/Parent/BP_BuildingComponent.BP_BuildingComponent_C"))
  (bind _returnvalue_2 (`GameplayStatics.GetCurrentLevelName` true))
  (set `local.L World Name` _returnvalue_2)
  (bind _asbp_game_instance_umsp (cast `/Game/UltimateSurvivalPack/Blueprints/BP_GameInstance_UMSP` (`GameplayStatics.GetGameInstance`)))
  (`/Engine/EditorBlueprintResources/StandardMacros.IsValid` _returnvalue
    (:`Is Valid`
      (bind _build_id (`/Game/UltimateSurvivalPack/Blueprints/BP_GameInstance_UMSP.Add New Building` _asbp_game_instance_umsp (make `/Game/UltimateSurvivalPack/Blueprints/Structs/S_BuildSave` (`local.Build Data`) (`local.Transform`) (`/Game/UltimateSurvivalPack/Blueprints/Buildings/Parent/BP_BuildingComponent.Build ID` _returnvalue) (`local.L World Name`) _ _ _ "" (`.Health_24_A0BD453941DAB13B0A4FDD99102D5C21` (break `/Game/UltimateSurvivalPack/Blueprints/Structs/S_Building` (`local.Build Data`))))))
      (`BlueprintMapLibrary.Map_Add` (`self.Building Actors`) _build_id (`local.Spawned Actor`))
      (return _build_id))
    (:`Is Not Valid`
      (bind _build_id_2 (`/Game/UltimateSurvivalPack/Blueprints/BP_GameInstance_UMSP.Add New Building` _asbp_game_instance_umsp (make `/Game/UltimateSurvivalPack/Blueprints/Structs/S_BuildSave` (`local.Build Data`) (`local.Transform`) "" (`local.L World Name`) _ _ _ "" (`.Health_24_A0BD453941DAB13B0A4FDD99102D5C21` (break `/Game/UltimateSurvivalPack/Blueprints/Structs/S_Building` (`local.Build Data`))))))
      (`BlueprintMapLibrary.Map_Add` (`self.Building Actors`) _build_id_2 (`local.Spawned Actor`))
      (return _build_id_2))))

(fn `Save Vehicle`
  (params (`Vehicle ID` :type String) (`Vehicle Save Data` :type "/Game/UltimateSurvivalPack/Blueprints/Structs/S_VehicleSaveData Structure"))
  (bind _asbp_game_instance_umsp (cast `/Game/UltimateSurvivalPack/Blueprints/BP_GameInstance_UMSP` (`GameplayStatics.GetGameInstance`)))
  (`/Game/UltimateSurvivalPack/Blueprints/BP_GameInstance_UMSP.Add Vehicle Save` _asbp_game_instance_umsp (`local.Vehicle ID`) `Vehicle Save Data`))

(fn `UserConstructionScript`)