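; BP_AISpawner is a placed actor that spawns one AI pawn of a configured class at its own location and yaw, and respawns it on request.
; On BeginPlay it spawns the pawn, stores the reference and, for BP_AIBase pawns, sets itself as their SpawnerReference.
; RequestRespawn waits RespawnDelay, then reruns the spawn logic, only if the stored AI is no longer valid when the request arrives.
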(event `self.ReceiveBeginPlay`
  (bind (_returnvalue_roll _returnvalue_pitch _returnvalue_yaw) (`KismetMathLibrary.BreakRotator` (`self.K2_GetActorRotation`)))
  (bind _returnvalue (`AIBlueprintHelperLibrary.SpawnAIFromClass` (`self.AI to Spawn`) null (`self.K2_GetActorLocation`) (`KismetMathLibrary.MakeRotator` 0.0 0.0 _returnvalue_yaw) true self :!label _label))
  (bind _output_get (set `self.AI Reference` _returnvalue))
  (bind _asbp_aibase (cast `/Game/UltimateSurvivalPack/Blueprints/AI/BP_AIBase` _output_get))
  (set `/Game/UltimateSurvivalPack/Blueprints/AI/BP_AIBase.Spawner Reference` self _asbp_aibase))

(event `/Game/UltimateSurvivalPack/Blueprints/Interface/BPI_Spawning.Request Respawn`
  (`self.AI Reference`
    (:`then`)
    (:`else`
      (`KismetSystemLibrary.Delay` (`self.Respawn Delay`))
      (goto _label))))

(fn `UserConstructionScript`)