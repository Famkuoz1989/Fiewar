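; BP_NPC_Gabriel is a dialogue NPC, Gabriel, who gives the player the supplies mission.
; It overrides On Question Answered: the "Answered Sure" answer ID adds mission:supplies from DT_Missions to the quest log through player controller 0's mission component.
; The function returns true, and the event graph holds only disabled default events.
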(fn `On Question Answered`
  (params (`Unique ID` :type Name) (Caller :type "/Game/UltimateSurvivalPack/Blueprints/Components/BP_MissionComponent Object Reference"))
  (returns (Success :type Boolean))
  (switch `name` `Unique ID`
    (:`Default`
      _)
    (:`AnsweredSure`
      (`/Game/UltimateSurvivalPack/Blueprints/Components/BP_MissionComponent.Add Quest to Quest Log` (`/Game/UltimateSurvivalPack/Blueprints/BFL_UMSPack.Get Mission Component` (`GameplayStatics.GetPlayerController` 0)) (make `/Game/UltimateSurvivalPack/Blueprints/Structs/S_MissionDatabase` "/Game/UltimateSurvivalPack/Blueprints/Datatable/Mission/DT_Missions.DT_Missions" "mission:supplies"))))
  (return true))

(fn `UserConstructionScript`
  (`parent.UserConstructionScript`))