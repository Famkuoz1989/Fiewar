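; Base NPC Blueprint for a modular human character that players can talk to through the dialogue and mission system.
; Interaction opens a datatable dialogue, preferring rows matching current mission objectives, and answered questions report mission progress.
; Construction assembles leader-posed body meshes with a tinted dynamic material.
; Selection toggles outline stencil and nametag, while nearby players become look targets, with turn-in-place rotation driven by an animation curve.
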(event `self.ReceiveTick`
  (params (DeltaSeconds :type "Float (single-precision)"))
  (`self.TurnInPlace`))

(event `/Game/UltimateSurvivalPack/Blueprints/Interface/BPI_InventorySystem.On Interacted`
  (params (Executor :type "Controller Object Reference"))
  (bind _missioncomponent (`/Game/UltimateSurvivalPack/Blueprints/BFL_UMSPack.Get Mission Component` Executor))
  ;[1 1 1] On Interact
  (bind _dialogue_id (`self.Select Dialogue` _missioncomponent))
  (`/Game/UltimateSurvivalPack/Blueprints/Components/BP_MissionComponent.CLIENT Open Dialogue` _missioncomponent (`self.Dialogue Datatable`) _dialogue_id self))

(event `/Game/UltimateSurvivalPack/Blueprints/Interface/BPI_InventorySystem.Toggle Selected`
  (params (Toggle :type Boolean))
  (bind _mesh (`self.Mesh`))
  (bind _nametag_widget (`self.Nametag Widget`))
  ;[1 1 1] On Selected
  (if Toggle
    (`PrimitiveComponent.SetRenderCustomDepth` _mesh true)
    (`PrimitiveComponent.SetRenderCustomDepth` (`self.Torso`) true)
    (`PrimitiveComponent.SetRenderCustomDepth` (`self.Bottom`) true)
    (`PrimitiveComponent.SetRenderCustomDepth` (`self.Head`) true)
    (`PrimitiveComponent.SetRenderCustomDepth` (`self.Backpack`) true)
    (`PrimitiveComponent.SetRenderCustomDepth` (`self.Eyebrows`) true)
    (`PrimitiveComponent.SetRenderCustomDepth` (`self.Eyes`) true)
    (`PrimitiveComponent.SetRenderCustomDepth` (`self.Beard`) true)
    (`PrimitiveComponent.SetRenderCustomDepth` (`self.Feet`) true)
    (`PrimitiveComponent.SetCustomDepthStencilValue` _mesh 1)
    (`PrimitiveComponent.SetCustomDepthStencilValue` (`self.Torso`) 1)
    (`PrimitiveComponent.SetCustomDepthStencilValue` (`self.Bottom`) 1)
    (`PrimitiveComponent.SetCustomDepthStencilValue` (`self.Head`) 1)
    (`PrimitiveComponent.SetCustomDepthStencilValue` (`self.Backpack`) 1)
    (`PrimitiveComponent.SetCustomDepthStencilValue` (`self.Eyebrows`) 1)
    (`PrimitiveComponent.SetCustomDepthStencilValue` (`self.Eyes`) 1)
    (`PrimitiveComponent.SetCustomDepthStencilValue` (`self.Beard`) 1)
    (`PrimitiveComponent.SetCustomDepthStencilValue` (`self.Feet`) 1)
    (`/Engine/EditorBlueprintResources/StandardMacros.DoOnce` false :!label _label
      (:`Completed`
        (`SceneComponent.SetVisibility` _nametag_widget true false)
        (bind _asw_npc_nametag (cast `/Game/UltimateSurvivalPack/Widget/W_NPC_Nametag` (`WidgetComponent.GetWidget` _nametag_widget)))
        (`/Game/UltimateSurvivalPack/Widget/W_NPC_Nametag.Blend ` _asw_npc_nametag (`self.NPC Name`))
        (goto _label_2 :!via `Reset`)))
    (else
      (`PrimitiveComponent.SetRenderCustomDepth` _mesh false)
      (`PrimitiveComponent.SetRenderCustomDepth` (`self.Torso`) false)
      (`PrimitiveComponent.SetRenderCustomDepth` (`self.Bottom`) false)
      (`PrimitiveComponent.SetRenderCustomDepth` (`self.Head`) false)
      (`PrimitiveComponent.SetRenderCustomDepth` (`self.Backpack`) false)
      (`PrimitiveComponent.SetRenderCustomDepth` (`self.Eyebrows`) false)
      (`PrimitiveComponent.SetRenderCustomDepth` (`self.Eyes`) false)
      (`PrimitiveComponent.SetRenderCustomDepth` (`self.Beard`) false)
      (`PrimitiveComponent.SetRenderCustomDepth` (`self.Feet`) false)
      (`PrimitiveComponent.SetCustomDepthStencilValue` _mesh 0)
      (`PrimitiveComponent.SetCustomDepthStencilValue` (`self.Torso`) 0)
      (`PrimitiveComponent.SetCustomDepthStencilValue` (`self.Bottom`) 0)
      (`PrimitiveComponent.SetCustomDepthStencilValue` (`self.Head`) 0)
      (`PrimitiveComponent.SetCustomDepthStencilValue` (`self.Backpack`) 0)
      (`PrimitiveComponent.SetCustomDepthStencilValue` (`self.Eyebrows`) 0)
      (`PrimitiveComponent.SetCustomDepthStencilValue` (`self.Eyes`) 0)
      (`PrimitiveComponent.SetCustomDepthStencilValue` (`self.Beard`) 0)
      (`PrimitiveComponent.SetCustomDepthStencilValue` (`self.Feet`) 0)
      (`/Engine/EditorBlueprintResources/StandardMacros.DoOnce` false :!label _label_2
        (:`Completed`
          (`SceneComponent.SetVisibility` (`self.Nametag Widget`) false false)
          (goto _label :!via `Reset`))))))

(event `/Game/UltimateSurvivalPack/Blueprints/Interface/BPI_InventorySystem.Local Overlap`
  (params (Overlap :type Boolean))
  (if Overlap
    (bind _output_get (set `self.Looking Actor` (`/Game/UltimateSurvivalPack/Blueprints/Components/BP_PlayerInventoryComponent.Human Player Character` (`/Game/UltimateSurvivalPack/Blueprints/BFL_UMSPack.Get Inventory Component` (`GameplayStatics.GetPlayerController` 0)))))
    (bind _asabp_human_npc (cast `/Game/UltimateSurvivalPack/Demo/Character/Animations/Human/ABP_Human_NPC` (`SkeletalMeshComponent.GetAnimInstance` (`self.Mesh`))))
    (set `/Game/UltimateSurvivalPack/Demo/Character/Animations/Human/ABP_Human_NPC.Looking Target` _output_get _asabp_human_npc)
    (else
      (bind _output_get_2 (set `self.Looking Actor` null))
      (bind _asabp_human_npc_2 (cast `/Game/UltimateSurvivalPack/Demo/Character/Animations/Human/ABP_Human_NPC` (`SkeletalMeshComponent.GetAnimInstance` (`self.Mesh`))))
      (set `/Game/UltimateSurvivalPack/Demo/Character/Animations/Human/ABP_Human_NPC.Looking Target` _output_get_2 _asabp_human_npc_2))))

(fn `Get Interaction Data`
  (returns (`Interaction Text` :type Text))
  (return (`|FormatText` "Talk to {name}" (`self.NPC Name`))))

(fn `Get Team ID`
  (returns (`Team ID` :type Byte))
  (return 0))

(fn `Local Can Overlap`
  (returns (Success :type Boolean))
  (return (< (`self.GetSquaredDistanceTo` (`Controller.K2_GetPawn` (`GameplayStatics.GetPlayerController` 0))) 160000.0)))

(fn `On Question Answered`
  (params (`Unique ID` :type Name) (Caller :type "/Game/UltimateSurvivalPack/Blueprints/Components/BP_MissionComponent Object Reference"))
  (returns (Success :type Boolean))
  (`/Game/UltimateSurvivalPack/Blueprints/Components/BP_MissionComponent.Receive Progress` Caller (make `/Game/UltimateSurvivalPack/Blueprints/Structs/S_TargetInformation` :`Target Type` "NewEnumerator3" :`Unique ID` `Unique ID`) "NewEnumerator3" true)
  (return true))

(fn `Select Dialogue`
  (params (MissionComponent :type "/Game/UltimateSurvivalPack/Blueprints/Components/BP_MissionComponent Object Reference"))
  (returns (`Dialogue ID` :type Name))
  (bind _dialogue_datatable (`self.Dialogue Datatable`))
  (if (`/Game/UltimateSurvivalPack/Blueprints/Components/BP_MissionComponent.Is In Mission ?` MissionComponent)
    (bind _outrownames (`DataTableFunctionLibrary.GetDataTableRowNames` _dialogue_datatable))
    (for _array_element _outrownames
      (bind _returnvalue (`|GetDataTableRow` _dialogue_datatable _array_element)
        (:`then`
          (bind (_usecustomdialogue _uniqueid) (break `/Game/UltimateSurvivalPack/Blueprints/Structs/S_MissionDialogue` (`.QuestInformation_16_86C991E3483DD6063741289843D8E21A` (break `/Game/UltimateSurvivalPack/Blueprints/Structs/S_Dialogue` _returnvalue))))
          (if _usecustomdialogue
            (if (`.Successful` (`/Game/UltimateSurvivalPack/Blueprints/Components/BP_MissionComponent.Find Target In Current Objectives` (`local.MissionComponent`) (make `/Game/UltimateSurvivalPack/Blueprints/Structs/S_TargetInformation` :`Target Type` "NewEnumerator3" :`Unique ID` _uniqueid)))
              (return _array_element)))))))
  (return (`self.Default Dialogue ID`)))

(fn `UserConstructionScript`
  (bind _human_dynamic_material (`self.Human Dynamic Material`))
  ;[1 1 1] Set Main Master Pose Component
  (`SkinnedMeshComponent.SetLeaderPoseComponent` (`self.Torso`) (`self.Mesh`) false false)
  (`SkinnedMeshComponent.SetLeaderPoseComponent` (`self.Bottom`) (`self.Mesh`) false false)
  (`SkinnedMeshComponent.SetLeaderPoseComponent` (`self.Feet`) (`self.Mesh`) false false)
  (`SkinnedMeshComponent.SetLeaderPoseComponent` (`self.Head`) (`self.Mesh`) false false)
  (`SkinnedMeshComponent.SetLeaderPoseComponent` (`self.Eyebrows`) (`self.Mesh`) false false)
  (`SkinnedMeshComponent.SetLeaderPoseComponent` (`self.Eyes`) (`self.Mesh`) false false)
  (`SkinnedMeshComponent.SetLeaderPoseComponent` (`self.Beard`) (`self.Mesh`) false false)
  (`SkinnedMeshComponent.SetLeaderPoseComponent` (`self.Backpack`) (`self.Mesh`) false false)
  ;[1 1 1] Create Human Dynamic Material
  (bind _returnvalue (`KismetMaterialLibrary.CreateDynamicMaterialInstance` "/Game/UltimateSurvivalPack/Demo/Character/Material/M_Human.M_Human"))
  (bind _output_get (set `self.Human Dynamic Material` _returnvalue))
  ;[1 1 1] Set Dynamic Material
  (`PrimitiveComponent.SetMaterial` (`self.Mesh`) 0 _output_get)
  (`PrimitiveComponent.SetMaterial` (`self.Eyebrows`) 0 _output_get)
  (`PrimitiveComponent.SetMaterial` (`self.Eyes`) 0 _output_get)
  (`PrimitiveComponent.SetMaterial` (`self.Beard`) 0 _output_get)
  (`PrimitiveComponent.SetMaterial` (`self.Head`) 0 _output_get)
  (`SkinnedMeshComponent.SetSkinnedAssetAndUpdate` (`self.Feet`) (`self.Feet Mesh`) true)
  (`SkinnedMeshComponent.SetSkinnedAssetAndUpdate` (`self.Torso`) (`self.Torso Mesh`) true)
  (`SkinnedMeshComponent.SetSkinnedAssetAndUpdate` (`self.Bottom`) (`self.Bottom Mesh`) true)
  (`SkinnedMeshComponent.SetSkinnedAssetAndUpdate` (`self.Head`) (`self.Head Mesh`) true)
  (`SkinnedMeshComponent.SetSkinnedAssetAndUpdate` (`self.Backpack`) (`self.Backpack Mesh`) true)
  (`SkinnedMeshComponent.SetSkinnedAssetAndUpdate` (`self.Eyebrows`) (`self.Eyebrows Mesh`) true)
  (`SkinnedMeshComponent.SetSkinnedAssetAndUpdate` (`self.Eyes`) (`self.Eyes Mesh`) true)
  (`SkinnedMeshComponent.SetSkinnedAssetAndUpdate` (`self.Beard`) (`self.Beard Mesh`) true)
  (`MaterialInstanceDynamic.SetVectorParameterValue` _human_dynamic_material "Skin Color" (`self.Skin Color`))
  (`MaterialInstanceDynamic.SetVectorParameterValue` _human_dynamic_material "Stubble Color" (`self.Stubble Color`))
  (`MaterialInstanceDynamic.SetVectorParameterValue` _human_dynamic_material "Hair Color" (`self.Hair Color`)))