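; BP_BaseViewMVP is a main-menu display actor that shows the selected soldier class and hands off to weapon customization.
; SetChillActorClass swaps the child actor to that class's view Blueprint when Equip is set or the class differs, then updates its weapon equipment.
; ActiveMeshViewNew starts the customization system, checks save availability, hides the child actor and plays an opening sound.
; SetHidIngameLight resets rotation and toggles light visibility by the GameInstance's current menu tab.
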(event `SetChillActorClass`
  (params (BaseClass :type "/Game/Systems/Enum/BaseClass Enum" :default "NewEnumerator5") (Equip :type Boolean))
  (bind _baseactor (`self.BaseActor`))
  ;[1 1 1] Comment
  (if Equip
    (set `self.Base Class` BaseClass :!label _label)
    (`ChildActorComponent.SetChildActorClass` _baseactor (select `/Game/Systems/Enum/BaseClass` (`self.Base Class`) :`NewEnumerator0` "/Game/ThirdPersonKit/Blueprints/BaseView/BP_Soldier_BaseViewMaimenu.BP_Soldier_BaseViewMaimenu_C" :`NewEnumerator1` "/Game/ThirdPersonKit/Blueprints/BaseView/BP_Medic_BaseViewMaimenu.BP_Medic_BaseViewMaimenu_C" :`NewEnumerator2` "/Game/ThirdPersonKit/Blueprints/BaseView/BP_Sniper_BaseViewMaimenu.BP_Sniper_BaseViewMaimenu_C" :`NewEnumerator3` "/Game/ThirdPersonKit/Blueprints/BaseView/BP_Mechanic_BaseViewMaimenu.BP_Mechanic_BaseViewMaimenu_C" :`NewEnumerator4` "/Game/ThirdPersonKit/Blueprints/BaseView/BP_Engineer_BaseViewMaimenu.BP_Engineer_BaseViewMaimenu_C" :!type "Actor Class Reference"))
    (bind _asbp_base_view_maimenu (cast `/Game/ThirdPersonKit/Blueprints/BaseView/BP_BaseViewMaimenu` (`ChildActorComponent.ChildActor` _baseactor)))
    (`/Game/ThirdPersonKit/Blueprints/BaseView/BP_BaseViewMaimenu.Update ClassBase Weapon EQ ` _asbp_base_view_maimenu Equip)
    (elif (not (`|EnumEquality` BaseClass (`self.Base Class`)))
      (goto _label))))

(fn `UserConstructionScript`)