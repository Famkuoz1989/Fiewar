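; Main menu preview stage actor that shows the weapon or character for weapon customization.
; BeginPlay creates the menu widget, hands it this actor and takes over the player's view.
; The game instance's MaimenuTab selects the visible display, active camera and light set, while restarting customization and playing an opening sound.
; Timelines slide the cameras between framings, reversing to return, and clicking the actor or cube enables rotation.
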(event `SetCamera`
  ;[1 1 1] Comment
  (`PlayerController.SetViewTargetWithBlend` (`GameplayStatics.GetPlayerController` 0) self 0.0 "VTBlend_Linear" 0.0 true :!label _label))

(event `self.ReceiveBeginPlay`
  ;[1 1 1] Comment
  (`|ExecutionSequence`
    (:`then_0`
      (`self.WBP_6CustSlots`
        (:`then`)
        (:`else`
          (bind _returnvalue (`|CreateWidget` "/Game/DUWepCustSys/BluePrints/UI/WBP_Maimenu.WBP_Maimenu_C"))
          (bind _output_get (set `self.WBP_6CustSlots` _returnvalue))
          (`UserWidget.AddToViewport` _output_get 0)
          (set `/Game/DUWepCustSys/BluePrints/UI/WBP_Maimenu.Act_WepPreview` self (`self.WBP_6CustSlots`))
          (goto _label))))
    (:`then_1`
      (`self.SetVisibilityMeahTab`))))

(event `self.ReceiveActorOnClicked`
  (params (ButtonPressed :type "Key Structure"))
  ;[1 1 1] Comment
  (set `self.CanRotate?` true :!label _label_2))

(event `self.Cube.OnClicked`
  (params (TouchedComponent :type "PrimitiveComponent Object Reference") (ButtonPressed :type "Key Structure"))
  ;[1 1 1] Comment
  (goto _label_2))

(event `Update Location Camera Base`
  (params (Close :type Boolean))
  ;[1 1 1] Update Location Camera Base
  (if Close
    (bind (_direction _newtrack_0) (`Timeline|CameraBaseMaimenuClose` :!via `PlayFromStart` :!label _label_3)
      (:`Update`
        (`SceneComponent.K2_SetRelativeLocation` (`self.CameraBaseLobby`) _newtrack_0 true false)))
    (else
      (goto _label_3 :!via `Reverse`))))

(event `Update Location Camera Weapon`
  (params (Close :type Boolean))
  ;[1 1 1] Update Location Camera Weapon
  (if Close
    (bind (_direction _newtrack_0) (`Timeline|Timeline Update Location Camera Weapon` :!via `PlayFromStart` :!label _label_4)
      (:`Update`
        (`SceneComponent.K2_SetRelativeLocation` (`self.CameraWeaponView`) _newtrack_0 true false)))
    (else
      (goto _label_4 :!via `Reverse`))))

(event `ActiveCameraTabCharacter`
  (bind _baseactor (`self.BaseActor`))
  (bind _returnvalue (`|EnumEquality` (`/Game/Systems/BP_GameInstance.MaimenuTab` (`/Game/Systems/FunctionLibrary/FunctionLibrary.Get Game Instance`)) "NewEnumerator20"))
  ;[1 1 1] ActiveCameraTabCharacter
  (`SceneComponent.K2_SetRelativeRotation` _baseactor (`KismetMathLibrary.MakeRotator` 0.0 0.0 (select `bool` _returnvalue :`false` 80.0 :`true` 60.0 :!type "Float (single-precision)")) false false)
  (`SceneComponent.SetVisibility` _baseactor true true)
  (`ActorComponent.SetActive` (`self.CameraBaseLobby`) true false)
  (if _returnvalue
    (bind (_direction _newtrack_0) (`Timeline|Timeline_ActiveCameraTabCharacter` :!via `PlayFromStart` :!label _label_5)
      (:`Update`
        (`SceneComponent.K2_SetRelativeLocation` (`self.CameraBaseLobby`) _newtrack_0 true false)))
    (else
      (goto _label_5 :!via `Reverse`))))

(event `ActiveCameraTabWeapon`
  ;[1 1 1] ActiveCameraTabWeapon
  (`SceneComponent.SetVisibility` (`self.WeaponActor`) true false)
  (`ActorComponent.SetActive` (`self.CameraWeaponView`) true false)
  (if (`|EnumEquality` (`/Game/Systems/BP_GameInstance.MaimenuTab` (`/Game/Systems/FunctionLibrary/FunctionLibrary.Get Game Instance`)) "NewEnumerator15")
    (bind (_direction _newtrack_0) (`Timeline|Timeline_0` :!via `PlayFromStart` :!label _label_6)
      (:`Update`
        (`SceneComponent.K2_SetRelativeLocation` (`self.CameraWeaponView`) _newtrack_0 true false)))
    (else
      (goto _label_6 :!via `Reverse`))))

(fn `SetVisibilityMeahTab`
  (bind _maimenutab (`/Game/Systems/BP_GameInstance.MaimenuTab` (`/Game/Systems/FunctionLibrary/FunctionLibrary.Get Game Instance`)))
  (`self.ActiveMeshViewNew`)
  (if (or (`|EnumEquality` _maimenutab "NewEnumerator17") (`|EnumEquality` _maimenutab "NewEnumerator15"))
    (`SceneComponent.SetVisibility` (`self.WeaponActor`) true false)
    (`self.ActiveCameraTabWeapon`)
    (elif (or (`|EnumEquality` _maimenutab "NewEnumerator13") (`|EnumEquality` _maimenutab "NewEnumerator20"))
      (`SceneComponent.SetVisibility` (`self.BaseActor`) true false)
      (`self.ActiveCameraTabCharacter`))))

(fn `Update Mesh Rotator Cube`
  ;[0 0 0] Toggle Camera
  (`self.ActiveMeshViewNew`))

(fn `UserConstructionScript`)