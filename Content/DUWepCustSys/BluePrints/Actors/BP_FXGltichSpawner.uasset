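; BP_FXGltichSpawner is an actor that repeatedly spawns BP_FXGltich effect actors around its own location at irregular intervals.
; Each spawn gets a random Y and Z offset from the root in world space, while X stays fixed, scattering effects across a vertical plane.
; Tick acts as a randomized timer: it disables itself, spawns immediately, then re-enables after a random delay of up to a few seconds.
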(event `self.ReceiveBeginPlay`)

(event `self.ReceiveTick`
  (params (DeltaSeconds :type "Float (single-precision)"))
  (bind (_returnvalue_x _returnvalue_y _returnvalue_z) (`KismetMathLibrary.BreakVector` (`SceneComponent.K2_GetComponentLocation` (`self.DefaultSceneRoot`))))
  (`self.SetActorTickEnabled` false)
  (`|ExecutionSequence`
    (:`then_0`
      (`KismetSystemLibrary.Delay` (`KismetMathLibrary.RandomFloatInRange` 0.0 4.0))
      (`self.SetActorTickEnabled` true))
    (:`then_1`
      (`|SpawnActorFromClass` "/Game/DUWepCustSys/BluePrints/Actors/BP_FXGltich.BP_FXGltich_C" (`KismetMathLibrary.MakeTransform` (`KismetMathLibrary.MakeVector` (+ _returnvalue_x 0.0) (+ _returnvalue_y (`KismetMathLibrary.RandomFloatInRange` -200.0 200.0)) (+ _returnvalue_z (`KismetMathLibrary.RandomFloatInRange` -100.0 100.0)))) "Undefined" "OverrideRootScale" null null))))

(fn `UserConstructionScript`)