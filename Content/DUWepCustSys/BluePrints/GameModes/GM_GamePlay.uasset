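; GM_GamePlay is the multiplayer match game mode for Deathmatch and Team Deathmatch, covering the lobby, spawning and match end.
; Joining players are tracked and balanced into teams, with their info pushed to every PC_GamePlay client.
; Ready checks enable starting, and a full lobby auto-starts after a delay.
; It spawns characters at tagged team starts, relays kills and time, routes deaths to scoring, and removes pawns for intermission.
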(event Custom|Initialize_Match
  ;[1 1 1] Comment
  (bind _aspc_game_play (Utilities|GetAllControllLer)
    (:then
      (Default|RespawnPlayer _aspc_game_play))))

(event Custom|Update%20Session%20InGame%20GM
  ;[1 1 1] Update sesion
  (Default|UpdateSessionIngame (CallFunction|GetGameInstance) true))

(event Custom|Client%20Add%20to%20Destroyd%20Log
  (params (Who%20destroyed :type Text) (Who%20was%20Destroyed :type Text) (Team :type MyTeam%20Enum :default "NewEnumerator0"))
  ;[0.1303 0.9103 1] Update Skill Killfeed
  (bind _aspc_game_play (Utilities|GetAllControllLer)
    (:then
      (Default|ClientAddtoDestroyedLog _aspc_game_play Who%20destroyed Who%20was%20Destroyed (Utilities|Enum|Equal(Enum) (Default|GetTeam _aspc_game_play) Team)))))

(event Custom|CheckPlayerReadyClassic-GM
  (bind _allplayercontrollersteama (Variables|Default|GetAllPlayerControllersTeamA))
  (bind _allplayercontrollersteamb (Variables|Default|GetAllPlayerControllersTeamB))
  (bind _allplayercontrollers (Variables|Default|GetAllPlayerControllers))
  (bind _returnvalue (Utilities|Array|Length _allplayercontrollersteamb))
  (bind _returnvalue_2 (Utilities|Array|Length _allplayercontrollers))
  (bind _returnvalue_3 (Utilities|Array|Length _allplayercontrollersteama))
  (bind _returnvalue_4 (== _returnvalue 5))
  (bind _returnvalue_5 (== _returnvalue_3 5))
  (bind _returnvalue_6 (== _returnvalue_2 10))
  (bind _returnvalue_7 (and _returnvalue_5 _returnvalue_4))
  ;[1 1 1] Check Ready Classic
  (if (> (Utilities|Array|Length (Variables|Default|GetAllPlayerControllers)) 3)
    (if (Utilities|Enum|Equal(Enum) (Variables|Default|GetGameMode) "NewEnumerator3")
      (bind _isready_ (CallFunction|CheckReady))
      (bind _aspc_game_play (Utilities|Casting|CastToPC_GamePlay (Game|GetPlayerController 0)))
      (Default|EnableStartGameClientMain _aspc_game_play _isready_ false)
      (if _returnvalue_6
        (Utilities|FlowControl|Delay 5.0)
        (if _returnvalue_6
          (for _array_element (Variables|Default|GetAllPlayerControllers) :!label _label
            (bind _aspc_game_play_2 (Utilities|Casting|CastToPC_GamePlay _array_element))
            (Default|EnableStartGameClientMain _aspc_game_play_2 false true))))
      (else
        (bind _isready__2 (CallFunction|CheckReady))
        (bind _aspc_game_play_3 (Utilities|Casting|CastToPC_GamePlay (Game|GetPlayerController 0)))
        (Default|EnableStartGameClientMain _aspc_game_play_3 _isready__2 false)
        (if _returnvalue_7
          (Utilities|FlowControl|Delay 5.0)
          (if _returnvalue_7
            (goto _label)))))
    (else
      (bind _aspc_game_play_4 (Utilities|Casting|CastToPC_GamePlay (Game|GetPlayerController 0)))
      (Default|EnableStartGameClientMain _aspc_game_play_4 false false))))

(event Custom|DeadPlayer
  (params (DeadTeam :type MyTeam%20Enum :default "NewEnumerator0"))
  (bind _gameplaystate (Variables|Default|GetGamePlayState))
  ;[1 0 0.8823] EndGameDead
  (Variables|Default|SetDead%20Team DeadTeam)
  (if (Utilities|Enum|Equal(Enum) (Variables|Default|GetGameMode) "NewEnumerator3")
    (Default|UpdateTopPlayerState _gameplaystate)
    (else
      (Default|UpdatePointTeam _gameplaystate (Variables|Default|GetDead%20Team)))))

(event Custom|Update%20End%20Game%20Gm%20Time
  ;[1 0 0.736] Show EndGame
  (Variables|Default|SetEnd%20GameGM true)
  (Utilities|FlowControl|Delay 2.0)
  (CallFunction|SignalIntermission))

(event Custom|UpdateTimeGM
  (params (TimeUpdate :type Float%20%28double-precision%29) (Point%20Team%20A :type Integer) (Point%20Team%20B :type Integer))
  ;[0.1208 0.4677 1] Update Time GM
  (bind _aspc_game_play (Utilities|GetAllControllLer)
    (:then
      (Default|PCUpdateTimeGame _aspc_game_play TimeUpdate Point%20Team%20A Point%20Team%20B))))

(event EventHandleStartingNewPlayer
  (params (NewPlayer :type Player%20Controller%20Object%20Reference))
  ;[1 1 1] Comment
)

(event EventPostLogin
  (params (NewPlayer :type Player%20Controller%20Object%20Reference))
  ;[1 1 1] Comment
  (bind _aspc_game_play (Utilities|Casting|CastToPC_GamePlay NewPlayer))
  (Variables|/Game/DUWepCustSys/BluePrints/GameModes/PC_GamePlay.PC_GamePlay_C|SetAs%20GM%20Gameplay _aspc_game_play self)
  (Variables|Default|SetGameMode (Variables|/Game/Systems/BP_GameInstance.BP_GameInstance_C|GetGameMode (CallFunction|GetGameInstance)))
  (Utilities|Array|AddUnique (Variables|Default|GetAllPlayerControllers) _aspc_game_play)
  (CallFunction|SelectTeam _aspc_game_play))

(event EventOnSwapPlayerControllers
  (params (OldPC :type Player%20Controller%20Object%20Reference) (NewPC :type Player%20Controller%20Object%20Reference))
  ;[1 1 1] Comment
  (switch string (Variables|Default|GetLobbyStatus)
    (:Waiting
      (Utilities|Array|AddUnique (Variables|Default|GetAllPlayerControllers) NewPC)
      (bind _aspc_game_play (Utilities|Casting|CastToPC_GamePlay NewPC))
      (Default|OCInitialize _aspc_game_play))))

(event EventOnLogout
  (params (ExitingController :type Controller%20Object%20Reference))
  ;[1 1 1] Comment
  (bind _aspc_game_play (Utilities|Casting|CastToPC_GamePlay ExitingController))
  (Utilities|Array|RemoveItem (Variables|Default|GetAllPlayerControllers) _aspc_game_play)
  (if (Utilities|Enum|Equal(Enum) (Default|GetTeam _aspc_game_play) "NewEnumerator1")
    (Math|Integer|DecrementInt (Variables|Default|GetTeam%20A%20amount)
      (:%20%20
        (Utilities|Array|RemoveItem (Variables|Default|GetAllPlayerControllersTeamA) _aspc_game_play)
        (Development|PrintString "remove A")))
    (else
      (Math|Integer|DecrementInt (Variables|Default|GetTeam%20B%20amount)
        (:%20%20
          (Utilities|Array|RemoveItem (Variables|Default|GetAllPlayerControllersTeamB) _aspc_game_play)
          (Development|PrintString "remove B")))))
  (CallFunction|UpdateAllConnectedPlayers (CallFunction|GetGameplayGamemode))
  (CallFunction|CheckPlayerReadyClassic-GM))

(fn ConstructionScript)

(fn SelectTeam
  (params (NewItem :type PC%20Game%20Play%20Object%20Reference%20%28by%20ref%29))
  (if (Utilities|Enum|Equal(Enum) (Variables|Default|GetGameMode) "NewEnumerator5")
    (if (< (Variables|Default|GetTeam%20A%20amount) (Variables|Default|GetTeam%20B%20amount))
      (Utilities|Array|AddUnique (Variables|Default|GetAllPlayerControllersTeamA) NewItem)
      (Default|SetTeamQM NewItem "NewEnumerator1")
      (Math|Integer|IncrementInt (Variables|Default|GetTeam%20A%20amount)
        (:%20%20
          _))
      (else
        (Utilities|Array|AddUnique (Variables|Default|GetAllPlayerControllersTeamB) NewItem :!label _label)
        (Default|SetTeamQM NewItem "NewEnumerator2")
        (Math|Integer|IncrementInt (Variables|Default|GetTeam%20B%20amount)
          (:%20%20
            _))))
    (else
      (goto _label)))
  (Default|UpdatePlayerInfor NewItem))

(fn RefreshConnectedPlayersArray
  ;[0.1979 0.1979 0.1979] Pulls each connected player's PlayerInfo and adds it to the array of ConnectedPlayers here in the GameMode
  (if (Utilities|Enum|Equal(Enum) (Variables|Default|GetGameMode) "NewEnumerator5")
    (Utilities|Array|Clear (Variables|Default|GetPlayer%20Infor%20ArrayA))
    (Utilities|Array|Clear (Variables|Default|GetPlayer%20Infor%20ArrayB))
    (Utilities|Array|Clear (Variables|Default|GetPlayer%20Infor))
    (Utilities|AddDataPlayerInfor (Variables|Default|GetPlayer%20Infor%20ArrayA) (Variables|Default|GetAllPlayerControllersTeamA)
      (:Completed
        (Utilities|AddDataPlayerInfor (Variables|Default|GetPlayer%20Infor%20ArrayB) (Variables|Default|GetAllPlayerControllersTeamB)
          (:Completed
            (Utilities|AddDataPlayerInfor (Variables|Default|GetPlayer%20Infor) (Variables|Default|GetAllPlayerControllers)
              (:Completed
                (CallFunction|PushClientUpdates true)
                (return)))))))
    (else
      (Utilities|Array|Clear (Variables|Default|GetPlayer%20Infor))
      (Utilities|AddDataPlayerInfor (Variables|Default|GetPlayer%20Infor) (Variables|Default|GetAllPlayerControllers)
        (:Completed
          (CallFunction|PushClientUpdates false)
          (return))))))

(fn UpdateAllConnectedPlayers
  (CallFunction|RefreshConnectedPlayersArray))

(fn SpawnPlayerGm
  (params (PCGameplay :type PC%20Game%20Play%20Object%20Reference) (My%20Team :type MyTeam%20Enum :default "NewEnumerator0"))
  (bind _returnvalue (Pawn|GetControlledPawn PCGameplay))
  (bind _asbp_game_play_state (CallFunction|GetGSGameplay))
  (if (not (Variables|Default|GetEnd%20GameGM))
    (Variables|Default|SetMy%20Team My%20Team)
    (switch Utilities|FlowControl|Switch|SwitchonGameMode_Type (Variables|Default|GetGameMode)
      (:NewEnumerator3
        (Variables|Default|SetActor%20Pawn%20Class "/Game/DUWepCustSys/BluePrints/TeamB_PlayerStartPawn.TeamB_PlayerStartPawn_C"))
      (:NewEnumerator5
        (Variables|Default|SetActor%20Pawn%20Class (Utilities|Select :Index (Variables|Default|GetMy%20Team) :NewEnumerator0 "/Game/DUWepCustSys/BluePrints/PlayerStartPawnBase.PlayerStartPawnBase_C" :NewEnumerator1 "/Game/DUWepCustSys/BluePrints/TeamA_PlayerStartPawn.TeamA_PlayerStartPawn_C" :NewEnumerator2 "/Game/DUWepCustSys/BluePrints/TeamB_PlayerStartPawn.TeamB_PlayerStartPawn_C" :NewEnumerator3 "/Game/DUWepCustSys/BluePrints/PlayerStartPawnBase.PlayerStartPawnBase_C" :NewEnumerator11 "/Game/DUWepCustSys/BluePrints/PlayerStartPawnBase.PlayerStartPawnBase_C"))))
    (Utilities|IsValid _returnvalue
      (:Is%20Valid
        (Actor|DestroyActor _returnvalue))
      (:Is%20Not%20Valid
        _))
    ;[0.1979 0.1979 0.1979] Searches for an empty PlayerStart, once we find one we spawn the player there
    (bind _outactors (Actor|GetAllActorsOfClass (Variables|Default|GetActor%20Pawn%20Class)))
    (bind _array_element (Utilities|Array|ForEachLoopwithBreak _outactors :!label _label)
      (:LoopBody
        (if (Utilities|Name|NotEqual(Name) (Variables|/Script/Engine.PlayerStart|GetPlayerStartTag _array_element) "Taken")
          (Variables|/Script/Engine.PlayerStart|SetPlayerStartTag _array_element "Taken")
          (goto _label Break)))
      (:Completed
        ;[0.1979 0.1979 0.1979] Spawns a Character and makes the incoming PlayerController Possess it
        (bind _returnvalue_2 (Game|SpawnActorfromClass "/Game/ThirdPersonKit/Blueprints/BP_PlayerCharacterBase.BP_PlayerCharacterBase_C" (Math|Transform|MakeTransform (.location (Transformation|GetActorTransform _array_element)) (.rotation (Transformation|GetActorTransform _array_element)) (.scale (Transformation|GetActorTransform _array_element))) "AlwaysSpawn" "MultiplyWithRoot" PCGameplay (Variables|Default|GetMy%20Team) 0))
        (Pawn|Possess PCGameplay _returnvalue_2)
        (Default|SRSetVisibility _returnvalue_2)
        (Default|UpdateUiGameplayPawn PCGameplay true)
        (Utilities|IsValid _asbp_game_play_state
          (:Is%20Valid
            (Default|RefreshScoreboard _asbp_game_play_state)
            (Utilities|FlowControl|DoOnce false
              (:Completed
                (Default|StarTimeGS (CallFunction|GetGSGameplay))))))))))

(fn ForceStartMatch
  (CallFunction|AttempttoStarttheMatch))

(fn AttempttoStarttheMatch
  (if (CallFunction|EveryonefromLobbyHere?)
    (Variables|Default|SetMatchGamePlay "NewEnumerator2")
    (Utilities|FlowControl|DoOnce false
      (:Completed
        _))
    (else
      (switch Utilities|FlowControl|Switch|SwitchonMatchGamePlayGM (Variables|Default|GetMatchGamePlay)
        (:NewEnumerator2
          _))))
  (bind _aspc_game_play (Utilities|GetAllControllLer)
    (:then
      (Default|OCInitialize _aspc_game_play))))

(fn EveryonefromLobbyHere?
  (return (== (Variables|Default|GetNumPlayers) 0)))

(fn PushClientUpdates
  (params (Team :type Boolean))
  (bind _aspc_game_play (Utilities|GetAllControllLer)
    (:then
      (if Team
        (Default|OCUpdateTeamConnectedPlayersList _aspc_game_play (Variables|Default|GetPlayer%20Infor%20ArrayA) (Variables|Default|GetPlayer%20Infor%20ArrayB))
        (else
          (Default|OCUpdateLobbyConnectedPlayersList _aspc_game_play (Variables|Default|GetPlayer%20Infor)))))
    (:Completed
      (return))))

(fn ChangeTeamGm
  (params (ID%20Change :type Integer) (Player%20Infor_Change :type Player%20Infor%20Struct%20Structure))
  (bind _player_infor_arraya (Variables|Default|GetPlayer%20Infor%20ArrayA))
  (bind _player_infor_arrayb (Variables|Default|GetPlayer%20Infor%20ArrayB))
  (bind _returnvalue (Utilities|Array|Length _player_infor_arraya))
  (bind _returnvalue_2 (Utilities|Array|Length _player_infor_arrayb))
  (Variables|Default|SetPlayer%20Infor_Change Player%20Infor_Change)
  (bind _array_element (Utilities|Array|ForEachLoopwithBreak (Variables|Default|GetAllPlayerControllers) :!label _label)
    (:LoopBody
      (bind _aspc_game_play (Utilities|Casting|CastToPC_GamePlay _array_element))
      (if (and (or (== (- _returnvalue_2 1) _returnvalue) (== (- _returnvalue 1) _returnvalue_2)) (== (Utilities|Struct|BreakSaveDataUser_Struct (.UserProfile (Utilities|Struct|BreakPlayerInfor_Struct (Variables|/Game/DUWepCustSys/BluePrints/GameModes/PC_GamePlay.PC_GamePlay_C|GetPlayerInfor _aspc_game_play)))) (Utilities|Struct|BreakSaveDataUser_Struct (.UserProfile (Utilities|Struct|BreakPlayerInfor_Struct (Variables|Default|GetPlayer%20Infor_Change))))))
        (switch Utilities|FlowControl|Switch|SwitchonMyTeam (.MyTeam (Utilities|Struct|BreakPlayerInfor_Struct (Variables|/Game/DUWepCustSys/BluePrints/GameModes/PC_GamePlay.PC_GamePlay_C|GetPlayerInfor _aspc_game_play)))
          (:NewEnumerator1
            (Utilities|Array|RemoveItem (Variables|Default|GetPlayer%20Infor%20ArrayA) (Variables|/Game/DUWepCustSys/BluePrints/GameModes/PC_GamePlay.PC_GamePlay_C|GetPlayerInfor _aspc_game_play))
            (bind _output_get (Variables|/Game/DUWepCustSys/BluePrints/GameModes/PC_GamePlay.PC_GamePlay_C|SetMy%20Team _aspc_game_play "NewEnumerator2"))
            (Utilities|Struct|SetmembersinPlayerInfor_Struct (Variables|/Game/DUWepCustSys/BluePrints/GameModes/PC_GamePlay.PC_GamePlay_C|GetPlayerInfor _aspc_game_play) _output_get)
            (Default|SavePlayerInfo _aspc_game_play (Variables|/Game/DUWepCustSys/BluePrints/GameModes/PC_GamePlay.PC_GamePlay_C|GetPlayerInfor _aspc_game_play))
            (Utilities|Array|AddUnique (Variables|Default|GetPlayer%20Infor%20ArrayB) (Variables|/Game/DUWepCustSys/BluePrints/GameModes/PC_GamePlay.PC_GamePlay_C|GetPlayerInfor _aspc_game_play))
            (goto _label Break))
          (:NewEnumerator2
            (Utilities|Array|RemoveItem (Variables|Default|GetPlayer%20Infor%20ArrayB) (Variables|/Game/DUWepCustSys/BluePrints/GameModes/PC_GamePlay.PC_GamePlay_C|GetPlayerInfor _aspc_game_play))
            (bind _output_get_2 (Variables|/Game/DUWepCustSys/BluePrints/GameModes/PC_GamePlay.PC_GamePlay_C|SetMy%20Team _aspc_game_play "NewEnumerator1"))
            (Utilities|Struct|SetmembersinPlayerInfor_Struct (Variables|/Game/DUWepCustSys/BluePrints/GameModes/PC_GamePlay.PC_GamePlay_C|GetPlayerInfor _aspc_game_play) _output_get_2)
            (Default|SavePlayerInfo _aspc_game_play (Variables|/Game/DUWepCustSys/BluePrints/GameModes/PC_GamePlay.PC_GamePlay_C|GetPlayerInfor _aspc_game_play))
            (Utilities|Array|AddUnique (Variables|Default|GetPlayer%20Infor%20ArrayA) (Variables|/Game/DUWepCustSys/BluePrints/GameModes/PC_GamePlay.PC_GamePlay_C|GetPlayerInfor _aspc_game_play))
            (goto _label Break)))))
    (:Completed
      (CallFunction|PushClientUpdates true)
      (CallFunction|CheckPlayerReadyClassic-GM))))

(fn UpdateDataTeam
  (Utilities|Array|Clear (Variables|Default|GetPlayer%20Infor%20ArrayB))
  (Utilities|Array|Clear (Variables|Default|GetPlayer%20Infor%20ArrayA))
  (for _array_element (Variables|Default|GetPlayer%20Infor)
    (switch Utilities|FlowControl|Switch|SwitchonMyTeam (.MyTeam (Utilities|Struct|BreakPlayerInfor_Struct _array_element))
      (:NewEnumerator1
        (Utilities|Array|AddUnique (Variables|Default|GetPlayer%20Infor%20ArrayA) _array_element))
      (:NewEnumerator2
        (Utilities|Array|AddUnique (Variables|Default|GetPlayer%20Infor%20ArrayB) _array_element))))
  (CallFunction|PushClientUpdates false)
  (return))

(fn UpdateUiPlayerName
  (bind _aspc_game_play (Utilities|GetAllControllLer)
    (:then
      (bind _asbp_player_character_base (Utilities|Casting|CastToBP_PlayerCharacterBase (Pawn|GetControlledPawn _aspc_game_play)))
      (Default|MCSetVisibility _asbp_player_character_base (Variables|/Game/ThirdPersonKit/Blueprints/BP_PlayerCharacterBase.BP_PlayerCharacterBase_C|GetMy%20Name _asbp_player_character_base))
      (Default|OCSetPlayerIndicatorVisibility _asbp_player_character_base))))

(fn UpdateUiPlayerNameHit
  (params (Hit :type Object%20Object%20Reference))
  (bind _aspc_game_play (Utilities|GetAllControllLer)
    (:then
      (bind _asbp_player_character_base (Utilities|Casting|CastToBP_PlayerCharacterBase (Pawn|GetControlledPawn _aspc_game_play)))
      (if (== _aspc_game_play Hit)
        (Default|VisibilityUiNameHitDamage _asbp_player_character_base true true)
        (Default|OCSetPlayerIndicatorVisibility _asbp_player_character_base)))))

(fn SignalIntermission
  (CallFunction|RemovePlayers)
  (Default|SignalIntermission (CallFunction|GetGSGameplay) (Variables|Default|GetEnd%20GameGM) (Variables|Default|GetDraw?)))

(fn RemovePlayers
  (bind _aspc_game_play (Utilities|GetAllControllLer)
    (:then
      (bind _asbp_player_character_base (Utilities|Casting|CastToBP_PlayerCharacterBase (Pawn|GetControlledPawn _aspc_game_play)))
      (Default|SRRemoveSelf _asbp_player_character_base))))

(fn CheckReady
  (LocalVariables|SetReady? true)
  (bind _array_element (Utilities|Array|ForEachLoopwithBreak (Variables|Default|GetAllPlayerControllers) :!label _label)
    (:LoopBody
      (bind _aspc_game_play (Utilities|Casting|CastToPC_GamePlay _array_element))
      (if (not (Variables|/Game/DUWepCustSys/BluePrints/GameModes/PC_GamePlay.PC_GamePlay_C|GetReady? _aspc_game_play))
        (LocalVariables|SetReady? false)
        (goto _label Break)))
    (:Completed
      (return (LocalVariables|GetReady?)))))