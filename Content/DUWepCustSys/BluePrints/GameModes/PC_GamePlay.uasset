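; Player controller for multiplayer team matches, linking the gameplay game mode to each client's team selection and HUD widgets.
; Player info built from the game instance goes through server-style events to the game mode and PlayerState, while client-style events update lobby lists, score, timer and kill log.
; It also handles host start, team changes, timed respawn, round-end input lock, and kicks or session teardown back to the main menu.
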(event `FindKickPlayer-PCServer`
  (params (DataPlayer :type "/Game/Systems/Enum/PlayerInfor_Struct Structure"))
  (bind _as_gm_gameplay (`self.As GM Gameplay`))
  ;[1 1 1] Classic
  ;;[1 1 1] Kick Player
  (bind _aspc_game_play (cast `/Game/DUWepCustSys/BluePrints/GameModes/PC_GamePlay` (`|GetArrayItem` (`/Game/DUWepCustSys/BluePrints/GameModes/GM_GamePlay.AllPlayerControllers` _as_gm_gameplay) (`KismetArrayLibrary.Array_Find` (`/Game/DUWepCustSys/BluePrints/GameModes/GM_GamePlay.Player Infor` _as_gm_gameplay) DataPlayer))))
  (`self.KickClientMain-PC` _aspc_game_play))

(event `KickClientMain-PC`
  ;[1 1 1] Classic
  ;;[1 1 1] Kick Player
  ;;;[1 1 1] Kick Player
  (`KismetSystemLibrary.PrintString` "Kick")
  (set `/Game/Systems/BP_GameInstance.MaimenuTab` "NewEnumerator13" (`/Game/Systems/FunctionLibrary/FunctionLibrary.Get Game Instance`))
  (`AdvancedSessionsLibrary.KickPlayer` self)
  (`/Game/Systems/FunctionLibrary/FunctionLibrary.Open Level Fade In Transition Screen` "MainMenu" "" "/Game/Texture/Login/1920x1080_Loading_Back.1920x1080_Loading_Back"))

(event `Update UiGameplay Pawn`
  (params (BeginLoad :type Boolean))
  (bind _wb_gameplay_hud (`self.WB_Gameplay_HUD`))
  ;[0.2577 1 0.1038] Respawn Player
  ;;[1 1 1] Update UiGameplay Pawn
  (set `/Game/Widget/GamePlayHUD/Ingame/WB_HP.HP` 100 (`/Game/Widget/GamePlayHUD/Ingame/WB_Gameplay_HUD.WB_HP` _wb_gameplay_hud))
  (`/Game/Widget/GamePlayHUD/Ingame/WB_Gameplay_HUD.PlayAnimOpenTab` _wb_gameplay_hud 0 BeginLoad))

(event `Start Respawn Timer`
  (params (ResPawn :type Boolean))
  ;[0.2577 1 0.1038] Respawn Player
  (set `self.ResPawn` ResPawn)
  (bind _returnvalue (`KismetSystemLibrary.K2_SetTimer` null "Respawn Player" 5.0))
  (set `self.Respawn Timer Handle` _returnvalue))

(event `self.ReceiveTick`
  (params (DeltaSeconds :type "Float (single-precision)"))
  ;[1 1 1] Tick
)

(event `UpdateReday-PCServer`
  (params (`Ready?` :type Boolean))
  ;[1 1 1] Classic
  ;;[1 1 1] Update Ready
  (set `self.Ready?` `Ready?`)
  (`/Game/DUWepCustSys/BluePrints/GameModes/GM_GamePlay.CheckPlayerReadyClassic-GM` (`self.As GM Gameplay`)))

(event `Client Add to Destroyed Log`
  (params (`Who destroyed` :type Text) (`Who was Destroyed` :type Text) (bIsMyTeam :type Boolean))
  ;[1 0.1057 0] SkillFee
  (`/Game/Widget/GamePlayHUD/Ingame/WB_Gameplay_HUD.Add to Destroyed Log ` (`self.WB_Gameplay_HUD`) `Who destroyed` `Who was Destroyed` bIsMyTeam))

(event `HostTriggerStartGame-PCServer`
  ;[1 1 1] Classic
  (for _array_element (`/Game/DUWepCustSys/BluePrints/GameModes/GM_GamePlay.AllPlayerControllers` (`self.As GM Gameplay`))
    (bind _aspc_game_play (cast `/Game/DUWepCustSys/BluePrints/GameModes/PC_GamePlay` _array_element))
    (`self.EnableStartGameClientMain` _aspc_game_play false true)))

(event `PC_UpdateTimeGame`
  (params (TimeUpdate :type "Float (double-precision)") (`Point Team A` :type Integer) (`Point Team B` :type Integer))
  (bind _wb_gameplay_hud (`self.WB_Gameplay_HUD`))
  ;[0.1447 1 0] Update TimeGame
  (`/Engine/EditorBlueprintResources/StandardMacros.IsValid` _wb_gameplay_hud
    (:`Is Valid`
      (`/Game/Widget/GamePlayHUD/Ingame/WB_RealTime_HUD.Update Time End` (`/Game/Widget/GamePlayHUD/Ingame/WB_Gameplay_HUD.WB_RealTime_HUD` _wb_gameplay_hud) TimeUpdate `Point Team A` `Point Team B`))))

(event `EnableStartGameClientMain`
  (params (bInIsEnabled :type Boolean) (`StartGame?` :type Boolean))
  ;[1 1 1] Classic
  ;;[1 1 1] Update Ready
  (bind _start_gameplay_wb (`self.Start_Gameplay_WB` :!label _label)
    (:`then`
      (if `StartGame?`
        (bind _wb_star_teamselection (`/Game/Widget/WB_Lobby/WB_SelectTeam/WB_GamePlay_TeamSelection.WB_Star_TeamSelection` (`/Game/DUWepCustSys/BluePrints/UI/WBP_StartGamePlay.WB_GamePlay_TeamSelection` _start_gameplay_wb)))
        (`/Game/Widget/WB_Lobby/WB_SelectTeam/WB_Star_TeamSelection.StartGame-TeamSelection` _wb_star_teamselection)
        (else
          (`/Game/Widget/WB_Lobby/WB_SelectTeam/WB_Star_TeamSelection.EnableStartGame-TeamSelect` _wb_star_teamselection bInIsEnabled))))
    (:`else`
      (`KismetSystemLibrary.Delay` 0.2)
      (goto _label))))

(event `PC_Signal_IntermissionEnGame`
  (params (`Scoreboard Data` :type "Array of /Game/Systems/Enum/PlayerInfor_Struct Structure (by ref)") (`End Game?` :type Boolean) (`Draw?` :type Boolean) (TeamWin :type "/Game/Systems/Enum/MyTeam Enum" :default "NewEnumerator0"))
  ;[1 0 0.902] PC_Signal_IntermissionEnGame
  (bind _wb_gameplay_hud (`self.WB_Gameplay_HUD`)
    (:`then`
      (`/Game/Widget/GamePlayHUD/Ingame/WB_Gameplay_HUD.Signal_Intermission_HUD` _wb_gameplay_hud `Scoreboard Data` `End Game?` `Draw?` TeamWin))
    (:`else`)))

(event `PC_ChangeTeam`
  (bind _playerinfor (`self.PlayerInfor`))
  ;[0.8921 0.04803 1] ChangeTeam
  (`/Game/DUWepCustSys/BluePrints/GameModes/GM_GamePlay.Change Team Gm` (`/Game/Systems/FunctionLibrary/FunctionLibrary.Get GameplayGamemode`) (`.ID_14_D595CA294908F62E3F5C8F85710F1FE4` (break `/Game/Systems/Enum/SaveDataUser_Struct` (`.UserProfile_23_B7B2895744458F4ED18C0497AD5EB9BF` (break `/Game/Systems/Enum/PlayerInfor_Struct` _playerinfor)))) _playerinfor))

(event `UpdatePlayerInfor`
  ;[1 1 1] Comment
  (bind _returnvalue (`|CreateWidget` "/Game/DUWepCustSys/BluePrints/UI/WBP_StartGamePlay.WBP_StartGamePlay_C" (`GameplayStatics.GetPlayerController` 0)))
  (set `self.Start_Gameplay_WB` _returnvalue)
  (`UserWidget.AddToViewport` (`self.Start_Gameplay_WB`) 0)
  (bind _playerinfor (`self.Fetch Player Info From Game Instance`))
  (`self.SR_SubmitUpdate` _playerinfor))

(event `RunServerPawnPlayer`
  ;[1 1 1] RunServerPawnPlayer
  (`self.Respawn Player`))

(event `OC_Initialize`
  ;[1 1 1] Comment
  (`self.Create Game Play QM`)
  (bind _wb_gameplay_hud (`self.WB_Gameplay_HUD`)
    (:`then`
      (`/Game/Widget/GamePlayHUD/Ingame/WB_Gameplay_HUD.Signal_MatchStart_Gameplay HUD` _wb_gameplay_hud)
      (`self.RunServerPawnPlayer`))
    (:`else`)))

(event `OC_Update__Lobby_ConnectedPlayers_List`
  (params (`Player Infor` :type "Array of /Game/Systems/Enum/PlayerInfor_Struct Structure"))
  ;[1 1 1] Comment
  (set `self.Player Infor` `Player Infor`)
  (bind _start_gameplay_wb (`self.Start_Gameplay_WB`)
    (:`then`
      (`/Game/Widget/WB_Lobby/WB_SelectTeam/WB_GamePlay_TeamSelection.Update_ConnectedPlayers_List` (`/Game/DUWepCustSys/BluePrints/UI/WBP_StartGamePlay.WB_GamePlay_TeamSelection` _start_gameplay_wb) (`self.Player Infor`)))
    (:`else`)))

(event `SR_SubmitUpdate`
  (params (PlayerInfor :type "/Game/Systems/Enum/PlayerInfor_Struct Structure"))
  ;[1 1 1] Comment
  (set `self.PlayerInfor` PlayerInfor)
  (`self.SavePlayerInfo` (`self.PlayerInfor`))
  (`/Game/DUWepCustSys/BluePrints/GameModes/GM_GamePlay.Update All Connected Players` (`/Game/Systems/FunctionLibrary/FunctionLibrary.Get GameplayGamemode`))
  (bind _asbp_player_state_gameplay (cast `/Game/DUWepCustSys/BluePrints/BP_PlayerStateGameplay` (`self.PlayerState`)))
  (`/Game/DUWepCustSys/BluePrints/BP_PlayerStateGameplay.SR_Update_PlayerInfo` _asbp_player_state_gameplay (`self.PlayerInfor`))
  (set `/Game/DUWepCustSys/BluePrints/BP_PlayerStateGameplay.My Team` (`self.My Team`) _asbp_player_state_gameplay))

(event `SavePlayerInfo`
  (params (InPlayerInfor :type "/Game/Systems/Enum/PlayerInfor_Struct Structure"))
  ;[1 1 1] Comment
  (set `/Game/Systems/BP_GameInstance.PlayerInfor` InPlayerInfor (`/Game/Systems/FunctionLibrary/FunctionLibrary.Get Game Instance`)))

(event `OC_Update_Team_ConnectedPlayers_List`
  (params (`Player Infor ArrayA` :type "Array of /Game/Systems/Enum/PlayerInfor_Struct Structure (by ref)") (`Player Infor ArrayB` :type "Array of /Game/Systems/Enum/PlayerInfor_Struct Structure (by ref)"))
  ;[1 1 1] Comment
  (bind _start_gameplay_wb (`self.Start_Gameplay_WB`)
    (:`then`
      (`/Game/Widget/WB_Lobby/WB_SelectTeam/WB_GamePlay_TeamSelection.Update_Team_ConnectedPlayers_List` (`/Game/DUWepCustSys/BluePrints/UI/WBP_StartGamePlay.WB_GamePlay_TeamSelection` _start_gameplay_wb) `Player Infor ArrayA` `Player Infor ArrayB`))
    (:`else`)))

(event `self.ReceiveEndPlay`
  (params (EndPlayReason :type "EEndPlayReason Enum" :default "Destroyed"))
  ;[1 1 1] Destroys the session and travels to MainMenu_Level incase of a End play
  (`DestroySessionCallbackProxy.DestroySession` self
    (:`OnSuccess`
      (`/Game/Systems/FunctionLibrary/FunctionLibrary.Open Level Fade In Transition Screen` "MainMenu" "" "/Game/Texture/Login/1920x1080_Loading_Back.1920x1080_Loading_Back"))))

(event `Kicked`
  ;[0.2138 1 0.2401] KichPlayer
  (`self.Handle_TransitionScreens_When_Kicked` 2.0
    (:`Completed`
      (`DestroySessionCallbackProxy.DestroySession` self
        (:`OnSuccess`
          (`/Game/Systems/FunctionLibrary/FunctionLibrary.Open Level Fade In Transition Screen` "MainMenu" "" "/Game/Texture/Login/1920x1080_Loading_Back.1920x1080_Loading_Back"))))))

(event `OC_Update_Scoreboard`
  (params (`Player Infor` :type "Array of /Game/Systems/Enum/PlayerInfor_Struct Structure"))
  ;[0.0508 1 0] OC_Update_Scoreboard
  (set `self.Player Infor` `Player Infor`)
  (bind _wb_gameplay_hud (`self.WB_Gameplay_HUD`)
    (:`then`
      (`/Game/Widget/GamePlayHUD/Ingame/WB_RealTime_HUD.UpdateTopPlayerUI` (`/Game/Widget/GamePlayHUD/Ingame/WB_Gameplay_HUD.WB_RealTime_HUD` _wb_gameplay_hud) (`self.Player Infor`)))
    (:`else`)))

(event `EndRound-PCServer`
  (bind _asgm_gameplay (`/Game/Systems/FunctionLibrary/FunctionLibrary.Get GameplayGamemode`))
  (`/Game/DUWepCustSys/BluePrints/GameModes/GM_GamePlay.DeadPlayer` _asgm_gameplay (`self.My Team`))
  (for _array_element (`/Game/DUWepCustSys/BluePrints/GameModes/GM_GamePlay.AllPlayerControllers` _asgm_gameplay)
    (bind _aspc_game_play (cast `/Game/DUWepCustSys/BluePrints/GameModes/PC_GamePlay` _array_element))
    (`self.EndRound-PCClient` _aspc_game_play)
    (`self.Start Respawn Timer` _aspc_game_play false))
  (`KismetSystemLibrary.K2_SetTimer` null "RS-Time" 5.0))

(event `EndRound-PCClient`
  (`self.DisableInput` self))

(event `Respawn-PCClient`
  (`self.EnableInput` self))

(fn `Create Game Play QM`
  (bind _wb_gameplay_hud (`self.WB_Gameplay_HUD`)
    (:`then`
      (`KismetSystemLibrary.PrintString` "999999999999999")
      (if (not (`Widget.IsInViewport` _wb_gameplay_hud))
        (`UserWidget.AddToViewport` (`self.WB_Gameplay_HUD`) 0 :!label _label)))
    (:`else`
      (bind _returnvalue (`|CreateWidget` "/Game/Widget/GamePlayHUD/Ingame/WB_Gameplay_HUD.WB_Gameplay_HUD_C" self))
      (set `self.WB_Gameplay_HUD` _returnvalue)
      (goto _label))))

(fn `Fetch Player Info From Game Instance`
  (returns (PlayerInfor :type "/Game/Systems/Enum/PlayerInfor_Struct Structure (by ref)"))
  (bind (_data_user _classeq) (`self.GetDataUser`))
  (bind _playerinfor (`self.PlayerInfor`))
  (bind (_username _password) (break `/Game/Systems/Enum/SaveDataUser_Struct` _data_user))
  (bind ((`DataHistory_36_0533B160456AA3B61A04F1A78CE6D0C6` _datahistory)) (break `/Game/Systems/Enum/PlayerInfor_Struct` _playerinfor))
  (setmembers `/Game/Systems/Enum/HistoryData_Struct` :`StructRef` _datahistory :`ClassDataEQ` _classeq)
  (bind _structout (setmembers `/Game/Systems/Enum/PlayerInfor_Struct` :`StructRef` _playerinfor :`MyTeam` (`self.My Team`) :`Hosts` (`KismetSystemLibrary.IsServer`) :`UserProfile` (make `/Game/Systems/Enum/SaveDataUser_Struct` _username _password (`KismetMathLibrary.RandomIntegerInRange` 0 1000)) :`DataHistory` _datahistory))
  (return _structout))

(fn `Get Team`
  (returns (`My Team` :type "/Game/Systems/Enum/MyTeam Enum"))
  (return (`self.My Team`)))

(fn `GetDataUser`
  (returns (`Data User` :type "/Game/Systems/Enum/SaveDataUser_Struct Structure") (ClassEQ :type "/Game/Systems/Enum/ClassData_Struct Structure"))
  (bind _asbp_game_instance (`/Game/Systems/FunctionLibrary/FunctionLibrary.Get Game Instance`))
  (return (`/Game/Systems/SaveGame_BP.Data User` (`/Game/Systems/BP_GameInstance.As Save Game BP` _asbp_game_instance)) (`BlueprintMapLibrary.Map_Find` (`/Game/Systems/BP_GameInstance.ClassBaseEquip` _asbp_game_instance) (`/Game/Systems/BP_GameInstance.EquipClassBase` _asbp_game_instance))))

(fn `Respawn Player`
  (`KismetSystemLibrary.K2_PauseTimerHandle` (`self.Respawn Timer Handle`))
  (`self.Respawn-PCClient`)
  (bind _asgm_game_play (cast `/Game/DUWepCustSys/BluePrints/GameModes/GM_GamePlay` (`GameplayStatics.GetGameMode`)))
  (`/Game/DUWepCustSys/BluePrints/GameModes/GM_GamePlay.Spawn Player Gm` _asgm_game_play self (`self.My Team`)))

(fn `RS-Time`
  (set `/Game/Systems/GS_GamePlay.Time` 0.0 (`/Game/Systems/FunctionLibrary/FunctionLibrary.Get GS Gameplay`)))

(fn `Set Team QM`
  (params (`My Team` :type "/Game/Systems/Enum/MyTeam Enum" :default "NewEnumerator0"))
  (bind _output_get (set `self.My Team` `My Team`))
  (bind _asbp_player_state_gameplay (cast `/Game/DUWepCustSys/BluePrints/BP_PlayerStateGameplay` (`self.PlayerState`)))
  (set `/Game/DUWepCustSys/BluePrints/BP_PlayerStateGameplay.My Team` _output_get _asbp_player_state_gameplay))

(fn `UserConstructionScript`)