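; Game mode for Break Mode that tracks round count and match score for two teams, A and B.
; Ending a round increments the round counter, awards the winning team a point, and calls the match-win event once its score exceeds half the GameInstance's Round value plus one.
; The match-win event only branches on the winning team and performs no actions yet.
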(event `EndRound-EventGM`
  (params (`TeamAWinRound?` :type Boolean))
  (bind _returnvalue (+ (/ (`/Game/Systems/BP_GameInstance.Round` (`/Game/Systems/FunctionLibrary/FunctionLibrary.Get Game Instance`)) 2) 1))
  (`/Engine/EditorBlueprintResources/StandardMacros.IncrementInt` (`self.Round?`)
    (:`  `
      (if `TeamAWinRound?`
        (set `self.PointTeamA` (+ (`self.PointTeamA`) 1))
        (else
          (set `self.PointTeamB` (+ (`self.PointTeamB`) 1))))
      (if (> (`self.PointTeamA`) _returnvalue)
        (`self.WinMatch-GMEvent` true)
        (elif (> (`self.PointTeamB`) _returnvalue)
          (`self.WinMatch-GMEvent` false))))))

(event `WinMatch-GMEvent`
  (params (`TeamAWinMatch?` :type Boolean))
  (if `TeamAWinMatch?`
    _))

(fn `UserConstructionScript`
  (`parent.UserConstructionScript`))